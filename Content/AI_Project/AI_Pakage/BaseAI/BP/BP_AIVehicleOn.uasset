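; AI soldier character with modular military gear; the name suggests a variant that rides on vehicles, though no vehicle logic appears here.
; BeginPlay copies current HP to the blackboard, then after a short delay calls Init and extends weapon range; the first Tick also calls Init.
; Tick makes the mesh ignore Pawn collision on death.
; The construction script slaves gear meshes to the body via master pose; debug-UI and other leftover graphs are unwired.
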(event EventBeginPlay
  (bind _asai_컨트롤러 (Utilities|Casting|CastToAIController (Pawn|GetController self)))
  (AI|Components|Blackboard|SetValueasFloat (Variables|/Script/AIModule.AIController|GetBlackboard _asai_컨트롤러) (Utilities|Name|MakeLiteralName "AI_HP") (Variables|/Script/BaseClassModule.StatComponent|GetcurHP (Variables|Default|GetAIStat)))
  (Utilities|FlowControl|Delay 1.0)
  (Class|AICharacter|Init)
  (Variables|/Script/AIClassModule.AIWeaponComponent|Setshot_MaxRange (Actor|GetComponentbyClass "/Script/AIClassModule.AIWeaponComponent") 1e+05))

(event EventTick
  (params (DeltaSeconds :type Float%20%28single-precision%29))
  (Utilities|FlowControl|Sequence
    (:then_0
      (if (not (Variables|Default|Getinit_tri))
        (Class|AICharacter|Init)
        (Variables|Default|Setinit_tri true)))
    (:then_1
      (if (Variables|/Script/BaseClassModule.StatComponent|GetbDie (Variables|Default|GetAIStat))
        (Collision|SetCollisionResponsetoChannel (Variables|Character|GetMesh) "ECC_Pawn" "ECR_Ignore")))))

(fn ConstructionScript
  (Class|SkinnedMeshComponent|SetMasterPoseComponent (Variables|Default|GetWarBeltPreset) (Variables|Character|GetMesh) false))