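; AI-controlled character with modular tactical gear and an overhead debug widget that shows its behavior state.
; BeginPlay seeds the Blackboard with current HP from AIStat.
; Tick reads combat state, SupTotal and cover use from the controller's Blackboard into the widget, then turns it toward the player camera.
; The construction script slaves all clothing and gear meshes to the body Mesh via master pose.
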(event EventBeginPlay
  (bind _asai_컨트롤러 (Utilities|Casting|CastToAIController (Pawn|GetController self)))
  (AI|Components|Blackboard|SetValueasFloat (Variables|/Script/AIModule.AIController|GetBlackboard _asai_컨트롤러) (Utilities|Name|MakeLiteralName "AI_HP") (Variables|/Script/BaseClassModule.StatComponent|GetcurHP (Variables|Default|GetAIStat))))

(event EventTick
  (params (DeltaSeconds :type Float%20%28single-precision%29))
  (bind _widget (Variables|Default|GetWidget))
  (bind _asai_debug_ui (Utilities|Casting|CastToAI_DebugUI (UserInterface|GetWidget (Variables|Default|GetWidget))))
  (bind _asaic_base_controller (Utilities|Casting|CastToAIC_BaseController (Pawn|GetController self)))
  (switch Utilities|FlowControl|Switch|SwitchonECombat (Utilities|Enum|ByteToEnumECombat (Class|BlackboardComponent|GetValueasEnum (AI|GetBlackboard _asaic_base_controller) (Variables|Default|GetKey%20Name)))
    (:Patrol
      (Rendering|Components|TextRender|SetText (Variables|/Game/AI_Project/AI_Pakage/Ui/AI_DebugUI.AI_DebugUI_C|GetCombatText _asai_debug_ui) "Patrol"))
    (:MoveCover
      (Rendering|Components|TextRender|SetText (Variables|/Game/AI_Project/AI_Pakage/Ui/AI_DebugUI.AI_DebugUI_C|GetCombatText _asai_debug_ui) "MoveCover"))
    (:Move
      (Rendering|Components|TextRender|SetText (Variables|/Game/AI_Project/AI_Pakage/Ui/AI_DebugUI.AI_DebugUI_C|GetCombatText _asai_debug_ui) "Move"))
    (:Attack
      (Rendering|Components|TextRender|SetText (Variables|/Game/AI_Project/AI_Pakage/Ui/AI_DebugUI.AI_DebugUI_C|GetCombatText _asai_debug_ui) "Attack"))
    (:InCover
      (Rendering|Components|TextRender|SetText (Variables|/Game/AI_Project/AI_Pakage/Ui/AI_DebugUI.AI_DebugUI_C|GetCombatText _asai_debug_ui) "In Cover")))
  (Transformation|SetWorldRotation _widget (Math|Rotator|FindLookatRotation (Transformation|GetWorldLocation _widget) (Transformation|GetWorldLocation (Variables|/Script/Engine.PlayerCameraManager|GetTransformComponent (Game|GetPlayerCameraManager 0)))) false false)
  (Rendering|Components|TextRender|SetText (Variables|/Game/AI_Project/AI_Pakage/Ui/AI_DebugUI.AI_DebugUI_C|GetSup_TotalPoint _asai_debug_ui) (Utilities|Text|ToText(Float) (Class|BlackboardComponent|GetValueasFloat (AI|GetBlackboard _asaic_base_controller) (Variables|Default|GetSup_Total)) "HalfToEven"))
  (Rendering|Components|TextRender|SetText (Variables|/Game/AI_Project/AI_Pakage/Ui/AI_DebugUI.AI_DebugUI_C|GetUseCover _asai_debug_ui) (Utilities|Text|ToText(Boolean) (ScalableFloat|GetValueasBool (AI|GetBlackboard _asaic_base_controller) (Variables|Default|GetAI_UseCover)))))

(fn ConstructionScript
  (Class|SkinnedMeshComponent|SetMasterPoseComponent (Variables|Default|GetWarBeltPreset) (Variables|Character|GetMesh) false))