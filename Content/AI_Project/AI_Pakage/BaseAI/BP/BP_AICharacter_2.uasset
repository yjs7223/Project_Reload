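; BP_AICharacter_2 is an AI character Blueprint that seeds its behavior data when play begins.
; On BeginPlay it gets its AIController and copies current HP from AIStat into the AI_HP blackboard key, with no later updates in this graph.
; Disconnected leftover nodes, partly marked as discarded, hold an old stop-on-sight check during Patrol and an input-struct rebuild.
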(event EventBeginPlay
  (bind _asai_컨트롤러 (Utilities|Casting|CastToAIController (Pawn|GetController self)))
  (AI|Components|Blackboard|SetValueasFloat (Variables|/Script/AIModule.AIController|GetBlackboard _asai_컨트롤러) (Utilities|Name|MakeLiteralName "AI_HP") (Variables|/Script/BaseClassModule.StatComponent|GetcurHP (Variables|Default|GetAIStat))))

(fn ConstructionScript)