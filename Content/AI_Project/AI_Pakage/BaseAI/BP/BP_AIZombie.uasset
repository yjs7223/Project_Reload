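; BP_AIZombie is a zombie AI Blueprint that tests physics-driven hit reactions through a DragonIKPhysics component.
; Tick unconditionally switches the capsule to the Ragdoll collision profile and enables mesh physics simulation every frame.
; BulletHitEvent2 passes the hit bone to DragonIKPhysics and applies an impulse at the hit location, while mesh hits from other actors also feed that component.
; BulletHitEvent is empty, and debug prints and disconnected experimental nodes remain.
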(event OnComponentHit(Mesh)
  (params (HitComponent :type Primitive%20Component%20Object%20Reference) (OtherActor :type Actor%20Object%20Reference) (OtherComp :type Primitive%20Component%20Object%20Reference) (NormalImpulse :type Vector :default "0, 0, 0") (Hit :type Hit%20Result%20Structure%20%28by%20ref%29))
  (if (!= OtherActor self)
    (Class|DragonIKPhysicsComponent|OnHitCallback (Variables|Default|GetDragonIKPhysics) Hit "None")))

(event Custom|Bullet%20Hit%20Event
  (params (Bone_Name :type Name)))

(event EventBeginPlay)

(event Collision|EventActorBeginOverlap
  (params (OtherActor :type Actor%20Object%20Reference)))

(event EventTick
  (params (DeltaSeconds :type Float%20%28single-precision%29))
  (if true
    (Collision|SetCollisionProfileName (Variables|Default|GetCapsuleComponent) "Ragdoll" true :!class /Script/Engine.PrimitiveComponent)
    (Physics|SetSimulatePhysics (Variables|Character|GetMesh) true)))

(event EventBulletHitEvent2
  (params (Bone_Name :type Name :default "None") (Hit_Location :type Vector :default "0, 0, 0") (Hit_Impulse :type Vector :default "0, 0, 0"))
  (Development|PrintString "1111111111111111111111111111111")
  (Class|DragonIKPhysicsComponent|OnHitCallback (Variables|Default|GetDragonIKPhysics) (Collision|MakeHitResult false false 0.0 0.0 "0, 0, 0" "0, 0, 0" "0,0,1" "0,0,1" 0 0) Bone_Name)
  (Physics|AddImpulseatLocation (Variables|Character|GetMesh) Hit_Impulse Hit_Location "None"))

(fn ConstructionScript)