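; BP_Supfix is an actor that fixes the Sup point level of AI characters standing inside it when play begins.
; On BeginPlay it sets each overlapping AICharacter's Sup_TotalPoint blackboard float and its AIStatComponent's SupMinPoint to the same hardcoded value.
; Characters entering later are unaffected: the Box overlap only compares against the first AICharacter found and does nothing.
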(event OnComponentBeginOverlap(Box)
  (params (OverlappedComponent :type Primitive%20Component%20Object%20Reference) (OtherActor :type Actor%20Object%20Reference) (OtherComp :type Primitive%20Component%20Object%20Reference) (OtherBodyIndex :type Integer) (bFromSweep :type Boolean) (SweepResult :type Hit%20Result%20Structure%20%28by%20ref%29))
  (bind _returnvalue (Actor|GetActorOfClass "/Script/AIClassModule.AICharacter"))
  (if (== OtherActor _returnvalue)
    _))

(event EventBeginPlay
  (for _array_element (Collision|GetOverlappingActors "/Script/AIClassModule.AICharacter" :!class /Script/Engine.Actor)
    (AI|Components|Blackboard|SetValueasFloat (AI|GetBlackboard _array_element) (Utilities|Name|MakeLiteralName "Sup_TotalPoint") 4e+01)
    (Variables|/Script/AIClassModule.AIStatComponent|Setsup_MinPoint (Actor|GetComponentbyClass _array_element "/Script/AIClassModule.AIStatComponent") 4e+01)))

(event Collision|EventActorBeginOverlap
  (params (OtherActor :type Actor%20Object%20Reference)))

(event EventTick
  (params (DeltaSeconds :type Float%20%28single-precision%29)))

(fn ConstructionScript)