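; BP_AIDog is an enemy AI character that can walk, warn of an explosion and explode on death.
; Tick sets CanWalk on its spider AnimBP once MoveStart is true.
; When ExplosionEnabled is set, a DoOnce prints a debug warning and reveals the explosion indicator in the enemy HP widget.
; The Stat DiePlay event spawns an actor at its transform, calls Explosion, then destroys the dog after a short delay.
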(event DiePlay(Stat)
  (Game|SpawnActorfromClass "/Game/Aws/Fs_MasterUseong.Fs_MasterUseong_C" (Transformation|GetActorTransform) "Undefined" 0 0)
  (Class|AIDog|Explosion)
  (Utilities|FlowControl|Delay 2.0)
  (Actor|DestroyActor self))

(event Collision|EventActorBeginOverlap
  (params (OtherActor :type Actor%20Object%20Reference)))

(event EventTick
  (params (DeltaSeconds :type Float%20%28single-precision%29))
  (Utilities|FlowControl|Sequence
    (:then_0
      (if (Variables|Default|GetMoveStart)
        (bind _asabp_spider (Utilities|Casting|CastToABP_Spider (Components|SkeletalMesh|GetAnimInstance (Variables|Character|GetMesh))))
        (Variables|/Game/Spider_Tank/Blueprints/ABP_Spider.ABP_Spider_C|SetCan%20Walk _asabp_spider true)))
    (:then_1
      (if (Variables|Default|GetexplosionEnabled)
        (Utilities|FlowControl|DoOnce false
          (:Completed
            (Development|PrintString "warn explosion" true true "(R=1.000000,G=0.000000,B=0.962501,A=1.000000)")
            (bind _aswbp_enemy_hp (Utilities|Casting|CastToWBP_EnemyHP (UserInterface|GetWidget (Variables|Default|GetWidget))))
            (Widget|SetRenderOpacity (Variables|/Game/yjs/UI/WBP_EnemyHP.WBP_EnemyHP_C|GetWBP_Explosion _aswbp_enemy_hp) 1.0)))))))

(fn ConstructionScript)