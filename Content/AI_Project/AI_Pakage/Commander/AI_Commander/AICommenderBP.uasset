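; AI commander pawn Blueprint that supplies its AICommander controller with cover point locations from the CoverSystem.
; Tick calls GetCoverArr whenever the controller's CoverArray is empty, so the query retries until covers are found.
; GetCoverArr queries covers within a large fixed bounds around the first CoverSystem actor, then refills CoverArray with each cover's location.
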(event EventBeginPlay)

(event Collision|EventActorBeginOverlap
  (params (OtherActor :type Actor%20Object%20Reference)))

(event EventTick
  (params (DeltaSeconds :type Float%20%28single-precision%29))
  (bind _asaicommander (Utilities|Casting|CastToAICommander (Pawn|GetController)))
  (if (Utilities|Array|IsEmpty (Variables|/Script/AIClassModule.AICommander|GetCoverArray _asaicommander))
    (CallFunction|GetCoverArr)))

(fn ConstructionScript)

(fn GetCoverArr
  (bind _returnvalue (Class|CoverSystem|GetCoverSystem))
  (bind _outactors (Actor|GetAllActorsOfClass "/Script/AICoverSystem.CoverSystem"))
  (bind _asaicommander (Utilities|Casting|CastToAICommander (Pawn|GetController)))
  (if (Utilities|Array|IsEmpty (Class|CoverSystem|GetCoversWithinBounds (Utilities|Array|Get(acopy) _outactors) (Class|KismetMathLibrary|MakeBoxSphereBounds (Transformation|GetActorLocation (Utilities|Array|Get(acopy) _outactors)) "10000.000000,10000.000000,10000.000000" 1e+04)))
    (return)
    (else
      (Utilities|Array|Clear (Variables|/Script/AIClassModule.AICommander|GetCoverArray _asaicommander))
      (for _array_element (Class|CoverSystem|GetCoversWithinBounds (Utilities|Array|Get(acopy) _outactors) (Class|KismetMathLibrary|MakeBoxSphereBounds (Transformation|GetActorLocation (Utilities|Array|Get(acopy) _outactors)) "10000.000000,10000.000000,10000.000000" 1e+04))
        (Utilities|Array|Add (Variables|/Script/AIClassModule.AICommander|GetCoverArray _asaicommander) (.location (.OutData (Class|CoverSystem|GetCoverData _returnvalue _array_element)))))
      (return))))