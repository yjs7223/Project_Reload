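; Combat drone component that computes flight steering to follow a target, avoid obstacles and teleport above it when too far away.
; DroneMovement refreshes distances, predicted target location and speed, turns the drone toward the target, then sets right, forward and up axes.
; Forward, side and vertical traces override those axes near obstacles; blocked forward paths trigger TryToFind, which steers by target height and yaw.
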(event EventDroneInfOwnerHUD
  (params (Control :type ST%20Drone%20Control%20Info%20Structure) (DroneInf :type ST%20Drone%20Hud%20Info%20Structure)))

(fn DroneMovement
  (CallFunction|TargetDistance)
  (CallFunction|ActorsLocation)
  (DroneMovement|DynamicSpeed)
  (DroneMovement|DroneYawRotation)
  (DroneMovement|DroneRightLeftMovement)
  (DroneMovement|DroneForwardMovement))

(fn DroneYawRotation
  (Variables|DroneInternals|SetLookAtRotYaw (.yaw (Math|Rotator|Delta(Rotator) (Transformation|GetActorRotation (Variables|DroneReferences|GetDrone)) (Math|Rotator|MakeRotator 0.0 0.0 (.yaw (Math|Rotator|FindLookatRotation (Variables|DroneInternals|GetDroneLocation) (Variables|DroneInternals|GetTargetLocationS)))))))
  (if (not (Variables|DroneInternals|GetCloseToTarget?))
    (LocalVariables|SetpYawForce (Math|Float|MapRangeClamped (Variables|DroneInfo|GetCurrentDistanceTarget) (Variables|DroneSetup|GetAcceptanceRadius) (Variables|DroneSetup|GetMaxDistanceToSpeed) (Variables|DroneSetup|GetMinYawRotationForce) (Variables|DroneSetup|GetMaxYawRotationForce)))
    (Variables|DroneInternals|SetRightAxisForce (Variables|DroneInternals|GetLookAtRotYaw))
    (bind _output_get (Variables|DroneInfo|SetAxisYaw (Math|Float|MapRangeClamped (Variables|DroneInternals|GetLookAtRotYaw) -9e+01 9e+01 (LocalVariables|GetpYawForce) (CallFunction|Invert (LocalVariables|GetpYawForce)))))
    (Variables|DroneInfo|SetYawAlpha (Math|Float|Absolute(Float) (Math|Float|MapRangeClamped (Variables|DroneInternals|GetLookAtRotYaw) -9e+01 9e+01 (LocalVariables|GetpYawForce) (CallFunction|Invert (LocalVariables|GetpYawForce)))))
    (Class|Actor|AddActorWorldRotation (Variables|DroneReferences|GetDrone) (Math|Rotator|MakeRotator 0.0 0.0 _output_get))
    (else
      (LocalVariables|SetpYawForce 1.0)
      (Variables|DroneInternals|SetRightAxisForce 0.0)
      (if (Variables|DroneInternals|GetIdleComplete)
        _))))

(fn DroneForwardTrace
  (bind _dronelocation (Variables|DroneInternals|GetDroneLocation))
  (bind _dronerotation (Variables|DroneInternals|GetDroneRotation))
  (bind _fwtracelenght (Variables|DroneInternals|GetFwTraceLenght))
  (bind _returnvalue (Math|Vector|RotateVector "0, 0,20.000000" _dronerotation))
  (bind _returnvalue_2 (+ _dronelocation _returnvalue))
  (bind (_bloking_ _distance) (CallFunction|Trace _returnvalue_2 (+ _returnvalue_2 (* (Variables|DroneInternals|GetDroneX_Vector) (Math|Float|MapRangeClamped (Variables|DroneInfo|GetCurrentDistanceTarget) (Variables|DroneSetup|GetAcceptanceRadius) _fwtracelenght (Math|Float|SelectFloat 1.5e+02 25.0 (> (Variables|DroneInternals|GetSpeedDrone) 2e+01)) _fwtracelenght))) (Variables|DroneInternals|GetActors%20to%20Ignore) (Variables|DroneSetup|GetDebugMode?) "(R=0.000000,G=1.000000,B=0.000000,A=1.000000)"))
  (LocalVariables|SetpRayDistance _distance)
  (bind _output_get (Variables|DroneInternals|SetForwardHit? _bloking_))
  (if _output_get ; ProximToHit?
    (DroneMovement|TrytoFind)
    (return (LocalVariables|GetpRayDistance) _output_get)
    (else
      (DroneMovement|DroneAltitude)
      (return (LocalVariables|GetpRayDistance) _output_get))))

(fn DroneRightLeftMovement
  (bind _currentdistancetarget (Variables|DroneInfo|GetCurrentDistanceTarget))
  (bind _rightaxisforce (Variables|DroneInternals|GetRightAxisForce))
  (bind _acceptanceradius (Variables|DroneSetup|GetAcceptanceRadius))
  (bind _maxdistancetospeed (Variables|DroneSetup|GetMaxDistanceToSpeed))
  (bind _returnvalue (Math|Float|MapRangeClamped _currentdistancetarget _acceptanceradius _maxdistancetospeed 0.0 1.0))
  (bind _hit_ (DroneMovement|DroneSidesTrace))
  (if (not _hit_)
    (Variables|DroneInfo|SetAxisRight (Math|Float|MapRangeClamped (Math|Float|Absolute(Float) _rightaxisforce) 0.0 (Variables|DroneSetup|GetYawAngleToRightForce) 0.0 (Math|Float|SelectFloat (CallFunction|Invert _returnvalue) _returnvalue (> _rightaxisforce 0.0))))))

(fn DroneSidesTrace
  (bind _dronelocation (Variables|DroneInternals|GetDroneLocation))
  (bind _dronez_vector (Variables|DroneInternals|GetDroneZ_Vector))
  (bind _droney_axistraceangle (Variables|DroneSetup|GetDroneY_AxisTraceAngle))
  (for _index (range 0 1)
    (LocalVariables|SetInvert? (> _index 0))
    (bind (_bloking_ _distance) (CallFunction|Trace _dronelocation (+ _dronelocation (Math|Vector|SelectVector (Math|Vector|RotateVectorAroundAxis (* (Variables|DroneInternals|GetDroneY_Vector) (Variables|DroneSetup|GetDroneY_AxisOffset)) (Math|Float|SelectFloat (CallFunction|Invert _droney_axistraceangle) _droney_axistraceangle (LocalVariables|GetInvert?)) _dronez_vector) (Math|Vector|RotateVectorAroundAxis (Math|Vector|RotateVectorAroundAxis (* (Variables|DroneInternals|GetDroneY_Vector) (Variables|DroneSetup|GetDroneY_AxisOffset)) (Math|Float|SelectFloat (CallFunction|Invert _droney_axistraceangle) _droney_axistraceangle (LocalVariables|GetInvert?)) _dronez_vector) 1.8e+02 _dronez_vector) (LocalVariables|GetInvert?))) (Variables|DroneInternals|GetActors%20to%20Ignore) (Variables|DroneSetup|GetDebugMode?) "(R=1.000000,G=0.000000,B=0.000000,A=1.000000)"))
    (LocalVariables|SetH _bloking_)
    (Variables|DroneInfo|SetAxisRight (Math|Float|SelectFloat (CallFunction|Invert (Math|Float|MapRangeClamped _distance 0.0 (Variables|DroneSetup|GetDroneY_AxisOffset) 1.0 0.5)) (Math|Float|MapRangeClamped _distance 0.0 (Variables|DroneSetup|GetDroneY_AxisOffset) 1.0 0.5) (LocalVariables|GetInvert?)))
    (if (LocalVariables|GetH)
      (return (LocalVariables|GetH))))
  (return (LocalVariables|GetH)))

(fn Teleport
  (bind _targetlocation (Variables|DroneInternals|GetTargetLocation))
  (bind (_x _y _z) (Math|Vector|BreakVector _targetlocation))
  (Transformation|Teleport (Variables|DroneReferences|GetDrone) (Math|Vector|MakeVector _x _y (+ _z (Variables|DroneSetup|GetTargetUpOffset))) "0, 0, 0")
  (Variables|DroneInfo|SetAxisForward 0.0)
  (Variables|DroneInfo|SetAxisRight 0.0)
  (Variables|DroneInfo|SetAxisUp 0.0)
  (Utilities|Time|ClearandInvalidateTimerbyHandle (Variables|DroneInternals|GetTeleportTimerHandle))
  (Development|PrintString "Teleporting" (Variables|DroneSetup|GetDebugMode?) true "(R=1.000000,G=0.883787,B=0.000000,A=1.000000)" :!pinned true) ; DEBUG_NODE
)

(fn DroneAltitude
  (bind _acceptanceradius (Variables|DroneSetup|GetAcceptanceRadius))
  (bind _hit_ (DroneMovement|DroneAltitudTrace))
  (if (not _hit_)
    (LocalVariables|SetpDroneZ_Location (.z (Variables|DroneInternals|GetDroneLocation)))
    (LocalVariables|SetpMinAlt (+ (.z (Variables|DroneInternals|GetTargetLocationS)) (Math|Float|Clamp(Float) (- _acceptanceradius (Variables|DroneSetup|GetRadiusVariation)) 5e+01 _acceptanceradius)))
    (LocalVariables|SetpMaxAlt (Variables|DroneSetup|GetAcceptanceRadius))
    (LocalVariables|SetpAxis (Math|Float|MapRangeClamped (Math|Float|Absolute(Float) (- (LocalVariables|GetpDroneZ_Location) (LocalVariables|GetpMinAlt))) 0.0 1.5e+02 0.0 1.0))
    (if (< (LocalVariables|GetpDroneZ_Location) (LocalVariables|GetpMinAlt))
      (Variables|DroneInfo|SetAxisUp (LocalVariables|GetpAxis))
      (elif (> (LocalVariables|GetpDroneZ_Location) (LocalVariables|GetpMaxAlt))
        (Variables|DroneInfo|SetAxisUp (CallFunction|Invert (LocalVariables|GetpAxis)))
        (else
          (Variables|DroneInfo|SetAxisUp 0.0))))))

(fn TrytoFind
  (bind _lookatrotyaw (Variables|DroneInternals|GetLookAtRotYaw))
  (bind _returnvalue (Math|Float|Absolute(Float) _lookatrotyaw))
  (bind _returnvalue_2 (Math|Float|MapRangeClamped _returnvalue 1e+01 9e+01 0.0 1.0))
  (if (or (Variables|DroneInternals|GetUpHit?) (Variables|DroneInternals|GetForwardHit?))
    (LocalVariables|SetpDronZ_Location (.z (Variables|DroneInternals|GetDroneLocation)))
    (LocalVariables|SetpTargetZ_Location (.z (Variables|DroneInternals|GetTargetLocationS)))
    (LocalVariables|SetpDiference (- (LocalVariables|GetpDronZ_Location) (LocalVariables|GetpTargetZ_Location)))
    (if (> (LocalVariables|GetpDronZ_Location) (LocalVariables|GetpTargetZ_Location))
      (Variables|DroneInfo|SetAxisUp (Math|Float|MapRangeClamped (LocalVariables|GetpDiference) 1e+02 0.0 -1.0 0.0))
      (if (> _lookatrotyaw 0.0) :!label _label
        (Variables|DroneInfo|SetAxisRight _returnvalue_2)
        (else
          (Variables|DroneInfo|SetAxisRight (CallFunction|Invert _returnvalue_2))))
      (elif (< (LocalVariables|GetpDronZ_Location) (LocalVariables|GetpTargetZ_Location))
        (Variables|DroneInfo|SetAxisUp (Math|Float|MapRangeClamped (Math|Float|Absolute(Float) (LocalVariables|GetpDiference)) 1e+02 0.0 1.0 0.0))
        (goto _label)
        (else
          (Variables|DroneInfo|SetAxisUp 0.0))))))

(fn DroneAltitudTrace
  (bind _dronelocation (Variables|DroneInternals|GetDroneLocation))
  (bind _dronez_axisoffset (Variables|DroneSetup|GetDroneZ_AxisOffset))
  (bind _dronez_vector (Variables|DroneInternals|GetDroneZ_Vector))
  (bind _returnvalue (* _dronez_vector _dronez_axisoffset))
  (for _index (range 0 1)
    (LocalVariables|SetInvert? (> _index 0))
    (bind (_bloking_ _distance) (CallFunction|Trace _dronelocation (Math|Vector|SelectVector (+ _dronelocation _returnvalue) (- _dronelocation _returnvalue) (not (LocalVariables|GetInvert?))) (Variables|DroneInternals|GetActors%20to%20Ignore) (Variables|DroneSetup|GetDebugMode?) "(R=0.000000,G=0.250000,B=1.000000,A=1.000000)"))
    (LocalVariables|SetH _bloking_)
    (Variables|DroneInfo|SetAxisUp (Math|Float|SelectFloat (CallFunction|Invert (Math|Float|MapRangeClamped _distance 0.0 (Variables|DroneSetup|GetDroneZ_AxisOffset) -1.0 0.0)) (Math|Float|MapRangeClamped _distance 0.0 (Variables|DroneSetup|GetDroneZ_AxisOffset) -1.0 0.0) (LocalVariables|GetInvert?)))
    (if (LocalVariables|GetH)
      (return (LocalVariables|GetH))))
  (bind _output_get (Variables|DroneInternals|SetUpHit? (LocalVariables|GetH)))
  (return _output_get))

(fn DynamicSpeed
  (bind _ownermaxspeed_ (Variables|DroneSetup|GetOwnerMaxSpeed?))
  (Variables|DroneInfo|SetDynamicDroneSpeed (Math|Float|MapRangeClamped (Variables|DroneInfo|GetCurrentDistanceTarget) (Variables|DroneSetup|GetAcceptanceRadius) _ownermaxspeed_ _ownermaxspeed_ (Variables|DroneSetup|GetDroneMaxSpeed))))

(fn DroneForwardMovement
  (bind (_distance _hit) (DroneMovement|DroneForwardTrace))
  (Variables|DroneInfo|SetAxisForward (Math|Float|SelectFloat (Math|Float|MapRangeClamped _distance (Variables|DroneInternals|GetFwTraceLenght) 0.0 1.0 0.25) (Math|Float|MapRangeClamped (Variables|DroneInfo|GetCurrentDistanceTarget) (Variables|DroneSetup|GetAcceptanceRadius) (Variables|DroneSetup|GetMaxDistanceToSpeed) 0.0 1.0) _hit))
  (if (not (Variables|DroneInternals|GetCloseToTarget?))
    (Variables|DroneInternals|SetIdleDelay? false)
    (Variables|DroneInternals|SetIdleTimeCounter 0.0)
    (Variables|DroneInternals|SetIdleSelector -1)
    (if (Variables|DroneInternals|GetNeedTeleport?)
      (DroneMovement|Teleport))))

(fn TargetDistance
  (bind _acceptanceradius (Variables|DroneSetup|GetAcceptanceRadius))
  (bind _output_get (Variables|DroneInfo|SetCurrentDistanceTarget (Transformation|GetDistanceTo (Variables|DroneReferences|GetDrone) (Variables|DroneInternals|GetTarget))))
  (Variables|DroneInternals|SetCloseToTarget? (<= _output_get (+ _acceptanceradius 1.0)))
  (Variables|DroneInternals|SetPredictLocation (< _output_get (* _acceptanceradius (Variables|DroneSetup|GetPredictLocationImportance))))
  (Variables|DroneInternals|SetNeedTeleport? (> _output_get (Variables|DroneSetup|GetTargetDistanceTeleport)))
  (Variables|DroneInternals|SetCanDoSkill? (< _output_get (Variables|DroneSkillsInternals|GetSkillDistance)))
  (Variables|DroneInternals|SetOwnerTooFar? (> (Transformation|GetDistanceTo (Variables|DroneReferences|GetDrone) (Variables|DroneInternals|GetTarget)) (Variables|DroneSetup|GetOwnerDistanceTeleport))))

(fn ActorsLocation
  (bind _drone (Variables|DroneReferences|GetDrone))
  (bind _target (Variables|DroneInternals|GetTarget))
  (bind _returnvalue (Transformation|GetActorLocation _target))
  (Variables|DroneInternals|SetTargetLocation _returnvalue)
  (Variables|DroneInternals|SetTargetLocationS (Math|Vector|SelectVector (+ _returnvalue (Transformation|GetVelocity _target)) _returnvalue (Variables|DroneInternals|GetPredictLocation)))
  (Variables|DroneInternals|SetDroneZ_Vector (Transformation|GetActorUpVector _drone))
  (Variables|DroneInternals|SetDroneY_Vector (Transformation|GetActorRightVector _drone))
  (Variables|DroneInternals|SetDroneX_Vector (Transformation|GetActorForwardVector _drone))
  (Variables|DroneInternals|SetDroneRotation (Transformation|GetActorRotation _drone))
  (Variables|DroneInternals|SetDroneLocation (Transformation|GetActorLocation _drone))
  (Variables|DroneInternals|SetOwnerLocation (Transformation|GetActorLocation (Variables|DroneInternals|GetTarget))))