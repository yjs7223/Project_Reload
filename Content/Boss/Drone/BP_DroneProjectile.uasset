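; Projectile for the drone boss that intermittently homes in on a Target actor.
; Speed and gravity are applied to ProjectileMovement in the construction script.
; With a valid Target, BeginPlay ignores the owner for collision, starts a one-second looping timer that alternates homing on and off, and destroys the projectile after ActivateTime.
; Tick eases rotation toward the Target using a fixed interpolation step rather than frame delta time.
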(event Custom|RotateToTarget
  (Transformation|SetActorRotation (Math|Interpolation|RInterpTo (Transformation|GetActorRotation) (Math|Rotator|FindLookatRotation (Transformation|GetActorLocation) (Transformation|GetActorLocation (Variables|Target|GetTarget))) 0.1 0.5)))

(event Custom|SetHomingValid
  (Variables|/Script/Engine.ProjectileMovementComponent|SetbIsHomingProjectile (Variables|Default|GetProjectileMovement) (Variables|ProjectileSettings|GetIsHoming))
  (Variables|ProjectileSettings|SetIsHoming (not (Variables|ProjectileSettings|GetIsHoming))))

(event EventBeginPlay
  (bind _projectilemovement (Variables|Default|GetProjectileMovement))
  (Variables|Target|GetTarget
    (:then
      (if (Variables|ProjectileSettings|GetIsHoming)
        _
        (else
          _))
      (Variables|/Script/Engine.ProjectileMovementComponent|SetbIsHomingProjectile _projectilemovement false)
      (Variables|/Script/Engine.ProjectileMovementComponent|SetHomingTargetComponent _projectilemovement (Variables|/Script/Engine.Actor|GetRootComponent (Variables|Target|GetTarget)))
      (Collision|IgnoreActorwhenMoving (Variables|Default|GetBoxCollision) (Components|GetOwner) true)
      (Utilities|Time|SetTimerbyEvent (delegate Custom|SetHomingValid) 1.0 true)
      (Utilities|FlowControl|Delay (Variables|ProjectileSettings|GetActivateTime))
      (Actor|DestroyActor))
    (:else)))

(event EventTick
  (params (DeltaSeconds :type Float%20%28single-precision%29))
  (CallFunction|RotatetoTarget))

(fn ConstructionScript
  (bind _projectilemovement (Variables|Default|GetProjectileMovement))
  (Variables|/Script/Engine.ProjectileMovementComponent|SetInitialSpeed _projectilemovement (Variables|ProjectileSettings|GetMinSpeed))
  (Variables|/Script/Engine.ProjectileMovementComponent|SetMaxSpeed _projectilemovement (Variables|ProjectileSettings|GetMaxSpeed))
  (Variables|/Script/Engine.ProjectileMovementComponent|SetProjectileGravityScale _projectilemovement (Variables|ProjectileSettings|GetGravity)))