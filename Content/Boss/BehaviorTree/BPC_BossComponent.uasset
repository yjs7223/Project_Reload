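; Boss component that seeds the AI Blackboard of its owning MyBossCharacter1 on BeginPlay.
; It caches the character and AI controller, then sets the boss as SelfActor and the BP_pc_Anim player pawn as TargetActor.
; It records the player's starting XY at boss height as Origin and their distance as Radius, and resets the angle and movement keys, suggesting setup for circling movement.
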(event EventBeginPlay
  (bind _returnvalue (Game|Player|GetPlayerPawn 0))
  (bind _returnvalue_2 (Transformation|GetActorLocation _returnvalue))
  (bind _asmy_boss_character_1 (Utilities|Casting|CastToMyBossCharacter1 (Components|GetOwner)))
  (bind _output_get (Variables|Default|SetCharacterRef _asmy_boss_character_1))
  (bind _output_get_2 (Variables|Default|SetControllerRef (AI|GetAIController _output_get)))
  (Utilities|IsValid _output_get_2
    (:Is%20Valid
      (AI|Components|Blackboard|SetValueasObject (Variables|/Script/AIModule.AIController|GetBlackboard (Variables|Default|GetControllerRef)) (Utilities|Name|MakeLiteralName "SelfActor") (Variables|Default|GetCharacterRef))
      (bind _asbp_player_characteer_2 (Utilities|Casting|CastToBP_pc_Anim (Pawn|GetControlledPawn (Game|GetPlayerController 0))))
      (AI|Components|Blackboard|SetValueasObject (Variables|/Script/AIModule.AIController|GetBlackboard (Variables|Default|GetControllerRef)) (Utilities|Name|MakeLiteralName "TargetActor") _asbp_player_characteer_2)
      (AI|Components|Blackboard|SetValueasVector (Variables|/Script/AIModule.AIController|GetBlackboard (Variables|Default|GetControllerRef)) (Utilities|Name|MakeLiteralName "Origin") (Math|Vector|MakeVector (.x _returnvalue_2) (.y _returnvalue_2) (.z (Transformation|GetActorLocation (Variables|Default|GetCharacterRef)))))
      (AI|Components|Blackboard|SetValueasFloat (Variables|/Script/AIModule.AIController|GetBlackboard (Variables|Default|GetControllerRef)) (Utilities|Name|MakeLiteralName "Radius") (Transformation|GetDistanceTo (Variables|Default|GetCharacterRef) (Game|Player|GetPlayerPawn 0)))
      (AI|Components|Blackboard|SetValueasFloat (Variables|/Script/AIModule.AIController|GetBlackboard (Variables|Default|GetControllerRef)) (Utilities|Name|MakeLiteralName "Angle") 0.0)
      (AI|Components|Blackboard|SetValueasFloat (Variables|/Script/AIModule.AIController|GetBlackboard (Variables|Default|GetControllerRef)) (Utilities|Name|MakeLiteralName "MoveAngle") 0.0)
      (AI|Components|Blackboard|SetValueasBool (Variables|/Script/AIModule.AIController|GetBlackboard (Variables|Default|GetControllerRef)) (Utilities|Name|MakeLiteralName "IsMove") false))))