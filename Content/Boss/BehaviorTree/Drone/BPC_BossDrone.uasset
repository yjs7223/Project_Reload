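; BPC_BossDrone is a component for the boss drone character that initializes its AI Blackboard on BeginPlay.
; It caches the owning drone and its AI controller, then writes the drone as SelfActor and the player's BP_pc_Anim pawn as TargetActor.
; It also seeds starting angle, X/Y radius and IsMoveAround keys, with move-around initially off.
; The file holds no movement logic itself.
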(event EventBeginPlay
  (bind _asmy_boss_drone_character (Utilities|Casting|CastToMyBossDroneCharacter (Components|GetOwner)))
  (bind _output_get (Variables|Default|SetCharacterRef _asmy_boss_drone_character))
  (bind _output_get_2 (Variables|Default|SetControllerRef (AI|GetAIController _output_get)))
  (Utilities|IsValid _output_get_2
    (:Is%20Valid
      (AI|Components|Blackboard|SetValueasObject (Variables|/Script/AIModule.AIController|GetBlackboard (Variables|Default|GetControllerRef)) (Utilities|Name|MakeLiteralName "SelfActor") (Variables|Default|GetCharacterRef))
      (bind _asbp_pc_anim (Utilities|Casting|CastToBP_pc_Anim (Pawn|GetControlledPawn (Game|GetPlayerController 0))))
      (AI|Components|Blackboard|SetValueasObject (Variables|/Script/AIModule.AIController|GetBlackboard (Variables|Default|GetControllerRef)) (Utilities|Name|MakeLiteralName "TargetActor") _asbp_pc_anim)
      (AI|Components|Blackboard|SetValueasFloat (Variables|/Script/AIModule.AIController|GetBlackboard (Variables|Default|GetControllerRef)) (Utilities|Name|MakeLiteralName "Angle") 0.0)
      (AI|Components|Blackboard|SetValueasFloat (Variables|/Script/AIModule.AIController|GetBlackboard (Variables|Default|GetControllerRef)) (Utilities|Name|MakeLiteralName "Radius_X") 45.0)
      (AI|Components|Blackboard|SetValueasFloat (Variables|/Script/AIModule.AIController|GetBlackboard (Variables|Default|GetControllerRef)) (Utilities|Name|MakeLiteralName "Radius_Y") 45.0)
      (AI|Components|Blackboard|SetValueasBool (Variables|/Script/AIModule.AIController|GetBlackboard (Variables|Default|GetControllerRef)) (Utilities|Name|MakeLiteralName "IsMoveAround") false))))