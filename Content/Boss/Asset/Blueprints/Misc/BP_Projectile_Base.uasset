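; Base projectile for boss abilities that deals point damage to actors it overlaps.
; On BeginPlay it takes final damage and damage type from its owning boss ability.
; Sphere overlaps damage each damageable actor once, skipping the instigator and tracking victims in DamagedActors.
; An optional DestroyOnHit flag destroys the projectile after dealing damage or on a blocking hit with anything but the instigator.
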(event OnComponentHit(Sphere)
  (params (HitComponent :type Primitive%20Component%20Object%20Reference) (OtherActor :type Actor%20Object%20Reference) (OtherComp :type Primitive%20Component%20Object%20Reference) (NormalImpulse :type Vector :default "0, 0, 0") (Hit :type Hit%20Result%20Structure%20%28by%20ref%29))
  (if (!= OtherActor (Game|GetInstigator))
    (if (Variables|Default|GetDestroyOnHit)
      (Actor|DestroyActor))))

(event OnComponentBeginOverlap(Sphere)
  (params (OverlappedComponent :type Primitive%20Component%20Object%20Reference) (OtherActor :type Actor%20Object%20Reference) (OtherComp :type Primitive%20Component%20Object%20Reference) (OtherBodyIndex :type Integer) (bFromSweep :type Boolean) (SweepResult :type Hit%20Result%20Structure%20%28by%20ref%29))
  (if (Math|Boolean|ANDBoolean (Variables|/Script/Engine.Actor|GetbCanBeDamaged OtherActor) (!= OtherActor (Game|GetInstigator)) (not (Utilities|Array|ContainsItem (Variables|Default|GetDamagedActors) OtherActor)))
    (Game|Damage|ApplyPointDamage OtherActor (Variables|Default|GetDamage) (Transformation|GetActorLocation) SweepResult 0 (Components|GetOwner) (Variables|Default|GetDamageType))
    (Utilities|Array|AddUnique (Variables|Default|GetDamagedActors) OtherActor)
    (if (Variables|Default|GetDestroyOnHit)
      (Actor|DestroyActor))))

(event EventBeginPlay
  (bind _asbp_boss_ability_base (Utilities|Casting|CastToBP_BossAbility_Base (Components|GetOwner)))
  (Variables|Default|SetDamage (Default|GetFinalDamage _asbp_boss_ability_base))
  (Variables|Default|SetDamageType (.DamageType (Utilities|Struct|BreakF_BossAbilityDamage (.Damage (Utilities|Struct|BreakF_BossAbility (Variables|/Game/BossAIToolkit/Blueprints/Abilities/BP_BossAbility_Base.BP_BossAbility_Base_C|GetAbilityInfo _asbp_boss_ability_base)))))))

(fn ConstructionScript)