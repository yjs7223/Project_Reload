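; Anim notify state that marks the damage window in boss animations.
; On begin and end it finds the owner's BPC_Boss_Behavior component and calls OnBeginDamage, passing the window duration, or OnEndDamage on its current ability.
; The ability handles the damage itself, and the notify returns false when the component or ability is invalid.
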(fn ReceivedNotifyBegin
  (params (MeshComp :type Skeletal%20Mesh%20Component%20Object%20Reference) (Animation :type Anim%20Sequence%20Base%20Object%20Reference) (TotalDuration :type Float%20%28single-precision%29))
  (bind _returnvalue (Components|GetOwner MeshComp))
  (bind _returnvalue_2 (Actor|GetComponentbyClass _returnvalue "/Game/BossAIToolkit/Blueprints/BPC_Boss_Behavior.BPC_Boss_Behavior_C"))
  (bind _currentability (Variables|/Game/BossAIToolkit/Blueprints/BPC_Boss_Behavior.BPC_Boss_Behavior_C|GetCurrentAbility _returnvalue_2))
  (Utilities|IsValid _returnvalue_2
    (:Is%20Valid
      (Utilities|IsValid _currentability
        (:Is%20Valid
          (Default|OnBeginDamage _currentability TotalDuration)
          (return true))
        (:Is%20Not%20Valid
          _)))
    (:Is%20Not%20Valid
      _))
  (return false))

(fn ReceivedNotifyEnd
  (params (MeshComp :type Skeletal%20Mesh%20Component%20Object%20Reference) (Animation :type Anim%20Sequence%20Base%20Object%20Reference))
  (bind _returnvalue (Components|GetOwner MeshComp))
  (bind _returnvalue_2 (Actor|GetComponentbyClass _returnvalue "/Game/BossAIToolkit/Blueprints/BPC_Boss_Behavior.BPC_Boss_Behavior_C"))
  (bind _currentability (Variables|/Game/BossAIToolkit/Blueprints/BPC_Boss_Behavior.BPC_Boss_Behavior_C|GetCurrentAbility _returnvalue_2))
  (Utilities|IsValid _returnvalue_2
    (:Is%20Valid
      (Utilities|IsValid _currentability
        (:Is%20Valid
          (Default|OnEndDamage _currentability)
          (return true))
        (:Is%20Not%20Valid
          _)))
    (:Is%20Not%20Valid
      _))
  (return false))