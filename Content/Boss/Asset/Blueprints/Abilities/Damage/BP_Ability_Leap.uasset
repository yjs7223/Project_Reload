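; Boss leap ability that launches the boss in an arc onto the target's position and deals damage during a damage window.
; A timeline scaled to the execute duration lerps the boss through start, raised midpoint and landing points, with sweep.
; A circle telegraphs the initial landing point, while optional air control retargets the landing during ascent.
; Damage is a radial burst when no hitboxes exist, otherwise per-tick hitbox traces.
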(event EventBeginPlay
  (|CallParentFunction)
  (Variables|Default|SetRadius (.X (Math|Vector|BreakVector (.Modifier (Utilities|Struct|BreakF_BossAbility (Variables|Default|GetAbilityInfo))))))
  (CallFunction|ForceRotateAI (Transformation|GetActorLocation (Variables|Default|GetTargetActor)) 0 false))

(event EventOnBeginDamage
  (params (Duration :type Float%20%28single-precision%29))
  (Variables|Default|SetCanDealDamage true)
  (if (== (Utilities|Array|Length (Variables|Default|GetHitboxes)) 0)
    (CallFunction|ApplyAbilityDamage 0 (Transformation|GetActorLocation (Variables|Default|GetBossRef)) true (Variables|Default|GetRadius) true)
    (CallFunction|RemoveTelegraph)))

(event EventOnEndDamage
  (Variables|Default|SetCanDealDamage false)
  (Utilities|Array|Clear (Variables|Default|GetDamagedActors))
  (CallFunction|ResetRotation))

(event EventTick
  (params (DeltaSeconds :type Float%20%28single-precision%29))
  (if (and (> (Utilities|Array|Length (Variables|Default|GetHitboxes)) 0) (Variables|Default|GetCanDealDamage))
    (bind _outactors (CallFunction|TraceHitbox))
    (for _array_element _outactors
      (CallFunction|ApplyAbilityDamage _array_element (Transformation|GetActorLocation (Variables|Default|GetBossRef)) false 0.0 true))))

(event EventOnExecute
  (params (Duration :type Float%20%28single-precision%29))
  (Components|Timeline|SetPlayRate (Variables|Default|GetLeap_Timeline) (/ 1.0 Duration))
  (Pawn|Components|CharacterMovement|SetMovementMode (Variables|/Script/Engine.Character|GetCharacterMovement (Variables|Default|GetBossRef)) "MOVE_Falling" 0)
  (Variables|Default|SetJumpPointA (Transformation|GetActorLocation (Variables|Default|GetBossRef)))
  (Variables|Default|SetJumpPointC (Transformation|GetActorLocation (Variables|Default|GetTargetActor)))
  (Variables|Default|SetJumpPointB (Math|Vector|MakeVector (.x (Math|Vector|Lerp(Vector) (Variables|Default|GetJumpPointA) (Variables|Default|GetJumpPointC) 0.5)) (.y (Math|Vector|Lerp(Vector) (Variables|Default|GetJumpPointA) (Variables|Default|GetJumpPointC) 0.5)) (+ (Math|Float|Max(Float) (.Z (Math|Vector|BreakVector (Variables|Default|GetJumpPointA))) (.Z (Math|Vector|BreakVector (Variables|Default|GetJumpPointC)))) 5e+02)))
  (CallFunction|TelegraphCircle (Variables|Default|GetRadius) (Variables|Default|GetJumpPointC))
  (bind (_direction _alpha1 _alpha2 _alpha3) (Timeline|Leap_Timeline PlayFromStart)
    (:Update
      (Transformation|SetActorLocation (Variables|Default|GetBossRef) (Math|Vector|MakeVector (.x (Math|Vector|Lerp(Vector) (Variables|Default|GetJumpPointA) (Variables|Default|GetJumpPointC) _alpha3)) (.y (Math|Vector|Lerp(Vector) (Variables|Default|GetJumpPointA) (Variables|Default|GetJumpPointC) _alpha3)) (.z (select (>= _alpha1 1.0) (Math|Vector|Lerp(Vector) (Variables|Default|GetJumpPointC) (Variables|Default|GetJumpPointB) _alpha2) (Math|Vector|Lerp(Vector) (Variables|Default|GetJumpPointA) (Variables|Default|GetJumpPointB) _alpha1)))) true false)
      (if (>= _alpha1 1.0)
        (CallFunction|ResetRotation)
        (elif (Variables|Default|GetAirControl)
          (Variables|Default|SetJumpPointC (Transformation|GetActorLocation (Variables|Default|GetTargetActor))))))))

(fn ConstructionScript
  (|CallParentFunction))