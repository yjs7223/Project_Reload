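; Boss ability Blueprint that deals damage through a traced hitbox during a damage window.
; On BeginPlay it force-rotates the AI toward the target actor's location.
; While the OnBeginDamage to OnEndDamage window is open, Tick traces the hitbox every frame and applies ability damage to each returned actor, with the boss's location as origin.
; Closing the window clears the damaged-actor list and resets rotation.
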(event EventBeginPlay
  (|CallParentFunction)
  (CallFunction|ForceRotateAI (Transformation|GetActorLocation (Variables|Default|GetTargetActor)) 0 false))

(event EventOnBeginDamage
  (params (Duration :type Float%20%28single-precision%29))
  (Variables|Default|SetCanDealDamage true))

(event EventOnEndDamage
  (Variables|Default|SetCanDealDamage false)
  (Utilities|Array|Clear (Variables|Default|GetDamagedActors))
  (CallFunction|ResetRotation))

(event EventTick
  (params (DeltaSeconds :type Float%20%28single-precision%29))
  (if (Variables|Default|GetCanDealDamage)
    (bind _outactors (CallFunction|TraceHitbox))
    (for _array_element _outactors
      (CallFunction|ApplyAbilityDamage _array_element (Transformation|GetActorLocation (Variables|Default|GetBossRef)) false 0.0 true))))

(fn ConstructionScript
  (|CallParentFunction))