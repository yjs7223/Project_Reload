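; Boss actor component that seeds the AI Blackboard for a behavior-tree boss built on CrunchPlayerCharacter1, stored under a BehaviorTreeNotUse folder.
; On BeginPlay it caches the owning character and its AI controller, then writes initial self, HP, attack range, skill, phase, dash and walk-speed keys.
; The target is player 0's BP_pc_Anim pawn; a failed cast stops setup, leaving the target and later keys unset.
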(event EventBeginPlay
  (bind _ascrunch_player_character_1 (Utilities|Casting|CastToCrunchPlayerCharacter1 (Components|GetOwner)))
  (bind _output_get (Variables|Default|SetCharacterRef _ascrunch_player_character_1))
  (bind _output_get_2 (Variables|Default|SetControllerRef (AI|GetAIController _output_get)))
  (Utilities|IsValid _output_get_2
    (:Is%20Valid
      (AI|Components|Blackboard|SetValueasObject (Variables|/Script/AIModule.AIController|GetBlackboard (Variables|Default|GetControllerRef)) (Utilities|Name|MakeLiteralName "SelfActor") (Variables|Default|GetCharacterRef))
      (AI|Components|Blackboard|SetValueasFloat (Variables|/Script/AIModule.AIController|GetBlackboard (Variables|Default|GetControllerRef)) (Utilities|Name|MakeLiteralName "Boss_HP") (Variables|Default|GetBossHP))
      (AI|Components|Blackboard|SetValueasFloat (Variables|/Script/AIModule.AIController|GetBlackboard (Variables|Default|GetControllerRef)) (Utilities|Name|MakeLiteralName "Atk_Range") (Variables|Default|GetAtkRange))
      (bind _asbp_pc_anim (Utilities|Casting|CastToBP_pc_Anim (Pawn|GetControlledPawn (Game|GetPlayerController 0))))
      (AI|Components|Blackboard|SetValueasObject (Variables|/Script/AIModule.AIController|GetBlackboard (Variables|Default|GetControllerRef)) (Utilities|Name|MakeLiteralName "TargetActor") _asbp_pc_anim)
      (AI|Components|Blackboard|SetValueasBool (Variables|/Script/AIModule.AIController|GetBlackboard (Variables|Default|GetControllerRef)) (Utilities|Name|MakeLiteralName "Has_Skill") true)
      (Class|BlackboardComponent|SetValueasInt (Variables|/Script/AIModule.AIController|GetBlackboard (Variables|Default|GetControllerRef)) (Utilities|Name|MakeLiteralName "Phase"))
      (AI|Components|Blackboard|SetValueasBool (Variables|/Script/AIModule.AIController|GetBlackboard (Variables|Default|GetControllerRef)) (Utilities|Name|MakeLiteralName "NeedDash") false)
      (AI|Components|Blackboard|SetValueasFloat (Variables|/Script/AIModule.AIController|GetBlackboard (Variables|Default|GetControllerRef)) (Utilities|Name|MakeLiteralName "MaxWalkSpeed") (Variables|/Script/Engine.CharacterMovementComponent|GetMaxWalkSpeed (Variables|/Script/Engine.Character|GetCharacterMovement _ascrunch_player_character_1))))))