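; BP_DroneCircle is a boss ability actor that acts as an explosion hazard with a spherical hitbox.
; On BeginPlay it arms damage and spawns the rocket-attack explosion and aftermath Niagara effects with a sound at its location.
; Once armed, an overlap on the sphere deals the boss weapon's maximum damage if the other actor has a StatComponent.
; The actor then destroys itself, whether or not damage was applied.
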(event OnComponentBeginOverlap(Hitbox_Sphere)
  (params (OverlappedComponent :type Primitive%20Component%20Object%20Reference) (OtherActor :type Actor%20Object%20Reference) (OtherComp :type Primitive%20Component%20Object%20Reference) (OtherBodyIndex :type Integer) (bFromSweep :type Boolean) (SweepResult :type Hit%20Result%20Structure%20%28by%20ref%29))
  (if (Variables|Default|GetIsDamage)
    (CallFunction|TakeDamage OtherActor)
    (Actor|DestroyActor)))

(event Custom|Take%20Damage
  (params (Other%20Actor :type Actor%20Object%20Reference))
  (bind _bossweapon (Variables|Default|GetBossWeapon))
  (if (Utilities|IsValid (Actor|GetComponentbyClass Other%20Actor "/Script/BaseClassModule.StatComponent"))
    (Class|BossWeaponComponent|TakeDamage _bossweapon Other%20Actor (Variables|/Script/BossModule.BossWeaponComponent|Getboss_MaxDmg _bossweapon))))

(event EventBeginPlay
  (bind _returnvalue (Transformation|GetActorLocation))
  (Variables|Default|SetIsDamage true)
  (Niagara|SpawnSystematLocation "/Game/RocketAttackFX/FX/Handheld/NS_RocketAttack_Explosion.NS_RocketAttack_Explosion" _returnvalue)
  (Niagara|SpawnSystematLocation "/Game/RocketAttackFX/FX/Handheld/NS_RocketAttack_Aftermath.NS_RocketAttack_Aftermath" _returnvalue)
  (Audio|PlaySoundatLocation "/Game/ExplosionSoundPack/ExplosionSoundsMONO/Wavs/explosion_large_07.explosion_large_07" _returnvalue "0, 0, 0" 1.0 1.0 0.0 0 0 0 0))

(fn ConstructionScript)