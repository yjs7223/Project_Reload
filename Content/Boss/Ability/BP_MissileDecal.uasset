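; Boss missile attack ground decal that telegraphs an impact zone, then explodes and destroys itself.
; BeginPlay creates dynamic materials for the outline and area decals, then a timeline animates the area's AreaValue.
; When the timeline finishes, it spawns Niagara explosion and aftermath effects with sound.
; A TakeDamage event forwards boss max damage to non-owner actors with a StatComponent, but its overlap-driven call is disconnected.
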(event OnComponentEndOverlap(Hitbox_Sphere)
  (params (OverlappedComponent :type Primitive%20Component%20Object%20Reference) (OtherActor :type Actor%20Object%20Reference) (OtherComp :type Primitive%20Component%20Object%20Reference) (OtherBodyIndex :type Integer)))

(event Custom|Take%20Damage
  (params (Other%20Actor :type Actor%20Object%20Reference))
  (bind _bossweapon (Variables|Default|GetBossWeapon))
  (if (and (!= Other%20Actor (Variables|Default|GetOwnerActor)) (Utilities|IsValid (Actor|GetComponentbyClass Other%20Actor "/Script/BaseClassModule.StatComponent")))
    (Class|BossWeaponComponent|TakeDamage _bossweapon Other%20Actor (Variables|/Script/BossModule.BossWeaponComponent|Getboss_MaxDmg _bossweapon))))

(event EventBeginPlay
  (bind _returnvalue (Transformation|GetActorLocation))
  (Variables|Default|SetIsDamage false)
  (Utilities|FlowControl|Sequence
    (:then_0
      (bind _returnvalue_2 (Rendering|Material|CreateDynamicMaterialInstance (Variables|Default|GetCircum) :!class /Script/Engine.DecalComponent))
      (bind _output_get (Variables|Default|SetCircumRef _returnvalue_2))
      (Rendering|Material|SetScalarParameterValue _output_get "Circum1Area0" 1.0 :!class /Script/Engine.MaterialInstanceDynamic))
    (:then_1
      (bind _returnvalue_3 (Rendering|Material|CreateDynamicMaterialInstance (Variables|Default|GetArea) :!class /Script/Engine.DecalComponent))
      (bind _output_get_2 (Variables|Default|SetAreaRef _returnvalue_3))
      (Rendering|Material|SetScalarParameterValue _output_get_2 "Circum1Area0" 0.0 :!class /Script/Engine.MaterialInstanceDynamic))
    (:then_2
      (Utilities|FlowControl|Delay 0.1)
      (bind _areavaluealpha (Timeline|AreaValueTimeline Play)
        (:Update
          (Rendering|Material|SetScalarParameterValue (Variables|Default|GetAreaRef) "AreaValue" _areavaluealpha :!class /Script/Engine.MaterialInstanceDynamic))
        (:Finished
          (Utilities|FlowControl|Delay 0.1)
          (Niagara|SpawnSystematLocation "/Game/RocketAttackFX/FX/Handheld/NS_RocketAttack_Explosion.NS_RocketAttack_Explosion" _returnvalue "0, 0, 0" "5.000000,5.000000,5.000000")
          (Niagara|SpawnSystematLocation "/Game/RocketAttackFX/FX/Handheld/NS_RocketAttack_Aftermath.NS_RocketAttack_Aftermath" _returnvalue "0, 0, 0" "5.000000,5.000000,5.000000")
          (Audio|PlaySoundatLocation "/Game/ExplosionSoundPack/ExplosionSoundsMONO/Wavs/explosion_large_07.explosion_large_07" _returnvalue "0, 0, 0" 1.0 1.0 0.0 0 0 0 0)
          (Variables|Default|SetIsDamage true)
          (Actor|DestroyActor))))))

(fn ConstructionScript)