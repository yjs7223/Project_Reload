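; Boss ability actor that shows a circular area telegraph, then destroys itself.
; BeginPlay creates dynamic materials for the outline and area, then a timeline animates the area's AreaValue before destruction.
; Hitbox end overlap deals the boss weapon's max damage to non-owner actors with a StatComponent, gated by IsDamage.
; The explosion effects, sound and code setting IsDamage true are disconnected, so the graph never enables damage.
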(event OnComponentEndOverlap(Hitbox_Sphere)
  (params (OverlappedComponent :type Primitive%20Component%20Object%20Reference) (OtherActor :type Actor%20Object%20Reference) (OtherComp :type Primitive%20Component%20Object%20Reference) (OtherBodyIndex :type Integer))
  (if (Variables|Default|GetIsDamage)
    (CallFunction|TakeDamage OtherActor)))

(event Custom|Take%20Damage
  (params (Other%20Actor :type Actor%20Object%20Reference))
  (bind _bossweapon (Variables|Default|GetBossWeapon))
  (if (and (!= Other%20Actor (Variables|Default|GetOwnerActor)) (Utilities|IsValid (Actor|GetComponentbyClass Other%20Actor "/Script/BaseClassModule.StatComponent")))
    (Class|BossWeaponComponent|TakeDamage _bossweapon Other%20Actor (Variables|/Script/BossModule.BossWeaponComponent|Getboss_MaxDmg _bossweapon))))

(event EventBeginPlay
  (Variables|Default|SetIsDamage false)
  (Utilities|FlowControl|Sequence
    (:then_0
      (bind _returnvalue (Rendering|Material|CreateDynamicMaterialInstance (Variables|Default|GetCircum) :!class /Script/Engine.DecalComponent))
      (bind _output_get (Variables|Default|SetCircumRef _returnvalue))
      (Rendering|Material|SetScalarParameterValue _output_get "Circum1Area0" 1.0 :!class /Script/Engine.MaterialInstanceDynamic))
    (:then_1
      (bind _returnvalue_2 (Rendering|Material|CreateDynamicMaterialInstance (Variables|Default|GetArea) :!class /Script/Engine.DecalComponent))
      (bind _output_get_2 (Variables|Default|SetAreaRef _returnvalue_2))
      (Rendering|Material|SetScalarParameterValue _output_get_2 "Circum1Area0" 0.0 :!class /Script/Engine.MaterialInstanceDynamic))
    (:then_2
      (Utilities|FlowControl|Delay 0.1)
      (bind _areavaluealpha (Timeline|AreaValueTimeline Play)
        (:Update
          (Rendering|Material|SetScalarParameterValue (Variables|Default|GetAreaRef) "AreaValue" _areavaluealpha :!class /Script/Engine.MaterialInstanceDynamic))
        (:Finished
          (Utilities|FlowControl|Delay 0.1)
          (Actor|DestroyActor))))))

(fn ConstructionScript)