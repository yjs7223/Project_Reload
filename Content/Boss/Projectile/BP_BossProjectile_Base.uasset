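; Base boss projectile that can briefly home in on a target and explodes on impact.
; With IsHoming and a valid target, it waits a second, homes and turns toward the target for about 1.5 seconds, then follows its velocity, self-destructing after six seconds.
; Hits fire the impact call, effect and sound, then an empty TakeDamage event before destruction.
; The construction script applies speed and gravity settings to the movement component.
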(event OnComponentHit(BoxCollision)
  (params (HitComponent :type Primitive%20Component%20Object%20Reference) (OtherActor :type Actor%20Object%20Reference) (OtherComp :type Primitive%20Component%20Object%20Reference) (NormalImpulse :type Vector :default "0, 0, 0") (Hit :type Hit%20Result%20Structure%20%28by%20ref%29))
  (bind _location (Collision|BreakHitResult Hit))
  (Default|CallOnProjectileImpact OtherActor Hit)
  (Effects|SpawnEmitteratLocation (Variables|Effects|GetImpact%20Effect) _location)
  (Audio|PlaySoundatLocation (Variables|Sounds|GetImpact%20Sound) _location "0, 0, 0" 1.0 1.0 0.0 0 0 0 0)
  (CallFunction|TakeDamage OtherActor)
  (Actor|DestroyActor))

(event Custom|Take%20Damage
  (params (Other%20Actor :type Actor%20Object%20Reference)))

(event Custom|RotateToTarget
  (Transformation|SetActorRotation (Math|Interpolation|RInterpTo (Transformation|GetActorRotation) (Math|Rotator|FindLookatRotation (Transformation|GetActorLocation) (Transformation|GetActorLocation (Variables|Target|GetTarget))) 0.1 0.5)))

(event EventBeginPlay
  (bind _projectilemovement (Variables|Default|GetProjectileMovement))
  (Variables|Target|GetTarget
    (:then
      (if (Variables|ProjectileSettings|GetIsHoming)
        (Variables|/Script/Engine.ProjectileMovementComponent|SetbIsHomingProjectile _projectilemovement false)
        (Variables|/Script/Engine.ProjectileMovementComponent|SetHomingTargetComponent _projectilemovement (Variables|/Script/Engine.Actor|GetRootComponent (Variables|Target|GetTarget)))
        (Collision|IgnoreActorwhenMoving (Variables|Default|GetBoxCollision) (Components|GetOwner) true)
        (Utilities|FlowControl|Delay 1.0)
        (Variables|Default|SetHoming true)
        (Utilities|FlowControl|Delay 5.0)
        (Actor|DestroyActor)))
    (:else)))

(event EventTick
  (params (DeltaSeconds :type Float%20%28single-precision%29))
  (bind _projectilemovement (Variables|Default|GetProjectileMovement))
  (if (Variables|Default|GetHoming)
    (Variables|Target|GetTarget
      (:then
        (Variables|/Script/Engine.ProjectileMovementComponent|SetbIsHomingProjectile (Variables|Default|GetProjectileMovement) true)
        (CallFunction|RotatetoTarget)
        (Utilities|FlowControl|Delay 1.5)
        (Variables|Default|SetHoming false))
      (:else))
    (else
      (Variables|/Script/Engine.ProjectileMovementComponent|SetbIsHomingProjectile _projectilemovement false)
      (Transformation|SetActorRotation (Math|Interpolation|RInterpTo (Transformation|GetActorRotation) (Math|Rotator|MakeRotfromX (Variables|/Script/Engine.MovementComponent|GetVelocity _projectilemovement)) 0.1 0.5)))))

(fn ConstructionScript
  (bind _projectilemovement (Variables|Default|GetProjectileMovement))
  (Variables|/Script/Engine.ProjectileMovementComponent|SetInitialSpeed _projectilemovement (Variables|ProjectileSettings|GetMinSpeed))
  (Variables|/Script/Engine.ProjectileMovementComponent|SetMaxSpeed _projectilemovement (Variables|ProjectileSettings|GetMaxSpeed))
  (Variables|/Script/Engine.ProjectileMovementComponent|SetProjectileGravityScale _projectilemovement (Variables|ProjectileSettings|GetGravity)))