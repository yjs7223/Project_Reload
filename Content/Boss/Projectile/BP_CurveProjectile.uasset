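; Boss missile that flies a randomized curved path toward its target, then homes in on it.
; A random offset control point slides toward the target location while the missile chases it via VInterpToConstant, bending the path.
; Near that location or after a timer, homing turns on and Tick also interpolates toward the target actor.
; It explodes with boss data-asset FX on hit, damaging StatComponents, or on death, and expires on a timer.
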(event OnComponentHit(SphereCollider)
  (params (HitComponent :type Primitive%20Component%20Object%20Reference) (OtherActor :type Actor%20Object%20Reference) (OtherComp :type Primitive%20Component%20Object%20Reference) (NormalImpulse :type Vector :default "0, 0, 0") (Hit :type Hit%20Result%20Structure%20%28by%20ref%29))
  (bind (_bblockinghit _binitialoverlap _time _distance _location _impactpoint _normal _impactnormal) (Collision|BreakHitResult Hit))
  (bind _returnvalue (Actor|GetComponentbyClass OtherActor "/Script/BaseClassModule.StatComponent"))
  (Effects|SpawnEmitteratLocation (Variables|/Script/BossModule.BossDataAsset|GetMissileExplodeParticle (Variables|/Game/Boss/MyBossCharacter1.MyBossCharacter1_C|GetBoss%20DA (Variables|Default|GetBoss%20Ref))) _location "0, 0, 0" (Variables|Default|GetParticle%20Scale))
  (Audio|PlaySoundatLocation (Variables|/Script/BossModule.BossDataAsset|GetMissileExplodeSound (Variables|/Game/Boss/MyBossCharacter1.MyBossCharacter1_C|GetBoss%20DA (Variables|Default|GetBoss%20Ref))) _location "0, 0, 0" 1.0 1.0 0.0 0 0 0 0)
  (if (Utilities|IsValid _returnvalue)
    (Class|StatComponent|AttackedBP _returnvalue 5.0 (Variables|Default|GetBoss%20Ref) "Normal" _impactnormal)
    (Actor|DestroyActor)
    (else
      (Actor|DestroyActor))))

(event Custom|RotateToTarget
  (Transformation|SetActorRotation (Math|Interpolation|RInterpTo (Transformation|GetActorRotation) (Math|Rotator|FindLookatRotation (Transformation|GetActorLocation) (Transformation|GetActorLocation (Game|Player|GetPlayerPawn 0))) 0.1 0.0)))

(event EventBeginPlay
  (bind _projectilemovement (Variables|Default|GetProjectileMovement))
  (Utilities|Time|SetTimerbyFunctionName 0 "Homing Bullet" 5.0)
  (Utilities|Time|SetTimerbyFunctionName 0 "Destroy Bullet" 2e+01)
  (Variables|/Script/Engine.ProjectileMovementComponent|SetbIsHomingProjectile _projectilemovement false)
  (Variables|/Script/Engine.ProjectileMovementComponent|SetHomingTargetComponent _projectilemovement (Variables|/Script/Engine.Actor|GetRootComponent (Variables|Default|GetTarget)))
  (Collision|IgnoreActorwhenMoving (Variables|Default|GetSphere%20Collider) (Components|GetOwner) true)
  (Utilities|FlowControl|Delay 0.01)
  (CallFunction|MidPointCalculator)
  (CallFunction|CurveControlPoint)
  (Components|Activation|Activate (Variables|Default|GetParticle%20Trail) false)
  (Utilities|FlowControl|Gate true) ; enters at Open
)

(event EventTick
  (params (DeltaSeconds :type Float%20%28single-precision%29))
  (bind _self self)
  (bind _returnvalue (Transformation|GetActorLocation _self))
  (if (Variables|/Script/Engine.ProjectileMovementComponent|GetbIsHomingProjectile (Variables|Default|GetProjectileMovement))
    (Transformation|SetActorLocation (Math|Interpolation|VInterptoConstant (Transformation|GetActorLocation) (Transformation|GetActorLocation (Variables|Default|GetTarget)) (Utilities|Time|GetWorldDeltaSeconds) (Variables|Default|GetProjectile%20speed)) false false))
  (CallFunction|RotatetoTarget)
  (if (Variables|/Script/BaseClassModule.StatComponent|GetbDie (Variables|Default|GetStat))
    (Effects|SpawnEmitteratLocation (Variables|/Script/BossModule.BossDataAsset|GetMissileExplodeParticle (Variables|/Game/Boss/MyBossCharacter1.MyBossCharacter1_C|GetBoss%20DA (Variables|Default|GetBoss%20Ref))) _returnvalue "0, 0, 0" (Variables|Default|GetParticle%20Scale))
    (Audio|PlaySoundatLocation (Variables|/Script/BossModule.BossDataAsset|GetMissileExplodeSound (Variables|/Game/Boss/MyBossCharacter1.MyBossCharacter1_C|GetBoss%20DA (Variables|Default|GetBoss%20Ref))) _returnvalue "0, 0, 0" 1.0 1.0 0.0 0 0 0 0)
    (Actor|DestroyActor)
    (else
      (Utilities|FlowControl|Gate true
        (:Exit
          (if (Utilities|Operators|NotEqual(!=) (Transformation|GetActorLocation) (Variables|Default|GetTarget%20Location) 1.5e+03)
            (Variables|Default|SetCurved%20Point (Math|Interpolation|VInterptoConstant (Variables|Default|GetCurved%20Point) (Variables|Default|GetTarget%20Location) (Utilities|Time|GetWorldDeltaSeconds) (Variables|Default|GetProjectile%20speed)))
            (Transformation|SetActorLocation (Math|Interpolation|VInterptoConstant (Transformation|GetActorLocation) (Variables|Default|GetCurved%20Point) (Utilities|Time|GetWorldDeltaSeconds) (Variables|Default|GetProjectile%20speed)) false false)
            (else
              (Variables|/Script/Engine.ProjectileMovementComponent|SetbIsHomingProjectile (Variables|Default|GetProjectileMovement) true))))))))

(fn ConstructionScript
  (Class|NiagaraComponent|SetAsset (Variables|Default|GetParticle%20Trail) (Variables|/Script/BossModule.BossDataAsset|GetMissileTrailFXNiagara (Variables|/Game/Boss/MyBossCharacter1.MyBossCharacter1_C|GetBoss%20DA (Variables|Default|GetBoss%20Ref))) true))

(fn MidPointCalculator
  (Variables|Default|SetMid%20Point (+ (* (- (Variables|Default|GetTarget%20Location) (Transformation|GetActorLocation)) (Math|Random|RandomFloatinRange (Variables|Default|GetMin%20Curve%20Point%20Distance) (Variables|Default|GetMax%20Curve%20Point%20Distance))) (Transformation|GetActorLocation))))

(fn CurveControlPoint
  (bind _mid_point (Variables|Default|GetMid%20Point))
  (bind _target_location (Variables|Default|GetTarget%20Location))
  (bind _returnvalue (Math|Rotator|FindLookatRotation _mid_point _target_location))
  (bind (_x _y) (Math|Rotator|BreakRotIntoAxes _returnvalue))
  (Variables|Default|SetCurved%20Point (+ (Variables|Default|GetMid%20Point) (Math|Vector|RotateVectorAroundAxis (* (Math|Random|RandomFloatinRange (Variables|Default|GetMin%20Curve%20Radius) (Variables|Default|GetMax%20Curve%20Radius)) _y) (Math|Random|RandomFloatinRange (Variables|Default|GetMin%20Angle) (Variables|Default|GetMax%20Angle)) _x))))

(fn DestroyBullet
  (Actor|DestroyActor))

(fn HomingBullet
  (Variables|/Script/Engine.ProjectileMovementComponent|SetbIsHomingProjectile (Variables|Default|GetProjectileMovement) true))