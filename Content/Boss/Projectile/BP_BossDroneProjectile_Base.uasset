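; Base projectile for boss drones that damages through StatComponent and destroys itself on impact.
; Construction applies speed and gravity; BeginPlay, given a valid Target, sets homing, ignores its owner and starts a five-second lifetime.
; Tick traces between previous and current positions to catch hits, skipping DroneRef and damaging only Player-tagged actors.
; Box collision hits fire an impact call, play effect and sound, and damage any actor with a StatComponent.
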(event OnComponentHit(BoxCollision)
  (params (HitComponent :type Primitive%20Component%20Object%20Reference) (OtherActor :type Actor%20Object%20Reference) (OtherComp :type Primitive%20Component%20Object%20Reference) (NormalImpulse :type Vector :default "0, 0, 0") (Hit :type Hit%20Result%20Structure%20%28by%20ref%29))
  (bind (_bblockinghit _binitialoverlap _time _distance _location _impactpoint _normal _impactnormal) (Collision|BreakHitResult Hit))
  (bind _returnvalue (Actor|GetComponentbyClass OtherActor "/Script/BaseClassModule.StatComponent"))
  (Default|CallOnProjectileImpact OtherActor Hit)
  (Effects|SpawnEmitteratLocation (Variables|Effects|GetImpact%20Effect) _location)
  (Audio|PlaySoundatLocation (Variables|Sounds|GetImpact%20Sound) _location "0, 0, 0" 1.0 1.0 0.0 0 0 0 0)
  (if (Utilities|IsValid _returnvalue)
    (Class|StatComponent|AttackedBP _returnvalue 5.0 (Variables|Default|GetDrone%20Ref) "Normal" _impactnormal)
    (Actor|DestroyActor)
    (else
      (Actor|DestroyActor))))

(event EventBeginPlay
  (Variables|Target|GetTarget
    (:then
      (Variables|/Script/Engine.ProjectileMovementComponent|SetbIsHomingProjectile (Variables|Default|GetProjectileMovement) (Variables|ProjectileSettings|GetIsHoming))
      (Collision|IgnoreActorwhenMoving (Variables|Default|GetBoxCollision) (Components|GetOwner) true)
      (Variables|Default|Setprev_Loc (Transformation|GetActorLocation))
      (Utilities|FlowControl|Delay 5.0)
      (Actor|DestroyActor))
    (:else)))

(event EventTick
  (params (DeltaSeconds :type Float%20%28single-precision%29))
  (bind _drone_ref (Variables|Default|GetDrone%20Ref))
  (Variables|Default|Setcur_Loc (Transformation|GetActorLocation))
  (bind (_outhit _returnvalue) (Collision|LineTraceByChannel (Variables|Default|Getprev_Loc) (Variables|Default|Getcur_Loc) "TraceTypeQuery6" false 0 "None" true "(R=0.000000,G=1.000000,B=0.023377,A=1.000000)" "(R=1.000000,G=0.000000,B=0.123685,A=1.000000)"))
  (if _returnvalue
    (if (!= (.HitActor (Collision|BreakHitResult _outhit)) _drone_ref)
      (if (Actor|ActorHasTag (.HitActor (Collision|BreakHitResult _outhit)) "Player")
        (Class|StatComponent|AttackedBP (Actor|GetComponentbyClass (.HitActor (Collision|BreakHitResult _outhit)) "/Script/BaseClassModule.StatComponent") 5.0 _drone_ref "Normal" (.ImpactNormal (Collision|BreakHitResult _outhit))))
      (Actor|DestroyActor)
      (else
        (Variables|Default|Setprev_Loc (Variables|Default|Getcur_Loc) :!label _label)))
    (else
      (goto _label))))

(fn ConstructionScript
  (bind _projectilemovement (Variables|Default|GetProjectileMovement))
  (Variables|/Script/Engine.ProjectileMovementComponent|SetInitialSpeed _projectilemovement (Variables|ProjectileSettings|GetMinSpeed))
  (Variables|/Script/Engine.ProjectileMovementComponent|SetMaxSpeed _projectilemovement (Variables|ProjectileSettings|GetMaxSpeed))
  (Variables|/Script/Engine.ProjectileMovementComponent|SetProjectileGravityScale _projectilemovement (Variables|ProjectileSettings|GetGravity)))