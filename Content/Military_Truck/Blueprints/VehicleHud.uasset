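; HUD for the military truck that draws its speed and current gear near the bottom-right of the screen while the in-car camera is off.
; Each DrawHUD event casts the owning pawn to Military_Truck and draws its display strings, with position and text scale derived from screen size relative to a 720p reference.
; A controls help text node is present but disconnected, so it never draws.
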(event EventDrawHUD
  (params (SizeX :type Integer) (SizeY :type Integer))
  (bind _asmilitary_truck (Utilities|Casting|CastToMilitary_Truck (Class|HUD|GetOwningPawn)))
  ;[1 1 1] Calculate ratio from 720p
  (if (not (Variables|/Game/Military_Truck/Blueprints/Military_Truck.Military_Truck_C|GetIn%20Car%20Camera _asmilitary_truck))
    (Utilities|FlowControl|Sequence
      (:then_0
        (Variables|Default|SetHUDXRatio (/ (Math|Conversions|ToFloat(Integer) SizeX) 1.28e+03)))
      (:then_1
        (Variables|Default|SetHUDYRatio (/ (Math|Conversions|ToFloat(Integer) SizeY) 7.2e+02)))
      (:then_2
        ;[1 1 1] Print vehicle speed
        (HUD|DrawText (Variables|/Game/Military_Truck/Blueprints/Military_Truck.Military_Truck_C|GetSpeed%20Display%20String _asmilitary_truck) "(R=1.000000,G=1.000000,B=1.000000,A=1.000000)" (* 1.13e+03 (Variables|Default|GetHUDXRatio)) (* 6.5e+02 (Variables|Default|GetHUDYRatio)) "/Engine/EngineFonts/RobotoDistanceField.RobotoDistanceField" (* 1.2 (Variables|Default|GetHUDYRatio)) false)
        ;[1 1 1] Print vehicle gear
        (HUD|DrawText (Variables|/Game/Military_Truck/Blueprints/Military_Truck.Military_Truck_C|GetGear%20Display%20String _asmilitary_truck) "(R=1.000000,G=1.000000,B=1.000000,A=1.000000)" (* 1.13e+03 (Variables|Default|GetHUDXRatio)) (* 6.8e+02 (Variables|Default|GetHUDYRatio)) "/Engine/EngineFonts/RobotoDistanceField.RobotoDistanceField" (* 1.2 (Variables|Default|GetHUDYRatio)) false) ; If True display Current Gear
      ))))

(fn ConstructionScript)