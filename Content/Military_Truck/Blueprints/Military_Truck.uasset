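; Drivable Chaos-vehicle military truck with throttle, steering, handbrake, flip reset, toggleable lights and doors, and switchable interior/chase cameras.
; Tick feeds RPM, speed and smoothed door amount to the AnimBP, and updates engine audio, exhaust, light materials and HUD strings.
; Light, door, flip and brake-light changes route through server events.
; The construction script configures cargo bed/tent variants, paint scheme and wear through material parameters.
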(event Custom|Flip
  (bind _returnvalue (Transformation|GetActorLocation))
  ;[1 1 1] Flip car
  ;;[0.2836 0.3542 0.092] Replication
  (Transformation|SetActorRotation (Math|Rotator|MakeRotator 0.0 0.0 (.yaw (Transformation|GetActorRotation))) true)
  (Transformation|SetActorLocation (Math|Vector|MakeVector (.x _returnvalue) (.y _returnvalue) (+ (.z _returnvalue) 2e+02)) false true))

(event Custom|Light%20switch
  ;[1 1 1] Lights switch in-game
  (bind _output_get (Variables|Vehicle|SetLights (not (Variables|Vehicle|GetLights))))
  (Rendering|Material|SetScalarParameterValueonMaterials (Variables|Character|GetMesh) "Lights" (Math|Conversions|ToFloat(Boolean) _output_get))
  (Rendering|SetVisibility (Variables|Default|GetSpotLight1) _output_get false))

(event Custom|Light%20switch%20on%20server
  ;[1 1 1] Lights switch in-game
  (CallFunction|LightSwitch))

(event Custom|Server%20Flip
  ;[1 1 1] Flip car
  ;;[0.2836 0.3542 0.092] Replication
  (CallFunction|Flip))

(event Custom|Door%20open
  ;[1 1 1] Door open control
  (Variables|Default|SetDoors_open (not (Variables|Default|GetDoors_open))))

(event Custom|Door%20open%20on%20server
  ;[1 1 1] Door open control
  (CallFunction|DoorOpen))

(event Custom|Client%20SetBrakeLights
  ;[1 1 1] Replicated Brake Lights
  (CallFunction|ServerSetBrakeLights (< (* (Vehicle|GetForwardSpeed (Variables|Default|GetVehicleMovementComponent)) (Input|AxisValues|GetMoveForward)) -0.1)))

(event Custom|Server%20SetBrakeLights
  (params (Brake :type Boolean))
  ;[1 1 1] Replicated Brake Lights
  (Variables|Default|SetLights_Brake_ON Brake))

(event EventTick
  (params (DeltaSeconds :type Float%20%28single-precision%29))
  (bind _internalcamera (Variables|Default|GetInternalCamera))
  (bind _vehiclemovementcomponent (Variables|Default|GetVehicleMovementComponent))
  (bind _springarm (Variables|Default|GetSpringArm))
  (bind _throttle (Variables|Default|GetThrottle))
  (bind _anim_bp (Variables|Default|GetAnim%20Bp))
  (bind _exhaust (Variables|Default|GetExhaust))
  (bind _returnvalue (Vehicle|GetForwardSpeed _vehiclemovementcomponent))
  (bind _returnvalue_2 (Math|Float|Absolute(Float) _throttle))
  (bind _relativerotation (Variables|/Script/Engine.SceneComponent|GetRelativeRotation _springarm))
  (bind _relativerotation_2 (Variables|/Script/Engine.SceneComponent|GetRelativeRotation _internalcamera))
  (bind (_roll _pitch _yaw) (Math|Rotator|BreakRotator _relativerotation))
  (bind (_roll_2 _pitch_2 _yaw_2) (Math|Rotator|BreakRotator _relativerotation_2))
  (bind _returnvalue_3 (* _throttle _returnvalue))
  (bind _returnvalue_4 (> _returnvalue_3 0.0))
  (bind _returnvalue_5 (Math|Conversions|ToFloat(Boolean) _returnvalue_4))
  (bind _returnvalue_6 (* _returnvalue_2 _returnvalue_5))
  (bind _returnvalue_7 (* _returnvalue_6 0.45))
  (bind _returnvalue_8 (+ _returnvalue_7 0.55))
  (Utilities|FlowControl|Sequence
    (:then_0
      ;[1 1 1] RPM
      (Variables|Default|SetRPM (Class|ChaosWheeledVehicleMovementComponent|GetEngineRotationSpeed (.AsChaos%20Wheeled%20Vehicle%20Movement%20Component (Utilities|Casting|CastToChaosWheeledVehicleMovementComponent (Variables|Default|GetVehicleMovementComponent)))))
      ;[1 1 1] Handle Mouse interior camera movement
      (Transformation|SetRelativeRotation _internalcamera (Math|Rotator|MakeRotator 0.0 (Math|Float|ClampAngle (+ (Input|AxisValues|GetLookUp) _pitch_2) -89.0 89.0) (+ _yaw_2 (Input|AxisValues|GetLookRight))) false false)
      ;[1 1 1] Handle Mouse exterior camera movement
      (Transformation|SetRelativeRotation _springarm (Math|Rotator|MakeRotator 0.0 (Math|Float|ClampAngle (+ (Input|AxisValues|GetLookUp) _pitch) -89.0 89.0) (+ _yaw (Input|AxisValues|GetLookRight))) false false)
      ;[1 1 1] Door movement
      (bind _output_get (Variables|Default|SetDoors_open_amount (Math|Float|Lerp (Variables|Default|GetDoors_open_amount) (Math|Conversions|ToFloat(Boolean) (Variables|Default|GetDoors_open)) 0.2)))
      (Variables|/Game/Military_Truck/Mesh/MT_AnimBlueprint.MT_AnimBlueprint_C|SetDoor_open (Variables|Default|GetAnim%20Bp) _output_get))
    (:then_2
      ;[1 1 1] Engine Sound
      (Audio|Parameter|SetFloatParameter (Variables|Default|GetEngine%20Sound) "RPM" (Variables|Default|GetRPM) :!class /Script/Engine.AudioComponent)
      ;;[1 1 1] Engine volume set
      (Audio|Components|Audio|SetVolumeMultiplier (Variables|Default|GetEngine%20Sound) _returnvalue_8 :!class /Script/Engine.AudioComponent)
      ;[1 1 1] Exhaust control
      (Effects|Components|ParticleSystem|SetFloatParameter _exhaust "Rate" _returnvalue_8)
      (Effects|Components|ParticleSystem|SetVectorParameter _exhaust "Velo" (Math|Vector|MakeVector (Math|Random|RandomFloatinRange -1e+02 1e+02) (Math|Random|RandomFloatinRange -1e+02 1e+02) (+ (/ (Variables|Default|GetRPM) 3e+01) 2.5e+02))))
    (:then_3
      (Utilities|FlowControl|Sequence
        (:then_0
          ;[1 1 1] Replicated Brake Lights
          (CallFunction|ClientSetBrakeLights))
        (:then_1
          ;[1 1 1] Stop/reverse lights
          (Rendering|Material|SetScalarParameterValueonMaterials (Variables|Character|GetMesh) "Light_reverse" (Math|Conversions|ToFloat(Boolean) (< (Vehicle|GetForwardSpeed (Variables|Default|GetVehicleMovementComponent)) -5.0)))
          (Rendering|Material|SetScalarParameterValueonMaterials (Variables|Character|GetMesh) "Light_stop" (Math|Conversions|ToFloat(Boolean) (Variables|Default|GetLights_Brake_ON)))
          ;[1 1 1] send RPM and speed to AnimBP
          (Variables|/Game/Military_Truck/Mesh/MT_AnimBlueprint.MT_AnimBlueprint_C|SetRPM _anim_bp (Variables|Default|GetRPM))
          (Variables|/Game/Military_Truck/Mesh/MT_AnimBlueprint.MT_AnimBlueprint_C|SetSpeed _anim_bp (* (Vehicle|GetForwardSpeed (Variables|Default|GetVehicleMovementComponent)) 0.036))
          (CallFunction|UpdateHUDString))))))

(event EventBeginPlay
  ;[1 1 1] Begin Play
  (bind _asmt_anim_blueprint (Utilities|Casting|CastToMT_AnimBlueprint (Components|SkeletalMesh|GetAnimInstance (Variables|Character|GetMesh))))
  (Variables|Default|SetAnim%20Bp _asmt_anim_blueprint)
  (CallFunction|CameraSwitch (Variables|Vehicle|GetIn%20Car%20Camera)))

(event Input|AxisEvents|InputAxisMoveRight
  (params (AxisValue :type Float%20%28single-precision%29))
  ;[1 1 1] Axis Input
  (Class|ChaosVehicleMovementComponent|SetSteeringInput (Variables|Default|GetVehicleMovementComponent) AxisValue))

(event Input|AxisEvents|InputAxisMoveForward
  (params (AxisValue :type Float%20%28single-precision%29))
  (bind _vehiclemovementcomponent (Variables|Default|GetVehicleMovementComponent))
  ;[1 1 1] Axis Input
  (bind _output_get (Variables|Default|SetThrottle AxisValue))
  (Class|ChaosVehicleMovementComponent|SetThrottleInput _vehiclemovementcomponent (Math|Float|Clamp(Float) _output_get))
  (Class|ChaosVehicleMovementComponent|SetBrakeInput _vehiclemovementcomponent (Math|Float|Clamp(Float) (* _output_get -1.0))))

(event Input|KeyboardEvents|L
  (params (Key :type Key%20Structure :default "None"))
  ;[1 1 1] Lights switch in-game
  (:Pressed
    (Networking|SwitchHasAuthority
      (:Authority
        (CallFunction|LightSwitch))
      (:Remote
        (CallFunction|LightSwitchonServer)))))

(event Input|KeyboardEvents|Enter
  (params (Key :type Key%20Structure :default "None"))
  ;[1 1 1] Door open control
  (:Pressed
    (Networking|SwitchHasAuthority
      (:Authority
        (CallFunction|DoorOpen))
      (:Remote
        (CallFunction|DoorOpenonServer)))))

(event Input|KeyboardEvents|R
  (params (Key :type Key%20Structure :default "None"))
  ;[1 1 1] Flip car
  (:Pressed
    ;;[0.2836 0.3542 0.092] Replication
    (Networking|SwitchHasAuthority
      (:Authority
        (CallFunction|Flip))
      (:Remote
        (CallFunction|ServerFlip)))))

(event Input|KeyboardEvents|C
  (params (Key :type Key%20Structure :default "None"))
  ;[1 1 1] Handle Camera switching
  (:Pressed
    (bind _output_get (Variables|Vehicle|SetIn%20Car%20Camera (not (Variables|Vehicle|GetIn%20Car%20Camera))))
    (CallFunction|CameraSwitch _output_get)))

(event Input|MouseEvents|MouseWheelUp
  (params (Key :type Key%20Structure :default "None"))
  (bind _springarm (Variables|Default|GetSpringArm))
  ;[1 1 1] Camera zoom
  (:Pressed
    (Variables|/Script/Engine.SpringArmComponent|SetTargetArmLength _springarm (Math|Float|Clamp(Float) (* (Variables|/Script/Engine.SpringArmComponent|GetTargetArmLength _springarm) 0.91) 1.5e+02 1.5e+03))))

(event Input|KeyboardEvents|SpaceBar
  (params (Key :type Key%20Structure :default "None"))
  (bind _vehiclemovementcomponent (Variables|Default|GetVehicleMovementComponent))
  ;[1 1 1] Axis Input
  (:Pressed
    (Class|ChaosVehicleMovementComponent|SetHandbrakeInput _vehiclemovementcomponent true))
  (:Released
    (Class|ChaosVehicleMovementComponent|SetHandbrakeInput _vehiclemovementcomponent false)))

(event Input|MouseEvents|MouseWheelDown
  (params (Key :type Key%20Structure :default "None"))
  (bind _springarm (Variables|Default|GetSpringArm))
  ;[1 1 1] Camera zoom
  (:Pressed
    (Variables|/Script/Engine.SpringArmComponent|SetTargetArmLength _springarm (Math|Float|Clamp(Float) (* (Variables|/Script/Engine.SpringArmComponent|GetTargetArmLength _springarm) 1.1) 0.0 1.5e+03))))

(fn ConstructionScript
  (bind _lights (Variables|Vehicle|GetLights))
  ;[1 1 1] Lights
  (Rendering|Material|SetScalarParameterValueonMaterials (Variables|Character|GetMesh) "Lights" (Math|Conversions|ToFloat(Boolean) _lights))
  (Rendering|SetVisibility (Variables|Default|GetSpotLight) _lights false)
  (CallFunction|CameraSwitch (Variables|Vehicle|GetIn%20Car%20Camera))
  (CallFunction|CargoBedSetup)
  ;[1 1 1] Paint color
  (bind _returnvalue (Rendering|Material|CreateDynamicMaterialInstance (Variables|Character|GetMesh) 3 "/Game/Military_Truck/Materials/vehicle_cab.vehicle_cab" "None" :!class /Script/Engine.PrimitiveComponent))
  (bind _returnvalue_2 (Rendering|Material|CreateDynamicMaterialInstance (Variables|Default|GetCargo_bed) 0 "/Game/Military_Truck/Materials/vehicle_cargo_bed.vehicle_cargo_bed" "None" :!class /Script/Engine.PrimitiveComponent))
  (bind _returnvalue_3 (Rendering|Material|CreateDynamicMaterialInstance (Variables|Default|GetTent_Skeletal) 0 "/Game/Military_Truck/Materials/vehicle_tent.vehicle_tent" "None" :!class /Script/Engine.PrimitiveComponent))
  (Rendering|Material|SetMaterial (Variables|Default|GetTent_Frame) 0 _returnvalue_3)
  (switch Utilities|FlowControl|Switch|SwitchonBody_paint_list (Variables|Vehicle|GetBody%20Paint)
    (:NewEnumerator3
      _)
    (:NewEnumerator2
      (Variables|Default|SetTexture_cab_clean "/Game/Military_Truck/Textures/Clean/vehicle_cab_BaseColor_Desert.vehicle_cab_BaseColor_Desert")
      (Variables|Default|SetTexture_cab_dirty "/Game/Military_Truck/Textures/Dirty/vehicle_cab_BaseColor_Desert.vehicle_cab_BaseColor_Desert")
      (Variables|Default|SetTexture_cargo_bed_clean "/Game/Military_Truck/Textures/Clean/vehicle_cargo_bed_BaseColor_Desert.vehicle_cargo_bed_BaseColor_Desert")
      (Variables|Default|SetTexture_cargo_bed_dirty "/Game/Military_Truck/Textures/Dirty/vehicle_cargo_bed_BaseColor_Desert.vehicle_cargo_bed_BaseColor_Desert")
      (Variables|Default|SetTexture_tent_dirty "/Game/Military_Truck/Textures/Dirty/vehicle_tent_BaseColor_Desert.vehicle_tent_BaseColor_Desert")
      (Variables|Default|SetTexture_tent_clean "/Game/Military_Truck/Textures/Clean/vehicle_tent_BaseColor_Desert.vehicle_tent_BaseColor_Desert")
      (Rendering|Material|SetTextureParameterValue _returnvalue "Cab_paint_clean" (Variables|Default|GetTexture_cab_clean) :!label _label)
      (Rendering|Material|SetTextureParameterValue _returnvalue "Cab_paint_dirty" (Variables|Default|GetTexture_cab_dirty))
      (Rendering|Material|SetTextureParameterValue _returnvalue_2 "Paint_clean" (Variables|Default|GetTexture_cargo_bed_clean))
      (Rendering|Material|SetTextureParameterValue _returnvalue_2 "Paint_dirty" (Variables|Default|GetTexture_cargo_bed_dirty))
      (Rendering|Material|SetTextureParameterValue _returnvalue_3 "Paint_clean" (Variables|Default|GetTexture_tent_clean))
      (Rendering|Material|SetTextureParameterValue _returnvalue_3 "Paint_dirty" (Variables|Default|GetTexture_tent_dirty)))
    (:NewEnumerator1
      (Variables|Default|SetTexture_cab_clean "/Game/Military_Truck/Textures/Clean/vehicle_cab_BaseColor_Camouflage.vehicle_cab_BaseColor_Camouflage")
      (Variables|Default|SetTexture_cab_dirty "/Game/Military_Truck/Textures/Dirty/vehicle_cab_BaseColor_Camouflage.vehicle_cab_BaseColor_Camouflage")
      (Variables|Default|SetTexture_cargo_bed_clean "/Game/Military_Truck/Textures/Clean/vehicle_cargo_bed_BaseColor_Camouflage.vehicle_cargo_bed_BaseColor_Camouflage")
      (Variables|Default|SetTexture_cargo_bed_dirty "/Game/Military_Truck/Textures/Dirty/vehicle_cargo_bed_BaseColor_Camouflage.vehicle_cargo_bed_BaseColor_Camouflage")
      (Variables|Default|SetTexture_tent_dirty "/Game/Military_Truck/Textures/Dirty/vehicle_tent_BaseColor_Camouflage.vehicle_tent_BaseColor_Camouflage")
      (Variables|Default|SetTexture_tent_clean "/Game/Military_Truck/Textures/Clean/vehicle_tent_BaseColor_Camouflage.vehicle_tent_BaseColor_Camouflage")
      (goto _label)))
  ;[1 1 1] Rust and Wear
  (Rendering|Material|SetScalarParameterValueonMaterials (Variables|Default|GetCargo_bed) "Rust and Wear" (Variables|Vehicle|GetRust%20and%20Wear))
  (Rendering|Material|SetScalarParameterValueonMaterials (Variables|Character|GetMesh) "Glass Dirt" (Variables|Vehicle|GetGlass%20Dirt)))

(fn CameraSwitch
  (params (In%20Car :type Boolean))
  (bind _camera (Variables|Default|GetCamera))
  (bind _internalcamera (Variables|Default|GetInternalCamera))
  (if In%20Car
    ;[1 1 1] Activate Internal, Deactivate chase
    (Components|Activation|Activate _internalcamera false)
    (Components|Activation|Deactivate _camera)
    (else
      ;[1 1 1] Deactivate Internal,  Activate chase
      (Components|Activation|Deactivate _internalcamera)
      (Components|Activation|Activate _camera false)))
  (return))

(fn CargoBedSetup
  (bind _cargo_bed (Variables|Default|GetCargo_bed))
  (bind _tent_frame (Variables|Default|GetTent_Frame))
  (bind _tent_skeletal (Variables|Default|GetTent_Skeletal))
  (switch Utilities|FlowControl|Switch|SwitchonCargo_bed_list (Variables|Vehicle|GetCargo%20Bed)
    (:NewEnumerator0
      (Rendering|SetVisibility _cargo_bed false false)
      (Collision|SetCollisionEnabled _cargo_bed "NoCollision"))
    (:NewEnumerator1
      (Rendering|SetVisibility _cargo_bed true false :!label _label)
      (Collision|SetCollisionEnabled _cargo_bed "PhysicsOnly"))
    (:NewEnumerator2
      (goto _label))
    (:NewEnumerator3
      (goto _label)))
  (switch Utilities|FlowControl|Switch|SwitchonCargo_bed_list (Variables|Vehicle|GetCargo%20Bed)
    (:NewEnumerator0
      (Rendering|SetVisibility _tent_frame false false :!label _label_2)
      (Collision|SetCollisionEnabled _tent_frame "NoCollision"))
    (:NewEnumerator1
      (goto _label_2))
    (:NewEnumerator2
      (Rendering|SetVisibility _tent_frame true false :!label _label_3)
      (Collision|SetCollisionEnabled _tent_frame "PhysicsOnly"))
    (:NewEnumerator3
      (goto _label_3)))
  (switch Utilities|FlowControl|Switch|SwitchonCargo_bed_list (Variables|Vehicle|GetCargo%20Bed)
    (:NewEnumerator0
      (Rendering|SetVisibility _tent_skeletal false false :!label _label_4))
    (:NewEnumerator1
      (goto _label_4))
    (:NewEnumerator2
      (goto _label_4))
    (:NewEnumerator3
      (Rendering|SetVisibility _tent_skeletal true false)))
  (return))

(fn UpdateHUDString
  (bind _vehiclemovementcomponent (Variables|Default|GetVehicleMovementComponent))
  (bind _rpm (Variables|Default|GetRPM))
  (bind _vehiclemovementcomponent_2 (Variables|Default|GetVehicleMovementComponent))
  (bind _returnvalue (Vehicle|GetForwardSpeed _vehiclemovementcomponent))
  (bind _returnvalue_2 (Class|ChaosVehicleMovementComponent|GetCurrentGear _vehiclemovementcomponent_2))
  (bind _returnvalue_3 (Math|Float|Floor _rpm))
  (bind _returnvalue_4 (Utilities|String|ToString(Integer) _returnvalue_3))
  (bind _returnvalue_5 (* _returnvalue 0.036))
  (bind _returnvalue_6 (Math|Float|Absolute(Float) _returnvalue_5))
  (bind _returnvalue_7 (Math|Float|Floor _returnvalue_6))
  (Variables|Default|SetSpeed%20Display%20String (Utilities|String|Append (Utilities|String|ToString(Integer) _returnvalue_7) " km/h"))
  (if (== _returnvalue_7 0)
    (Variables|Default|SetGear%20Display%20String (Utilities|String|Append "N" "  /  " _returnvalue_4))
    (elif (== _returnvalue_2 -1)
      (Variables|Default|SetGear%20Display%20String (Utilities|String|Append "R" "  /  " _returnvalue_4))
      (else
        (Variables|Default|SetGear%20Display%20String (Utilities|String|Append (Utilities|String|ToString(Integer) _returnvalue_2) "  /  " _returnvalue_4))))))