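; Dummy car actor that laps a spline to demonstrate interactive Niagara effects such as sand, snow and leaves.
; The CarMove timeline maps its Cartrack alpha to spline distance, setting the dummy's location and rotation each update.
; TimeToComplete sets the play rate, and the timeline restarts on finish to loop.
; When NiagaraVFXActive is set, the car's world position feeds the Niagara component's Position2 variable.
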(event Custom|CarVFX
  (bind _spline (Variables|Default|GetSpline))
  ;[1 1 1] Spline Movement Car Logic
  (Components|Timeline|SetPlayRate (Variables|Default|GetCarMove) (/ 1.0 (Variables|Default|GetTimeToComplete)))
  (bind _cartrack (Timeline|CarMove PlayFromStart)
    (:Update
      (Transformation|SetWorldTransform (Variables|Default|GetDummy) (Math|Transform|MakeTransform (Spline|GetLocationatDistanceAlongSpline _spline (Math|Float|Lerp 0.0 (Spline|GetSplineLength _spline) _cartrack) "World") (Spline|GetRotationatDistanceAlongSpline _spline (Math|Float|Lerp 0.0 (Spline|GetSplineLength _spline) _cartrack) "World")) false false)
      (if (Variables|Default|GetNiagara%20VFX%20active?)
        ;[1 1 1] VFX Niagara Interaction Logic
        ; Niagara VFX - pick NS effects (Sand, Snow, Leaves)
        ; BP CAR DUMMY - collion object (car) that interacts with effect
        ; You can setup it in other blueprints by this logic
        (Niagara|SetNiagaraVariable(Vector3) (Variables|/Script/Niagara.NiagaraActor|GetNiagaraComponent (Variables|Default|GetNiagara%20VFX)) "Position2" (Transformation|GetWorldLocation (Variables|Default|GetBP_CAR_DUMMY)))))
    (:Finished
      (CallFunction|CarVFX)
      (Timeline|CarMove PlayFromStart))))

(event EventBeginPlay
  ;[1 1 1] Spline Movement Car Logic
  (Variables|Default|SetSpline (Variables|Default|GetSpline))
  (CallFunction|CarVFX :!label _label)
  (bind _cartrack (Timeline|CarMove PlayFromStart)
    (:Update
      (Transformation|SetWorldTransform (Variables|Default|GetDummy) (Math|Transform|MakeTransform (Spline|GetLocationatDistanceAlongSpline (Variables|Default|GetSpline) (Math|Float|Lerp 0.0 (Spline|GetSplineLength (Variables|Default|GetSpline)) _cartrack) "World") (Spline|GetRotationatDistanceAlongSpline (Variables|Default|GetSpline) (Math|Float|Lerp 0.0 (Spline|GetSplineLength (Variables|Default|GetSpline)) _cartrack) "World")) false false)
      (if (Variables|Default|GetNiagara%20VFX%20active?)
        ;[1 1 1] VFX Niagara Interaction Logic
        ; Niagara VFX - pick NS effects (Sand, Snow, Leaves)
        ; BP CAR DUMMY - collion object (car) that interacts with effect
        ; You can setup it in other blueprints by this logic
        (Niagara|SetNiagaraVariable(Vector3) (Variables|/Script/Niagara.NiagaraActor|GetNiagaraComponent (Variables|Default|GetNiagara%20VFX)) "Position2" (Transformation|GetWorldLocation (Variables|Default|GetBP_CAR_DUMMY)))))
    (:Finished
      (goto _label))))

(fn ConstructionScript)