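; Player armored vehicle that drives itself along the level's BP_Path spline while the mouse aims its turret.
; BeginPlay sets full throttle, then half after a delay; Tick steers toward a look-ahead spline point, and manual drive inputs are disconnected.
; Control rotation relative to the vehicle feeds turret aim and offset in the vehicle AnimBP and yaws the gunner mesh.
; Gun handle sockets drive the gunner's hand poses through ABP_VehicleCharactor.
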(event EventTick
  (params (DeltaSeconds :type Float%20%28single-precision%29))
  (bind _steering_input (CallFunction|FindPath (Variables|Default|GetPath)))
  (Class|ChaosVehicleMovementComponent|SetSteeringInput (Variables|Default|GetChaosWheeledVehicleMovement) _steering_input)
  (CallFunction|AnimationSetting))

(event EventBeginPlay
  (bind _chaoswheeledvehiclemovement (Variables|Default|GetChaosWheeledVehicleMovement))
  (bind _returnvalue (Actor|GetActorOfClass "/Game/_SGJ/BP_Path.BP_Path_C"))
  (Variables|Default|SetPath _returnvalue)
  (Class|ChaosVehicleMovementComponent|SetThrottleInput _chaoswheeledvehiclemovement 1.0)
  (Variables|Default|SetTurretOffSet (- (Transformation|GetSocketLocation (Variables|Character|GetMesh) "turret_jnt") (Transformation|GetWorldLocation (Variables|Default|GetPlayerMesh))))
  (Utilities|FlowControl|Delay 3.0)
  (Class|ChaosVehicleMovementComponent|SetThrottleInput _chaoswheeledvehiclemovement 0.5))

(event Input|AxisEvents|InputAxisTurnRight/LeftMouse
  (params (AxisValue :type Float%20%28single-precision%29))
  (Pawn|Input|AddControllerYawInput AxisValue))

(event Input|AxisEvents|InputAxisLookUp/DownMouse
  (params (AxisValue :type Float%20%28single-precision%29))
  (Pawn|Input|AddControllerPitchInput AxisValue))

(event Input|AxisEvents|InputAxisMoveForward/Backward
  (params (AxisValue :type Float%20%28single-precision%29)))

(event Input|AxisEvents|InputAxisMoveRight/Left
  (params (AxisValue :type Float%20%28single-precision%29)))

(fn ConstructionScript)

(fn FindPath
  (params (Path :type BP%20Path%20Object%20Reference))
  (bind _returnvalue (Transformation|GetActorLocation))
  (bind _spline (Variables|/Game/_SGJ/BP_Path.BP_Path_C|GetSpline Path))
  (return (Math|Float|MapRangeClamped (.Yaw (Math|Rotator|BreakRotator (Math|Rotator|Delta(Rotator) (Transformation|GetActorRotation) (Math|Rotator|FindLookatRotation (Transformation|GetActorLocation) (Spline|FindLocationClosesttoWorldLocation _spline (+ (* (Math|Vector|Normalize (Class|SplineComponent|FindTangentClosesttoWorldLocation _spline _returnvalue "World")) 1e+03) _returnvalue) "World"))))) 45.0 -45.0 -1.0 1.0)))

(fn AnimationSetting
  (bind _mesh (Variables|Character|GetMesh))
  (|ViehicleAnimationSetting)
  (bind _asabp_vehicle_charactor (Utilities|Casting|CastToABP_VehicleCharactor (Components|SkeletalMesh|GetAnimInstance (Variables|Default|GetPlayerMesh))))
  (Default|SettingHand _asabp_vehicle_charactor (Transformation|GetSocketLocation _mesh "Gun_Handle_R") (Transformation|GetSocketLocation _mesh "Gun_Handle_L") (Transformation|GetSocketRotation _mesh "Gun_Handle_R") (Transformation|GetSocketRotation _mesh "Gun_Handle_L")))