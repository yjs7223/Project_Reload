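; Explosive barrel actor that blows up when its Stat component fires DiePlay, guarded by a flag so it happens once.
; It swaps the barrel mesh for a geometry collection and spawns a field system actor and a Niagara explosion.
; A sphere overlap then finds nearby Vehicle-type objects and applies knockback damage from the blast point through their StatComponent.
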(event DiePlay(Stat)
  (bind _self self)
  (bind _returnvalue (Transformation|GetActorLocation _self))
  (bind _returnvalue_2 (+ _returnvalue "0,0,50.000000"))
  (if (Variables|Default|GetDestroyChk)
    (AddComponent|AddGeometryCollectionComponent false (Transformation|GetRelativeTransform (Variables|Default|GetBarrel)))
    (Components|DestroyComponent (Variables|Default|GetBarrel))
    (Variables|Default|SetDestroyChk false)
    (Game|SpawnActorfromClass "/Game/Aws/Fs_MasterUseong.Fs_MasterUseong_C" (Transformation|GetActorTransform _self) "Undefined" 0 0)
    (Niagara|SpawnSystematLocation "/Game/CarVFX/Niagara/Explosion/NS_Car_Expl_1.NS_Car_Expl_1" _returnvalue_2 "0, 0, 0" "0.800000,0.800000,0.800000")
    (bind _outactors (Collision|SphereOverlapActors _returnvalue_2 5e+02 (Utilities|Array|MakeArray "ObjectTypeQuery5") "/Script/Engine.Actor"))
    (for _array_element _outactors
      (Utilities|IsValid (Actor|GetComponentbyClass _array_element "/Script/BaseClassModule.StatComponent")
        (:Is%20Valid
          (Class|StatComponent|AttackedBP (Actor|GetComponentbyClass _array_element "/Script/BaseClassModule.StatComponent") (Variables|Default|GetDamage) 0 "Knockback" _returnvalue_2))))))

(event EventBeginPlay)

(event Collision|EventActorBeginOverlap
  (params (OtherActor :type Actor%20Object%20Reference)))

(event EventTick
  (params (DeltaSeconds :type Float%20%28single-precision%29)))

(fn ConstructionScript)