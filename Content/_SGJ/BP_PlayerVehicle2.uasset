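; Self-driving Chaos vehicle that follows the nearest BP_Path spline as either the main car or a car keeping formation around it.
; Each Tick, FindPath turns heading error toward a spline lookahead into steering and throttle, with a forward box trace triggering timed sidesteps.
; Non-main cars decelerate by dot product to their offset slot, switching to a navmesh-built spline while decelerating.
; On death, non-main cars explode into a damaged wreck.
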(event DiePlay(Stat)
  (bind _self self)
  (bind _returnvalue (Transformation|GetActorLocation _self))
  ;[1 1 1] 파괴
  (if (not (Variables|Default|GetMain_Car))
    (Niagara|SpawnSystematLocation "/Game/CarVFX/Niagara/Explosion/NS_Car_Expl_1.NS_Car_Expl_1" _returnvalue "0, 0, 0" "3.000000,3.000000,3.000000")
    (Game|SpawnActorfromClass "/Game/Aws/BP_Damaged.BP_Damaged_C" (Math|Transform|MakeTransform _returnvalue (Transformation|GetActorRotation _self) "1.000000,1.000000,1.000000") "Undefined" 0 0)
    (Niagara|SpawnSystematLocation "/Game/CarVFX/Niagara/Damaged/NS_Car_Damaged_Fire_1.NS_Car_Damaged_Fire_1" _returnvalue "0, 0, 0" "3.000000,3.000000,3.000000")
    (Game|SpawnActorfromClass "/Game/_SGJ/BP_VehicleShake.BP_VehicleShake_C" (Math|Transform|MakeTransform _returnvalue "0, 0, 0" "1.000000,1.000000,1.000000") "Undefined" 0 0)
    (Actor|DestroyActor)))

(event Custom|Avoidance
  (params (HitActor :type Actor%20Object%20Reference))
  (bind _returnvalue (Transformation|GetActorLocation HitActor))
  (Variables|Default|SetBoxHit true)
  (Development|PrintString "in")
  (bind _returnvalue_2 (Collision|BoxTraceByChannel _returnvalue (+ _returnvalue (* (Transformation|GetActorRightVector) 5e+02)) "100.000000,100.000000,100.000000" "0, 0, 0" "TraceTypeQuery1" false (Utilities|Array|MakeArray HitActor) "ForDuration" true "(R=1.000000,G=0.000000,B=0.000000,A=1.000000)" "(R=0.000000,G=1.000000,B=0.000000,A=1.000000)" 3.0))
  (if _returnvalue_2
    (Variables|Default|SetAvoidNum -0.7)
    (else
      (Variables|Default|SetAvoidNum 0.7)))
  (Utilities|FlowControl|Delay 0.8)
  (Variables|Default|SetAvoidNum 0.0)
  (Variables|Default|SetBoxHit false))

(event EventTick
  (params (DeltaSeconds :type Float%20%28single-precision%29))
  (bind _chaoswheeledvehiclemovement (Variables|Default|GetChaosWheeledVehicleMovement))
  (CallFunction|ForwardCheck)
  (if (Variables|Default|GetMain_Car)
    _
    (else
      (CallFunction|MainCarCheck)))
  (if (> (Variables|Default|GetDestination) 0)
    (CallFunction|FindClosePoint))
  (bind (_steering_input _brake_input _throttle_input) (CallFunction|FindPath))
  (Class|ChaosVehicleMovementComponent|SetSteeringInput _chaoswheeledvehiclemovement _steering_input)
  (Class|ChaosVehicleMovementComponent|SetThrottleInput _chaoswheeledvehiclemovement _throttle_input))

(event EventBeginPlay
  (CallFunction|FindClosePath)
  (bind _returnvalue (Actor|GetActorOfClass "/Game/_SGJ/BP_pc_Vehicle.BP_pc_Vehicle_C"))
  (Variables|Default|SetPC_Vehicle _returnvalue)
  (bind _outactors (Actor|GetAllActorsOfClass "/Game/_SGJ/BP_PlayerVehicle.BP_PlayerVehicle_C"))
  (for _array_element _outactors
    (if (Variables|BP_PlayerVehicle2_C|GetMain_Car _array_element)
      (Variables|Default|SetTargetCar _array_element))))

(fn ConstructionScript)

(fn FindPath
  (bind _returnvalue (Transformation|GetActorLocation))
  (if (== (Variables|Default|GetDeceleration) 0.0)
    (Variables|Default|SetTempSpline (Variables|/Game/_SGJ/BP_Path.BP_Path_C|GetSpline (Variables|Default|GetPath)))
    (else
      (Variables|Default|SetTempSpline (Variables|Default|GetSpline))))
  (if (Variables|Default|GetBoxHit)
    (return (Variables|Default|GetAvoidNum) 0.0 (Math|Float|MapRangeClamped (Math|Float|Absolute(Float) (.Yaw (Math|Rotator|BreakRotator (Math|Rotator|Delta(Rotator) (Transformation|GetActorRotation) (Math|Rotator|FindLookatRotation (Transformation|GetActorLocation) (Spline|FindLocationClosesttoWorldLocation (Variables|Default|GetTempSpline) (+ (* (Math|Vector|Normalize (Class|SplineComponent|FindTangentClosesttoWorldLocation (Variables|Default|GetTempSpline) _returnvalue "World")) 1e+03) _returnvalue) "World")))))) 0.0 45.0 (- 1.0 (Variables|Default|GetDeceleration)) 0.4))
    (else
      (return (Math|Float|MapRangeClamped (.Yaw (Math|Rotator|BreakRotator (Math|Rotator|Delta(Rotator) (Transformation|GetActorRotation) (Math|Rotator|FindLookatRotation (Transformation|GetActorLocation) (Spline|FindLocationClosesttoWorldLocation (Variables|Default|GetTempSpline) (+ (* (Math|Vector|Normalize (Class|SplineComponent|FindTangentClosesttoWorldLocation (Variables|Default|GetTempSpline) _returnvalue "World")) 1e+03) _returnvalue) "World"))))) 45.0 -45.0 -1.0 1.0) 0.0 (Math|Float|MapRangeClamped (Math|Float|Absolute(Float) (.Yaw (Math|Rotator|BreakRotator (Math|Rotator|Delta(Rotator) (Transformation|GetActorRotation) (Math|Rotator|FindLookatRotation (Transformation|GetActorLocation) (Spline|FindLocationClosesttoWorldLocation (Variables|Default|GetTempSpline) (+ (* (Math|Vector|Normalize (Class|SplineComponent|FindTangentClosesttoWorldLocation (Variables|Default|GetTempSpline) _returnvalue "World")) 1e+03) _returnvalue) "World")))))) 0.0 45.0 (- 1.0 (Variables|Default|GetDeceleration)) 0.4)))))

(fn SetPcPath
  (params (Path1 :type BP%20Path%20Object%20Reference))
  (Variables|Default|SetPath Path1))

(fn GetPcPath
  (return (Variables|Default|GetPath)))

(fn CarDead)

(fn FindClosePath
  (bind _outactors (Actor|GetAllActorsOfClass "/Game/_SGJ/BP_Path.BP_Path_C"))
  (for _array_element _outactors
    (if (Utilities|IsValid (Variables|Default|GetPath))
      (if (> (Math|Vector|VectorLength (- (Transformation|GetActorLocation (Variables|Default|GetPath)) (Transformation|GetActorLocation))) (Math|Vector|VectorLength (- (Transformation|GetActorLocation) (Transformation|GetActorLocation _array_element))))
        (Variables|Default|SetPath _array_element))
      (else
        (Variables|Default|SetPath _array_element))))
  (return))

(fn ChangePath
  (bind _outactors (Actor|GetAllActorsOfClass "/Game/_SGJ/BP_Path.BP_Path_C"))
  (for _array_element _outactors
    (if (!= (Variables|Default|GetPath) _array_element)
      (Utilities|IsValid (Variables|Default|GetTempPath)
        (:Is%20Valid
          (if (> (Math|Vector|VectorLength (- (Transformation|GetActorLocation (Variables|Default|GetTempPath)) (Transformation|GetActorLocation))) (Math|Vector|VectorLength (- (Transformation|GetActorLocation) (Transformation|GetActorLocation _array_element))))
            (Variables|Default|SetTempPath _array_element)
            (Development|PrintText "Set!")))
        (:Is%20Not%20Valid
          (Variables|Default|SetTempPath _array_element)))))
  (Variables|Default|SetPath (Variables|Default|GetTempPath))
  (Variables|Default|SetTempPath 0)
  (return))

(fn ForwardCheck
  (bind _returnvalue (Transformation|GetActorLocation))
  (bind _returnvalue_2 (+ _returnvalue "0,0.000000,100.000000"))
  (bind (_outhit _returnvalue_3) (Collision|BoxTraceByChannel _returnvalue_2 (+ _returnvalue_2 (* (Transformation|GetActorForwardVector) 1.7e+03)) "100.000000,150.000000,50.000000" "0, 0, 0" "TraceTypeQuery9" false 0 "ForDuration" true "(R=1.000000,G=0.000000,B=0.000000,A=1.000000)" "(R=0.000000,G=1.000000,B=0.000000,A=1.000000)" 0.0))
  (if _returnvalue_3
    (CallFunction|Avoidance (.HitActor (Collision|BreakHitResult _outhit)))))

(fn MainCarCheck
  (bind _returnvalue (Transformation|GetActorForwardVector))
  (bind _returnvalue_2 (Transformation|GetActorLocation))
  (bind _targetcar (Variables|Default|GetTargetCar))
  (bind _destinationvector (Variables|Default|GetDestinationVector))
  (bind _returnvalue_3 (Transformation|GetActorLocation _targetcar))
  (bind _returnvalue_4 (+ _returnvalue_3 _destinationvector))
  (bind _returnvalue_5 (- _returnvalue_4 _returnvalue_2))
  (bind _returnvalue_6 (Math|Vector|DotProduct _returnvalue _returnvalue_5))
  (if (< _returnvalue_6 0.0)
    (Variables|Default|SetDeceleration (Math|Float|MapRangeClamped _returnvalue_6 -9e+01 0.0 0.4 0.0))
    (else
      (Variables|Default|SetDeceleration (Math|Float|MapRangeClamped _returnvalue_6 9e+01 0.0 0.0 0.4))))
  (return))

(fn SetDestination
  (if (and (== (Variables|Default|GetDestination) 0) (!= (Variables|Default|GetMain_Car) true))
    (bind _outactors (Actor|GetAllActorsOfClass "/Game/_SGJ/BP_PlayerVehicle.BP_PlayerVehicle_C"))
    (for _array_element _outactors
      _)
    (else
      (return))))

(fn FindClosePoint
  (bind _targetcar (Variables|Default|GetTargetCar))
  (bind _returnvalue (Transformation|GetActorForwardVector _targetcar))
  (bind _returnvalue_2 (Transformation|GetActorRightVector _targetcar))
  (Spline|ClearSplinePoints (Variables|Default|GetSpline) true)
  (bind _returnvalue_3 (Class|NavigationSystemV1|FindPathtoLocationSynchronously (Transformation|GetActorLocation) (Transformation|GetActorLocation (Variables|Default|GetTargetCar)) 0 "/Script/AIModule.NavFilter_AIControllerDefault"))
  (for _array_element (Variables|/Script/NavigationSystem.NavigationPath|GetPathPoints _returnvalue_3)
    (switch int (Variables|Default|GetDestination)
      (:1
        (Variables|Default|SetDestinationVector (* _returnvalue 7e+02)))
      (:2
        (Variables|Default|SetDestinationVector (* _returnvalue_2 -5e+02)))
      (:3
        (Variables|Default|SetDestinationVector (* _returnvalue_2 5e+02)))
      (:4
        (Variables|Default|SetDestinationVector (* _returnvalue -7e+02))))
    (Spline|AddSplinePoint (Variables|Default|GetSpline) (+ _array_element (Variables|Default|GetDestinationVector)) "World" true))
  (return))