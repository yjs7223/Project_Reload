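; Player vehicle pawn, a Chaos wheeled MRAP that drives itself along the level's BP_Path spline while the player aims with the mouse.
; Throttle starts full and halves after three seconds; each tick steers toward a spline point found by projecting a tangent-based look-ahead.
; AnimationSetting turns the player mesh with control yaw and feeds turret rotation, pivot-corrected location and aim pitch to the AnimBlueprint.
; Manual driving inputs are disconnected.
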(event EventTick
  (params (DeltaSeconds :type Float%20%28single-precision%29))
  (bind _steering_input (CallFunction|FindPath (Variables|Default|GetPath)))
  (Class|ChaosVehicleMovementComponent|SetSteeringInput (Variables|Default|GetChaosWheeledVehicleMovement) _steering_input)
  (CallFunction|AnimationSetting))

(event EventBeginPlay
  (bind _chaoswheeledvehiclemovement (Variables|Default|GetChaosWheeledVehicleMovement))
  (bind _returnvalue (Actor|GetActorOfClass "/Game/_SGJ/BP_Path.BP_Path_C"))
  (Variables|Default|SetPath _returnvalue)
  (Class|ChaosVehicleMovementComponent|SetThrottleInput _chaoswheeledvehiclemovement 1.0)
  (Variables|Default|SetTurretOffSet (- (Transformation|GetSocketLocation (Variables|Character|GetMesh) "turret_jnt") (Transformation|GetWorldLocation (Variables|Default|GetPlayerMesh))))
  (Utilities|FlowControl|Delay 3.0)
  (Class|ChaosVehicleMovementComponent|SetThrottleInput _chaoswheeledvehiclemovement 0.5))

(event Input|AxisEvents|InputAxisTurnRight/LeftMouse
  (params (AxisValue :type Float%20%28single-precision%29))
  (Pawn|Input|AddControllerYawInput AxisValue))

(event Input|AxisEvents|InputAxisLookUp/DownMouse
  (params (AxisValue :type Float%20%28single-precision%29))
  (Pawn|Input|AddControllerPitchInput AxisValue))

(event Input|AxisEvents|InputAxisMoveForward/Backward
  (params (AxisValue :type Float%20%28single-precision%29)))

(event Input|AxisEvents|InputAxisMoveRight/Left
  (params (AxisValue :type Float%20%28single-precision%29)))

(fn ConstructionScript)

(fn FindPath
  (params (Path :type BP%20Path%20Object%20Reference))
  (bind _returnvalue (Transformation|GetActorLocation))
  (bind _spline (Variables|/Game/_SGJ/BP_Path.BP_Path_C|GetSpline Path))
  (return (Math|Float|MapRangeClamped (.Yaw (Math|Rotator|BreakRotator (Math|Rotator|Delta(Rotator) (Transformation|GetActorRotation) (Math|Rotator|FindLookatRotation (Transformation|GetActorLocation) (Spline|FindLocationClosesttoWorldLocation _spline (+ (* (Math|Vector|Normalize (Class|SplineComponent|FindTangentClosesttoWorldLocation _spline _returnvalue "World")) 1e+03) _returnvalue) "World"))))) 45.0 -45.0 -1.0 1.0)))

(fn AnimationSetting
  (bind _returnvalue (Transformation|GetActorRotation))
  (bind _returnvalue_2 (Pawn|GetController))
  (bind _turretoffset (Variables|Default|GetTurretOffSet))
  (bind _returnvalue_3 (Pawn|GetControlRotation _returnvalue_2 :!class /Script/Engine.Controller))
  (bind _returnvalue_4 (Math|Rotator|Delta(Rotator) _returnvalue_3 _returnvalue))
  (bind (_roll _pitch _yaw) (Math|Rotator|BreakRotator _returnvalue_4))
  (bind _returnvalue_5 (Math|Rotator|MakeRotator 0.0 0.0 _yaw))
  (bind _aswest_mrap_oshkosh_anim_blueprint (Utilities|Casting|CastToSKEL_West_MRAP_Oshkosh_AnimBlueprint (Components|SkeletalMesh|GetAnimInstance (Variables|Character|GetMesh))))
  (Transformation|SetRelativeRotation (Variables|Default|GetPlayerMesh) (Math|Rotator|MakeRotator 0.0 0.0 (+ _yaw -9e+01)) false false)
  (Variables|/Game/VigilanteContent/Vehicles/West_MRAP_Oshkosh/SKEL_West_MRAP_Oshkosh_AnimBlueprint.SKEL_West_MRAP_Oshkosh_AnimBlueprint_C|SetAimPitch _aswest_mrap_oshkosh_anim_blueprint _pitch)
  (Variables|/Game/VigilanteContent/Vehicles/West_MRAP_Oshkosh/SKEL_West_MRAP_Oshkosh_AnimBlueprint.SKEL_West_MRAP_Oshkosh_AnimBlueprint_C|SetTurretRotation _aswest_mrap_oshkosh_anim_blueprint _returnvalue_5)
  (Variables|/Game/VigilanteContent/Vehicles/West_MRAP_Oshkosh/SKEL_West_MRAP_Oshkosh_AnimBlueprint.SKEL_West_MRAP_Oshkosh_AnimBlueprint_C|SetTurretLocation _aswest_mrap_oshkosh_anim_blueprint (- (Math|Vector|RotateVector _turretoffset _returnvalue_5) _turretoffset)))