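; BP_pc_Vehicle is a player actor that rides along with the main BP_PlayerVehicle, always in aiming mode.
; BeginPlay finds the vehicle flagged MainCar, grants infinite weapon ammo and repositions the follow spring arm.
; Tick snaps the actor to that vehicle's Sphere location without taking its rotation and forces the aiming input on.
; A looping timer, its short interval randomized once at start, repeatedly fires a camera shake to simulate car motion.
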(event Custom|CarShake
  (Class|MatineeCameraShake|StartMatineeCameraShake (Game|GetPlayerCameraManager 0) "/Game/Aws/asd/BP_SlidingStartCameraShake_2.BP_SlidingStartCameraShake_2_C" 1.0 "CameraLocal" "0, 0, 0"))

(event EventTick
  (params (DeltaSeconds :type Float%20%28single-precision%29))
  (bind _m_inputcomponent (Variables|Default|Getm_InputComponent))
  (Variables|/Script/BaseClassModule.BaseInputComponent|Setm_inputData _m_inputcomponent (Utilities|Struct|MakeInputData (.movevec (Utilities|Struct|BreakInputData (Variables|/Script/BaseClassModule.BaseInputComponent|Getm_inputData _m_inputcomponent))) (.IsFire (Utilities|Struct|BreakInputData (Variables|/Script/BaseClassModule.BaseInputComponent|Getm_inputData _m_inputcomponent))) true (.IsReload (Utilities|Struct|BreakInputData (Variables|/Script/BaseClassModule.BaseInputComponent|Getm_inputData _m_inputcomponent)))))
  (Transformation|SetActorLocation (Transformation|GetWorldLocation (Variables|/Game/_SGJ/BP_PlayerVehicle.BP_PlayerVehicle_C|GetSphere (Variables|Default|GetPC_Vehicle))) false false))

(event EventBeginPlay
  (Utilities|Time|SetTimerbyEvent (delegate Custom|CarShake) (Math|Random|RandomFloatinRange 0.05 0.1) true)
  (bind _outactors (Actor|GetAllActorsOfClass "/Game/_SGJ/BP_PlayerVehicle.BP_PlayerVehicle_C"))
  (for _array_element _outactors
    (if (Variables|/Game/_SGJ/BP_PlayerVehicle.BP_PlayerVehicle_C|GetMain_Car _array_element)
      (Utilities|IsValid _array_element
        (:Is%20Valid
          (Variables|Default|SetPC_Vehicle _array_element)
          (Variables|/Script/PlayerModule.PlayerWeaponComponent|Setammoinfinite (Actor|GetComponentbyClass "/Script/PlayerModule.PlayerWeaponComponent") true)
          (Transformation|SetRelativeLocationAndRotation (Variables|Default|Getm_FollowSpringArm) (Math|Vector|MakeVector 0.0 0.0 1.5e+02) "0, 0, 0" false false))
        (:Is%20Not%20Valid
          (Development|PrintString "no_vehicle"))))))

(event Collision|EventActorBeginOverlap
  (params (OtherActor :type Actor%20Object%20Reference)))

(fn ConstructionScript)