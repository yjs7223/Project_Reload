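; BP_Missile is a homing missile actor that chases its Target and explodes on reaching it.
; Every Tick, Move snaps rotation toward the Target and teleports forward by a fixed, frame-rate-dependent step without sweep.
; A distance check, rather than collision, triggers the Niagara explosion, sound and two BP_VehicleShake variant actors, then destroys the missile.
; The file itself applies no damage to the Target.
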(event EventTick
  (params (DeltaSeconds :type Float%20%28single-precision%29))
  (CallFunction|Move))

(event EventBeginPlay)

(fn ConstructionScript)

(fn Move
  (bind _returnvalue (Transformation|GetActorLocation))
  (Transformation|SetActorRotation (Math|Rotator|FindLookatRotation (Transformation|GetActorLocation) (Transformation|GetActorLocation (Variables|Default|GetTarget))))
  (Transformation|SetActorLocation (+ (Transformation|GetActorLocation) (* (Transformation|GetActorForwardVector) 2e+02)) false true)
  (if (< (Math|Vector|Distance(Vector) (Transformation|GetActorLocation) (Transformation|GetActorLocation (Variables|Default|GetTarget))) 2e+02)
    (Niagara|SpawnSystematLocation "/Game/CarVFX/Niagara/Explosion/NS_Car_Expl_1.NS_Car_Expl_1" (Transformation|GetActorLocation) "0, 0, 0" "3.000000,3.000000,3.000000")
    (Game|SpawnActorfromClass "/Game/_SGJ/BP_VehicleShake.BP_VehicleShake_C" (Math|Transform|MakeTransform "0, 0, 0" "0, 0, 0" "1.000000,1.000000,1.000000") "Undefined" 0 0)
    (Audio|PlaySoundatLocation "/Game/_SGJ/Sound/EXPLOSION/RPG_EXPLOSION_Cue.RPG_EXPLOSION_Cue" _returnvalue "0, 0, 0" 1.0 1.0 0.0 0 0 0 0)
    (Game|SpawnActorfromClass "/Game/_SGJ/BP_VehicleShake1.BP_VehicleShake1_C" (Math|Transform|MakeTransform _returnvalue "0, 0, 0" "1.000000,1.000000,1.000000") "Undefined" 0 0)
    (Actor|DestroyActor)))