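; Self-driving Chaos vehicle that follows the BP_Path spline whose actor is closest at BeginPlay, at constant full throttle.
; Each tick, FindPath derives steering from the yaw toward a look-ahead spline point.
; On death, non-main cars spawn explosion and fire effects, a damaged wreck and a shake actor, then destroy themselves.
; Speed regulation by distance and angle to the main car exists, but its throttle/brake wiring never runs.
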(event DiePlay(Stat)
  (bind _self self)
  (bind _returnvalue (Transformation|GetActorLocation _self))
  (if (not (Variables|Default|GetMain_Car))
    (Niagara|SpawnSystematLocation "/Game/CarVFX/Niagara/Explosion/NS_Car_Expl_1.NS_Car_Expl_1" _returnvalue "0, 0, 0" "3.000000,3.000000,3.000000")
    (Game|SpawnActorfromClass "/Game/Aws/BP_Damaged.BP_Damaged_C" (Math|Transform|MakeTransform _returnvalue "0, 0, 0" "1.000000,1.000000,1.000000") "Undefined" 0 0)
    (Niagara|SpawnSystematLocation "/Game/CarVFX/Niagara/Damaged/NS_Car_Damaged_Fire_1.NS_Car_Damaged_Fire_1" _returnvalue "0, 0, 0" "3.000000,3.000000,3.000000")
    (Game|SpawnActorfromClass "/Game/_SGJ/BP_VehicleShake.BP_VehicleShake_C" (Math|Transform|MakeTransform _returnvalue "0, 0, 0" "1.000000,1.000000,1.000000") "Undefined" 0 0)
    (Actor|DestroyActor)))

(event EventTick
  (params (DeltaSeconds :type Float%20%28single-precision%29))
  (bind _chaoswheeledvehiclemovement (Variables|Default|GetChaosWheeledVehicleMovement))
  (bind _steering_input (CallFunction|FindPath (Variables|Default|GetPath)))
  (Class|ChaosVehicleMovementComponent|SetSteeringInput _chaoswheeledvehiclemovement _steering_input)
  (Class|ChaosVehicleMovementComponent|SetThrottleInput _chaoswheeledvehiclemovement 1.0))

(event EventBeginPlay
  (CallFunction|FindClosePath)
  (bind _outactors (Actor|GetAllActorsOfClass "/Game/_SGJ/BP_PlayerVehicle.BP_PlayerVehicle_C"))
  (for _array_element _outactors
    (if (Variables|BP_PlayerVehicle_2_C|GetMain_Car _array_element)
      (Variables|Default|SetTargetCar _array_element))))

(fn ConstructionScript)

(fn FindPath
  (params (Path :type BP%20Path%20Object%20Reference))
  (bind _returnvalue (Transformation|GetActorLocation))
  (bind _returnvalue_2 (Transformation|GetActorLocation))
  (bind _returnvalue_3 (Transformation|GetActorRotation))
  (bind _spline (Variables|/Game/_SGJ/BP_Path.BP_Path_C|GetSpline Path))
  (bind _returnvalue_4 (Class|SplineComponent|FindTangentClosesttoWorldLocation _spline _returnvalue_2 "World"))
  (bind _returnvalue_5 (Math|Vector|Normalize _returnvalue_4))
  (bind _returnvalue_6 (* _returnvalue_5 1e+03))
  (bind _returnvalue_7 (+ _returnvalue_6 _returnvalue_2))
  (bind _returnvalue_8 (Spline|FindLocationClosesttoWorldLocation _spline _returnvalue_7 "World"))
  (bind _returnvalue_9 (Math|Rotator|FindLookatRotation _returnvalue _returnvalue_8))
  (bind _returnvalue_10 (Math|Rotator|Delta(Rotator) _returnvalue_3 _returnvalue_9))
  (bind _yaw (Math|Rotator|BreakRotator _returnvalue_10))
  (bind _returnvalue_11 (Math|Float|Absolute(Float) _yaw))
  (return (Math|Float|MapRangeClamped _yaw 45.0 -45.0 -1.0 1.0) (Math|Float|MapRangeClamped _returnvalue_11 0.0 45.0 0.0 0.3) (Math|Float|MapRangeClamped _returnvalue_11 0.0 45.0 1.0 0.0)))

(fn FindClosePath
  (bind _outactors (Actor|GetAllActorsOfClass "/Game/_SGJ/BP_Path.BP_Path_C"))
  (for _array_element _outactors
    (if (Utilities|IsValid (Variables|Default|GetPath))
      (if (> (Math|Vector|VectorLength (- (Transformation|GetActorLocation (Variables|Default|GetPath)) (Transformation|GetActorLocation))) (Math|Vector|VectorLength (- (Transformation|GetActorLocation) (Transformation|GetActorLocation _array_element))))
        (Variables|Default|SetPath _array_element))
      (else
        (Variables|Default|SetPath _array_element))))
  (return))

(fn CarSpeedChage)