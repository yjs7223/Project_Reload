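; Test AI pawn for grenade throwing that copies its current HP to the AI controller's Blackboard on BeginPlay.
; Tick runs through a three-second Delay into FireInTheHole, which throws at fixed velocity.
; The unused ShotGrenade solves the ballistic angle to the last BP_pc_Anim found, spawning BP_Grenade on the high arc when reachable.
; Patrol-stop and input-struct fragments are also disconnected.
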(event EventBeginPlay
  (bind _asai_컨트롤러 (Utilities|Casting|CastToAIController (Pawn|GetController self)))
  (AI|Components|Blackboard|SetValueasFloat (Variables|/Script/AIModule.AIController|GetBlackboard _asai_컨트롤러) (Utilities|Name|MakeLiteralName "AI_HP") (Variables|/Script/BaseClassModule.StatComponent|GetcurHP (Variables|Default|GetAIStat))))

(event Collision|EventActorBeginOverlap
  (params (OtherActor :type Actor%20Object%20Reference)))

(event EventTick
  (params (DeltaSeconds :type Float%20%28single-precision%29))
  (Utilities|FlowControl|Delay 3.0)
  (Class|AICharacter|FireintheHole self 1e+03))

(fn ConstructionScript)

(fn ShotGrenade
  (bind _returnvalue (Transformation|GetActorLocation))
  (bind _returnvalue_2 (Transformation|GetActorLocation))
  (bind _velocity (Variables|Default|GetVelocity))
  (bind _gravity (Variables|Default|GetGravity))
  (bind _returnvalue_3 (Math|Float|Square _velocity))
  (bind _outactors (Actor|GetAllActorsOfClass "/Game/yjs/BP_pc_Anim.BP_pc_Anim_C"))
  (for _array_element _outactors
    _)
  (if (>= (- (Math|Float|Square _returnvalue_3) (* (+ (* (Math|Float|Square (Math|Vector2D|Vector2DLength (Math|Vector2D|MakeVector2D (- (.x (Transformation|GetActorLocation _array_element)) (.x _returnvalue)) (- (.y (Transformation|GetActorLocation _array_element)) (.y _returnvalue))))) _gravity) (* (* (- (.z (Transformation|GetActorLocation _array_element)) (.z _returnvalue)) _returnvalue_3) 2.0)) _gravity)) 0.0)
    (Game|SpawnActorfromClass "/Game/Aws/BP_Grenade.BP_Grenade_C" (Math|Transform|MakeTransform _returnvalue_2 (Math|Rotator|MakeRotator (.roll (Math|Rotator|FindLookatRotation _returnvalue_2 (Transformation|GetActorLocation _array_element))) (Class|KismetMathLibrary|DegAtan (/ (+ (Math|Float|Sqrt (- (Math|Float|Square _returnvalue_3) (* (+ (* (Math|Float|Square (Math|Vector2D|Vector2DLength (Math|Vector2D|MakeVector2D (- (.x (Transformation|GetActorLocation _array_element)) (.x _returnvalue)) (- (.y (Transformation|GetActorLocation _array_element)) (.y _returnvalue))))) _gravity) (* (* (- (.z (Transformation|GetActorLocation _array_element)) (.z _returnvalue)) _returnvalue_3) 2.0)) _gravity))) _returnvalue_3) (* (Math|Vector2D|Vector2DLength (Math|Vector2D|MakeVector2D (- (.x (Transformation|GetActorLocation _array_element)) (.x _returnvalue)) (- (.y (Transformation|GetActorLocation _array_element)) (.y _returnvalue)))) _gravity))) (.yaw (Math|Rotator|FindLookatRotation _returnvalue_2 (Transformation|GetActorLocation _array_element)))) "1.000000,1.000000,1.000000") "Undefined" 0 0)
    (Development|PrintText (Utilities|Text|ToText(Float) (Math|Float|Min(Float) 0.0 (Class|KismetMathLibrary|DegAtan (/ (- _returnvalue_3 (Math|Float|Sqrt (- (Math|Float|Square _returnvalue_3) (* (+ (* (Math|Float|Square (Math|Vector2D|Vector2DLength (Math|Vector2D|MakeVector2D (- (.x (Transformation|GetActorLocation _array_element)) (.x _returnvalue)) (- (.y (Transformation|GetActorLocation _array_element)) (.y _returnvalue))))) _gravity) (* (* (- (.z (Transformation|GetActorLocation _array_element)) (.z _returnvalue)) _returnvalue_3) 2.0)) _gravity)))) (* (Math|Vector2D|Vector2DLength (Math|Vector2D|MakeVector2D (- (.x (Transformation|GetActorLocation _array_element)) (.x _returnvalue)) (- (.y (Transformation|GetActorLocation _array_element)) (.y _returnvalue)))) _gravity)))) "HalfToEven"))))