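; Enemy helicopter that calls a spline path-stepping function each Tick and carries a machine gun.
; ShotEvent fires bursts at Target with random spread and decaying pitch offset, pairing line-trace damage with spawned bullets.
; On death a timeline drives height and yaw spin, and a mesh hit at zero HP explodes it.
; Vehicle-movement steering, automatic firing and homing missile logic are disconnected, so nothing here triggers the gun.
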(event DiePlay(Stat)
  ;[1 1 1] 사망 이벤트 시작
  (Variables|Default|SetDieChk false)
  (bind _die (Timeline|타임라인_0 Play)
    (:Update
      ;[1 1 1] 높이 낮추기
      (Utilities|FlowControl|Sequence
        (:then_0
          (bind _output_get (Variables|Default|SetUp%20Axis%20Value _die))
          (if (== _output_get 0.0)
            (Utilities|FlowControl|DoOnce false :!label _label
              (:Completed
                (Variables|Default|SetHelicopter%20Height (.z (Transformation|GetActorLocation)))))
            (else
              (goto _label Reset))))
        (:then_1
          (Class|ChaosVehicleMovementComponent|SetYawInput (Variables|Default|GetVehicleMovementComponent) (* _die 1e+02)))))))

(event OnComponentHit(Mesh)
  (params (HitComponent :type Primitive%20Component%20Object%20Reference) (OtherActor :type Actor%20Object%20Reference) (OtherComp :type Primitive%20Component%20Object%20Reference) (NormalImpulse :type Vector :default "0, 0, 0") (Hit :type Hit%20Result%20Structure%20%28by%20ref%29))
  (if (<= (Variables|/Script/BaseClassModule.StatComponent|GetcurHP (Variables|Default|GetStat)) 0.0)
    (CallFunction|Bomb)))

(event Custom|Bomb
  (bind _returnvalue (Transformation|GetActorLocation))
  ;[1 1 1] 사망 이벤트
  (Game|SpawnActorfromClass "/Game/Aws/BluePrints/BP_HelDamage.BP_HelDamage_C" (Math|Transform|MakeTransform _returnvalue (Transformation|GetActorRotation) "1.000000,1.000000,1.000000") "Undefined" 0 0)
  (Niagara|SpawnSystematLocation "/Game/Aws/NS_Car_Expl_1.NS_Car_Expl_1" (+ _returnvalue "") "0, 0, 0" "5.000000,5.000000,5.000000")
  (Audio|PlaySoundatLocation "/Game/AI_Project/AI_Pakage/BaseAI/Sound/Explosion_Dog_Cue.Explosion_Dog_Cue" _returnvalue "0, 0, 0" 1.0 1.0 0.0 0 0 0 0)
  (Actor|DestroyActor))

(event Custom|ShotEvent
  (bind _shotspread (Variables|Default|GetShotSpread))
  (bind _arrow (Variables|Default|GetArrow))
  (bind _target (Variables|Default|GetTarget))
  (bind _arrow_2 (Variables|Default|GetArrow))
  (bind _returnvalue (Transformation|GetWorldLocation _arrow_2))
  (bind _returnvalue_2 (Transformation|GetWorldLocation _arrow))
  (bind _returnvalue_3 (Transformation|GetActorLocation _target))
  (bind _relativerotation (Variables|/Script/Engine.SceneComponent|GetRelativeRotation _arrow))
  (bind _returnvalue_4 (Math|Rotator|FindLookatRotation _returnvalue_2 _returnvalue_3))
  ;[1 1 1] 코멘트
  (Variables|Default|SetShotRine (Variables|Default|GetMax_ShotRine))
  (bind _returnvalue_5 (Niagara|SpawnSystemAttached "/Game/Bullet_Impact_Hit/Prefabs/For_Games/Muzzle_Flash_Only/Niagara_Riffle_MuzzleFlash_Radial_01.Niagara_Riffle_MuzzleFlash_Radial_01" (Variables|Default|GetArrow) "None" "0, 0, 0" "0, 0, 0" "KeepRelativeOffset" true))
  (Variables|Default|SetMachineGunCount (Variables|Default|GetMax_MachinGunCount))
  (if (!= (Variables|Default|GetMachineGunCount) 0) :!label _label
    ;;[1 1 1] 사격 방향 및 반동 실행
    (Transformation|SetWorldRotation _arrow (Math|Rotator|MakeRotator (.roll _returnvalue_4) (.pitch _returnvalue_4) (.yaw _returnvalue_4)) false false)
    (Transformation|SetWorldRotation _arrow (Math|Rotator|MakeRotator (.roll _returnvalue_4) (.pitch _returnvalue_4) (+ (.yaw _returnvalue_4) (Math|Random|RandomFloatinRange (* _shotspread -1.0) _shotspread))) false false)
    (Transformation|SetRelativeRotation (Variables|Default|GetArrow) (Math|Rotator|MakeRotator (.roll _relativerotation) (- (.pitch _relativerotation) (Variables|Default|GetShotRine)) (.yaw _relativerotation)) false false)
    (Audio|PlaySoundatLocation "/Game/Aws/SD_Gattling.SD_Gattling" _returnvalue_2 "0, 0, 0" 1.0 1.0 0.0 0 0 0 0)
    ;;[1 1 1] 사격 실행
    (bind _outhit (Collision|LineTraceByChannel _returnvalue (+ _returnvalue (* (Math|Vector|GetForwardVector _arrow_2) 5e+04)) "TraceTypeQuery1" false 0 "ForOneFrame" true "(R=1.000000,G=0.000000,B=0.000000,A=1.000000)" "(R=0.000000,G=1.000000,B=0.000000,A=1.000000)" 0.5))
    (Game|SpawnActorfromClass "/Game/Aws/BluePrints/BP_Bullet.BP_Bullet_C" (Math|Transform|MakeTransform (Transformation|GetWorldLocation _arrow_2) (Transformation|GetWorldRotation _arrow_2) "1.000000,1.000000,1.000000") "Undefined" self 0)
    (if (Actor|ActorHasTag (.HitActor (Collision|BreakHitResult _outhit)) "Player")
      (Niagara|SpawnSystematLocation "/Game/UHitImpactNiagara/UltimateEffect/NS_Impact_Blood.NS_Impact_Blood" (.Location (Collision|BreakHitResult _outhit)))
      (Class|StatComponent|AttackedBP (Actor|GetComponentbyClass (.HitActor (Collision|BreakHitResult _outhit)) "/Script/BaseClassModule.StatComponent") 3e+01 0 "Normal" (.ImpactNormal (Collision|BreakHitResult _outhit)))
      (else
        (if (Actor|ActorHasTag (.HitActor (Collision|BreakHitResult _outhit)) "Car")
          (Niagara|SpawnSystematLocation "/Game/UHitImpactNiagara/UltimateEffect/Fx_Bullet_Robot_Normal_Impact.Fx_Bullet_Robot_Normal_Impact" (.Location (Collision|BreakHitResult _outhit)) "0, 0, 0" "0.500000,0.500000,0.500000")
          (else
            (Niagara|SpawnSystematLocation "/Game/Bullet_Impact_Hit/Prefabs/For_Games/Impact_Fx_Only/Fx_Bullet_Ground_Impact.Fx_Bullet_Ground_Impact" (.Location (Collision|BreakHitResult _outhit)) "0, 0, 0" "0.500000,0.500000,0.500000")))
        (Class|StatComponent|AttackedBP (Actor|GetComponentbyClass (.HitActor (Collision|BreakHitResult _outhit)) "/Script/BaseClassModule.StatComponent") 3e+01 0 "Normal" (.ImpactNormal (Collision|BreakHitResult _outhit)))))
    (Utilities|FlowControl|Delay 0.05)
    (Math|Integer|DecrementInt (Variables|Default|GetMachineGunCount)
      (:%20%20
        (if true
          (Variables|Default|SetShotRine (- (Variables|Default|GetShotRine) (/ (Variables|Default|GetMax_ShotRine) (/ (Variables|Default|GetMax_MachinGunCount) 2))))
          (goto _label))))
    (else
      (Variables|Default|SetGun%20Shooting false)
      (Variables|Default|SetReloadingTime (Variables|Default|GetMaxReloadingTime))
      (Class|NiagaraComponent|SetAutoDestroy _returnvalue_5 true)
      (Components|DestroyComponent _returnvalue_5))))

(event Custom|Homming)

(event EventTick
  (params (DeltaSeconds :type Float%20%28single-precision%29))
  (CallFunction|FindPath))

(event EventBeginPlay
  (Variables|Default|SetReloadingTime 1e+01))

(fn ConstructionScript)

(fn FindTarget
  (bind _returnvalue (Transformation|GetActorLocation))
  (bind _returnvalue_2 (Transformation|GetActorRotation))
  (bind _target (Variables|Default|GetTarget))
  (bind _returnvalue_3 (Transformation|GetActorLocation _target))
  (bind _returnvalue_4 (Math|Vector|MakeVector (.x _returnvalue) (.y _returnvalue) 0.0))
  (bind _returnvalue_5 (Math|Vector|GetForwardVector _returnvalue_2))
  (bind _returnvalue_6 (Math|Vector|MakeVector (.x _returnvalue_3) (.y _returnvalue_3) 0.0))
  (bind _returnvalue_7 (Math|Vector|Normalize _returnvalue_5))
  (bind _returnvalue_8 (- _returnvalue_6 _returnvalue_4))
  (bind _returnvalue_9 (Math|Vector|Normalize _returnvalue_8))
  (Utilities|IsValid (Variables|Default|GetTarget)
    (:Is%20Valid
      (if (>= (Math|Float|Absolute(Float) (* (Class|KismetMathLibrary|DegAcos (Math|Vector|DotProduct _returnvalue_7 _returnvalue_9)) (Math|Float|Sign(Float) (.z (Math|Vector|CrossProduct _returnvalue_7 _returnvalue_9))))) 1.2e+02)
        (Variables|Default|SetYawInput 0.0)
        (else
          (Variables|Default|SetYawInput 1.0)))
      (return (Variables|Default|GetYawInput)))))

(fn HeightTarget
  (bind _returnvalue (Transformation|GetActorLocation))
  (bind _target (Variables|Default|GetTarget))
  (bind _returnvalue_2 (Transformation|GetActorLocation _target))
  (bind _returnvalue_3 (- (.z _returnvalue) (.z _returnvalue_2)))
  (if (>= _returnvalue_3 (Variables|Height|GetHeightValue))
    (Variables|Default|SetHeightLock true)
    (Variables|Height|SetSetTrottle 0.0 :!label _label)
    (else
      (if (and (<= _returnvalue_3 (Variables|Height|GetLowHeight)) (Variables|Default|GetHeightLock))
        (Variables|Default|SetHeightLock false))
      (if (Variables|Default|GetHeightLock)
        (goto _label)
        (else
          (Variables|Height|SetSetTrottle 1.0)))))
  (return (Variables|Height|GetSetTrottle)))

(fn FindMoveTarget
  (params (foward%20input :type Float%20%28double-precision%29))
  (if (>= (Class|ChaosVehicleMovementComponent|GetForwardSpeedMPH (Variables|Default|GetVehicleMovementComponent)) 3e+01)
    (Variables|Default|SetFowardInput 0.0 :!label _label)
    (elif true
      (if (<= (.pitch (Transformation|GetActorRotation)) -15.0)
        (goto _label)
        (else
          (Variables|Default|SetFowardInput 1.0)))
      (else
        (Variables|Default|SetFowardInput -1.0))))
  (Class|ChaosVehicleMovementComponent|SetPitchInput (Variables|Default|GetVehicleMovementComponent) (Variables|Default|GetFowardInput)))

(fn RollFIX
  (params (YawInput :type Float%20%28double-precision%29))
  (bind _returnvalue (Transformation|GetActorRotation))
  (if (<= YawInput 0.3)
    (Variables|Default|SetRollFixRotation 3.0)
    (else
      (Variables|Default|SetRollFixRotation 5.0)))
  (if (>= (Math|Float|Absolute(Float) (.roll _returnvalue)) (Variables|Default|GetRollFixRotation))
    (if (>= (.roll _returnvalue) 0.0)
      (Variables|Default|SetSetROll -1.0)
      (else
        (Variables|Default|SetSetROll 1.0)))
    (else
      (Variables|Default|SetSetROll 0.0)))
  (Class|ChaosVehicleMovementComponent|SetRollInput (Variables|Default|GetVehicleMovementComponent) (Variables|Default|GetSetROll)))

(fn RollScaleSetting
  (params (YawChk :type Float%20%28double-precision%29))
  (if (>= YawChk 0.0)
    (Variables|Default|SetSetROll 1.0)
    (else
      (Variables|Default|SetSetROll -1.0)))
  (Class|ChaosVehicleMovementComponent|SetRollInput (Variables|Default|GetVehicleMovementComponent) (Variables|Default|GetSetROll)))

(fn FindPath
  (params (Path :type BP%20Path%20Object%20Reference))
  (bind _returnvalue (Transformation|GetActorLocation))
  (bind _spline (Variables|/Game/_SGJ/BP_Path.BP_Path_C|GetSpline Path))
  (Transformation|SetActorLocation (+ (Spline|FindLocationClosesttoWorldLocation _spline (+ (* (Math|Vector|Normalize (Class|SplineComponent|FindTangentClosesttoWorldLocation _spline _returnvalue "World")) 1e+01) _returnvalue) "World") (Transformation|GetActorLocation)) false false)
  (return))