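; BP_GrenadeDummy is a timed grenade actor that displays a growing range indicator, then explodes visually and destroys itself, applying no damage.
; On BeginPlay it hides GrenadeRange at zero scale, speeds up its own time, and after short delays runs the DecalScale timeline to grow the indicator.
; The timeline's end spawns the explosion particle.
; Once armed, Sphere overlaps with actors other than itself or BP_GrenadeTest enable Grenade physics.
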(event OnComponentBeginOverlap(Sphere)
  (params (OverlappedComponent :type Primitive%20Component%20Object%20Reference) (OtherActor :type Actor%20Object%20Reference) (OtherComp :type Primitive%20Component%20Object%20Reference) (OtherBodyIndex :type Integer) (bFromSweep :type Boolean) (SweepResult :type Hit%20Result%20Structure%20%28by%20ref%29))
  (if (Variables|Default|GetOverlap%20CHK)
    (if (not (== OtherActor self))
      (if (not (== OtherActor "/Game/Aws/BluePrints/BP_GrenadeTest.BP_GrenadeTest"))
        (Physics|SetSimulatePhysics (Variables|Default|GetGrenade) true)
        (Utilities|FlowControl|Delay 0.2)))))

(event Custom|Explosion
  (bind _self self)
  (bind _grenaderange (Variables|Default|GetGrenadeRange))
  (Utilities|FlowControl|Delay 3.0)
  (Transformation|SetWorldRotation _grenaderange "90.000000, 0, 0" false false)
  (bind _새_트랙_0 (Timeline|DecalScale Play)
    (:Update
      (Transformation|SetWorldScale3D _grenaderange _새_트랙_0))
    (:Finished
      (Effects|SpawnEmitteratLocation "/Game/ThirdPersonKit/Particles/P_Explosion.P_Explosion" (Transformation|GetActorLocation _self) "0, 0, 0" "5.000000,5.000000,5.000000")
      (Actor|DestroyActor _self))))

(event EventBeginPlay
  (Transformation|SetWorldScale3D (Variables|Default|GetGrenadeRange) "0, 0, 0")
  (Variables|Default|SetCustomTimeDilation 1.5)
  (Utilities|FlowControl|Delay 0.5)
  (Variables|Default|SetOverlap%20CHK true)
  (CallFunction|Explosion))

(event Collision|EventActorBeginOverlap
  (params (OtherActor :type Actor%20Object%20Reference)))

(event EventTick
  (params (DeltaSeconds :type Float%20%28single-precision%29)))

(fn ConstructionScript)