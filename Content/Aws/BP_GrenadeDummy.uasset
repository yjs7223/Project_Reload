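; BP_GrenadeDummy is a grenade stand-in actor that switches its Grenade component to physics simulation when its sphere overlaps something.
; BeginPlay speeds up the actor's custom time dilation and arms the overlap check after a short delay.
; The sphere overlap ignores itself and BP_GrenadeTest, enables physics, then ends on a delay with nothing after it.
; The Explosion event is an empty stub.
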(event OnComponentBeginOverlap(Sphere)
  (params (OverlappedComponent :type Primitive%20Component%20Object%20Reference) (OtherActor :type Actor%20Object%20Reference) (OtherComp :type Primitive%20Component%20Object%20Reference) (OtherBodyIndex :type Integer) (bFromSweep :type Boolean) (SweepResult :type Hit%20Result%20Structure%20%28by%20ref%29))
  (if (Variables|Default|GetOverlap%20CHK)
    (if (not (== OtherActor self))
      (if (not (== OtherActor "/Game/Aws/BP_GrenadeTest.BP_GrenadeTest"))
        (Physics|SetSimulatePhysics (Variables|Default|GetGrenade) true)
        (Utilities|FlowControl|Delay 0.2)))))

(event Custom|Explosion)

(event EventBeginPlay
  (Variables|Default|SetCustomTimeDilation 1.5)
  (Utilities|FlowControl|Delay 0.5)
  (Variables|Default|SetOverlap%20CHK true))

(event Collision|EventActorBeginOverlap
  (params (OtherActor :type Actor%20Object%20Reference)))

(event EventTick
  (params (DeltaSeconds :type Float%20%28single-precision%29)))

(fn ConstructionScript)