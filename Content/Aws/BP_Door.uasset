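; BP_Door is a door actor that swings open and shut automatically, with no player interaction wired.
; BeginPlay waits briefly, calls DoorOpen, waits again, then calls CloseDoor.
; Each event captures the current actor rotation and plays its own timeline, adding the track value to that yaw to rotate the whole actor.
; Overlap and Tick events are unused, and the construction script is empty.
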(event Custom|Door%20Open
  (Variables|Default|SetRotation (Transformation|GetActorRotation))
  (bind _새_트랙_0 (Timeline|OpenDoor Play)
    (:Update
      (Transformation|SetActorRotation (Math|Rotator|MakeRotator (.roll (Variables|Default|GetRotation)) (.pitch (Variables|Default|GetRotation)) (+ (.yaw (Variables|Default|GetRotation)) _새_트랙_0))))))

(event Custom|Close%20Door
  (Variables|Default|SetRotation (Transformation|GetActorRotation))
  (bind _새_트랙_0 (Timeline|타임라인_0 Play)
    (:Update
      (Transformation|SetActorRotation (Math|Rotator|MakeRotator (.roll (Variables|Default|GetRotation)) (.pitch (Variables|Default|GetRotation)) (+ (.yaw (Variables|Default|GetRotation)) _새_트랙_0))))))

(event EventBeginPlay
  (Utilities|FlowControl|Delay 2.0)
  (CallFunction|DoorOpen)
  (Utilities|FlowControl|Delay 1.0)
  (CallFunction|CloseDoor))

(event Collision|EventActorBeginOverlap
  (params (OtherActor :type Actor%20Object%20Reference)))

(event EventTick
  (params (DeltaSeconds :type Float%20%28single-precision%29)))

(fn ConstructionScript)