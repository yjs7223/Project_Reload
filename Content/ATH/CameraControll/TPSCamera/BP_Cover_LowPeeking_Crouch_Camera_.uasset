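; Third-person camera Blueprint for low peeking from cover while crouched.
; On initialization it caches the player character's cover and base input components.
; Its IsControlled check returns true only when the peeking state is low left or low right and the player is aiming, in cover and crouched.
; The file holds only this activation condition, with no camera positioning logic.
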(event EventInitalize
  (bind _m_playercharacter (Variables|Default|Getm_PlayerCharacter))
  (Variables|Default|SetCover (Actor|GetComponentbyClass _m_playercharacter "/Script/BaseClassModule.CoverComponent"))
  (Variables|Default|SetInput (Actor|GetComponentbyClass _m_playercharacter "/Script/BaseClassModule.BaseInputComponent")))

(fn IsControlled
  (bind _cover (Variables|Default|GetCover))
  (bind _returnvalue (Class|CoverComponent|GetPeekingState _cover))
  (bind _output_get (Variables|Default|SetpeekingState _returnvalue))
  (return (and (or (Utilities|Enum|Equal(Enum) _output_get "LowRight") (Utilities|Enum|Equal(Enum) _output_get "LowLeft")) (Math|Boolean|ANDBoolean (.IsAiming (Utilities|Struct|BreakInputData (Variables|/Script/BaseClassModule.BaseInputComponent|Getm_inputData (Variables|Default|GetInput)))) (Variables|/Script/BaseClassModule.CoverComponent|Getm_IsCover _cover) (Variables|/Script/Engine.Character|GetbIsCrouched (Variables|Default|Getm_PlayerCharacter))))))