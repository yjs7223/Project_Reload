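; Camera behaviour for the third-person camera that applies while the player aims from cover.
; On initialization it caches the player character's cover and base input components.
; Its IsControlled check returns true only when the input data reports aiming and the cover component reports the character is in cover.
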(event EventInitalize
  (bind _m_playercharacter (Variables|Default|Getm_PlayerCharacter))
  (Variables|Default|SetCover (Actor|GetComponentbyClass _m_playercharacter "/Script/BaseClassModule.CoverComponent"))
  (Variables|Default|SetInput (Actor|GetComponentbyClass _m_playercharacter "/Script/BaseClassModule.BaseInputComponent")))

(fn IsControlled
  (return (and (.IsAiming (Utilities|Struct|BreakInputData (Variables|/Script/BaseClassModule.BaseInputComponent|Getm_inputData (Variables|Default|GetInput)))) (Variables|/Script/BaseClassModule.CoverComponent|Getm_IsCover (Variables|Default|GetCover)))))