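; BP_CrouchMovingAiming_CameraControllPakage is a third-person camera control package for when the player crouches, moves and aims at once.
; On initialization it caches the character's input component and its custom base movement component.
; Its IsControlled check is true only while the character is crouched, the input data reports aiming, and velocity is non-zero within a small tolerance.
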(event EventInitalize
  (Variables|Default|SetInput (Actor|GetComponentbyClass (Variables|Default|Getm_PlayerCharacter) "/Script/BaseClassModule.BaseInputComponent"))
  (bind _asbase_character_movement_component (Utilities|Casting|CastToBaseCharacterMovementComponent (Variables|/Script/Engine.Character|GetCharacterMovement (Variables|Default|Getm_PlayerCharacter))))
  (Variables|Default|SetMovement _asbase_character_movement_component))

(fn IsControlled
  (return (Math|Boolean|ANDBoolean (Variables|/Script/Engine.Character|GetbIsCrouched (Variables|Default|Getm_PlayerCharacter)) (.IsAiming (Utilities|Struct|BreakInputData (Variables|/Script/BaseClassModule.BaseInputComponent|Getm_inputData (Variables|Default|GetInput)))) (Utilities|Operators|NotEqual(!=) :A (Variables|/Script/Engine.MovementComponent|GetVelocity (Variables|Default|GetMovement)) :ErrorTolerance 0.1))))