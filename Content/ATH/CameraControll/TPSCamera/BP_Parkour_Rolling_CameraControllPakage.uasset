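; BP_Parkour_Rolling_CameraControllPakage is a TPS camera control package for the parkour roll.
; On initialize it caches the player character's BPC_Parkour component.
; IsControlled reports true while that component flags both IsRoll and IsAction; its additional crouching branch requires the same two flags, so crouching does not change the result.
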(event EventInitalize
  (Variables|Default|SetBPC%20Parkour (Actor|GetComponentbyClass (Variables|Default|Getm_PlayerCharacter) "/Game/yjs/BPC_Parkour.BPC_Parkour_C")))

(fn IsControlled
  (bind _bpc_parkour (Variables|Default|GetBPC%20Parkour))
  (bind _bpc_parkour_2 (Variables|Default|GetBPC%20Parkour))
  (return (or (and (Variables|/Game/yjs/BPC_Parkour.BPC_Parkour_C|GetisRoll _bpc_parkour_2) (Variables|/Game/yjs/BPC_Parkour.BPC_Parkour_C|GetisAction _bpc_parkour_2)) (Math|Boolean|ANDBoolean (AI|Components|NavMovement|IsCrouching (Variables|Default|GetMovement)) (Variables|/Game/yjs/BPC_Parkour.BPC_Parkour_C|GetisRoll _bpc_parkour) (Variables|/Game/yjs/BPC_Parkour.BPC_Parkour_C|GetisAction _bpc_parkour)))))