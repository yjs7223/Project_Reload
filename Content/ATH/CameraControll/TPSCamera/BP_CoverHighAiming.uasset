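; BP_CoverHighAiming is a third-person camera Blueprint that decides when the high-cover aiming camera has control.
; On initialization it caches the player character's input and cover components.
; Its IsControlled check returns true only while the player is aiming, in cover, and peeking from the high left or high right position.
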(event EventInitalize
  (bind _m_playercharacter (Variables|Default|Getm_PlayerCharacter))
  (Variables|Default|SetInput (Actor|GetComponentbyClass _m_playercharacter "/Script/BaseClassModule.BaseInputComponent"))
  (Variables|Default|SetCover (Actor|GetComponentbyClass _m_playercharacter "/Script/BaseClassModule.CoverComponent")))

(fn IsControlled
  (bind _cover (Variables|Default|GetCover))
  (bind _returnvalue (Class|CoverComponent|GetPeekingState _cover))
  (bind _output_get (Variables|Default|SetNewVar_0 _returnvalue))
  (return (Math|Boolean|ANDBoolean (.IsAiming (Utilities|Struct|BreakInputData (Variables|/Script/BaseClassModule.BaseInputComponent|Getm_inputData (Variables|Default|GetInput)))) (Variables|/Script/BaseClassModule.CoverComponent|Getm_IsCover _cover) (or (Utilities|Enum|Equal(Enum) _output_get "HighRight") (Utilities|Enum|Equal(Enum) _output_get "HighLeft")))))