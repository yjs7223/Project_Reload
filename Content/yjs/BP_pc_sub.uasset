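; Player character Blueprint that handles parkour inputs and landing animations, and puts a widget on screen at BeginPlay.
; Left Alt and Space Bar call Vault and Roll on the BPCParkour component.
; OnLanded reads vertical velocity to play a normal or strong landing montage, and none for gentle landings.
; Tab starts a montage on the mesh with no asset set, disabling input and re-enabling it only on completion.
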(event EventBeginPlay
  (bind _returnvalue (UserInterface|CreateWidget 0))
  (UserInterface|Viewport|AddtoViewport _returnvalue 0))

(event EventOnLanded
  (params (Hit :type Hit%20Result%20Structure%20%28by%20ref%29))
  (bind _returnvalue (Transformation|GetVelocity))
  (if (and (< (.z _returnvalue) -3e+02) (>= (.z _returnvalue) -8e+02))
    (Animation|Montage|PlayMontage (Variables|Character|GetMesh) "/Game/NewAnim/Land/AM_JumpLandInPlace_01.AM_JumpLandInPlace_01")
    (elif (< (.z _returnvalue) -8e+02)
      (Animation|Montage|PlayMontage (Variables|Character|GetMesh) "/Game/NewAnim/Land/AM_LandStrong_01.AM_LandStrong_01"))))

(event Collision|EventActorBeginOverlap
  (params (OtherActor :type Actor%20Object%20Reference)))

(event Input|KeyboardEvents|SpaceBar
  (params (Key :type Key%20Structure))
  (:Pressed
    (Default|Roll (Variables|Default|GetBPC_Parkour))))

(event Input|KeyboardEvents|V
  (params (Key :type Key%20Structure)))

(event Input|KeyboardEvents|Tab
  (params (Key :type Key%20Structure))
  (:Pressed
    (Animation|Montage|PlayMontage (Variables|Character|GetMesh) 0
      (:then
        (Input|DisableInput 0))
      (:OnCompleted
        (Input|EnableInput 0)))))

(event Input|KeyboardEvents|LeftAlt
  (params (Key :type Key%20Structure))
  (:Pressed
    (Default|Vault (Variables|Default|GetBPC_Parkour))))

(fn ConstructionScript)