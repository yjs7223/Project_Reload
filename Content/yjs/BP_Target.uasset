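; BP_Target is a scoring target that turns hit locations into points and shows the running total on a WBP_TargetScore widget.
; HIt_Target takes the hit's Y/Z offset from the actor in world axes and scores it from 10, falling linearly with distance.
; Scores of at least 1 are added, truncated to an integer, while the total stays below 1000.
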(event Custom|HIt_Target
  (params (location :type Vector))
  (bind _returnvalue (|calcLoc location))
  (bind _returnvalue_2 (|CalcScore _returnvalue))
  (if (and (>= _returnvalue_2 1) (< (Math|Float|Truncate (+ _returnvalue_2 (Variables|Default|Getscore))) 1000))
    (bind _output_get (Variables|Default|Setscore (Math|Float|Truncate (+ _returnvalue_2 (Variables|Default|Getscore)))))
    (bind _aswbp_target_score (Utilities|Casting|CastToWBP_TargetScore (UserInterface|GetUserWidgetObject (Variables|Default|GetWidget))))
    (Default|UpdateScore _aswbp_target_score (Utilities|Text|ToText(Integer) _output_get))))

(event EventBeginPlay)

(event Collision|EventActorBeginOverlap
  (params (OtherActor :type Actor%20Object%20Reference)))

(event EventTick
  (params (DeltaSeconds :type Float%20%28single-precision%29)))

(event Collision|EventHit
  (params (MyComp :type Primitive%20Component%20Object%20Reference) (Other :type Actor%20Object%20Reference) (OtherComp :type Primitive%20Component%20Object%20Reference) (bSelfMoved :type Boolean) (HitLocation :type Vector :default "0, 0, 0") (HitNormal :type Vector :default "0, 0, 0") (NormalImpulse :type Vector :default "0, 0, 0") (Hit :type Hit%20Result%20Structure%20%28by%20ref%29)))

(fn ConstructionScript)