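; Character component that adds motion-warped parkour (vault, step up, climb, high climb) and a dodge roll.
; Vault sweeps forward at rising heights, then traces down across the obstacle for ledge, top and landing points.
; VaultMotionWarp picks a move by height, sets warp targets, and plays its montage in Flying mode, sometimes without collision.
; Roll warps a crouched montage along last input; IsAction blocks overlapping moves, and actions cancel any active cover.
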(event Custom|Vault%20Motion%20Warp
  (bind _tracer (Variables|Default|GetTracer))
  (bind _tracer_2 (Variables|Default|GetTracer))
  (bind _tracer_3 (Variables|Default|GetTracer))
  (bind _vaultmiddlepos (Variables|Default|GetVaultMiddlePos))
  (bind _motionwarping (Variables|Default|GetMotionWarping))
  (bind _motionwarping_2 (Variables|Default|GetMotionWarping))
  (bind _tracer_4 (Variables|Default|GetTracer))
  (bind _returnvalue (Transformation|GetActorRotation _tracer_4))
  (bind _returnvalue_2 (Transformation|GetActorRotation _tracer_2))
  (bind _returnvalue_3 (Transformation|GetActorRotation _tracer))
  (bind _returnvalue_4 (Math|Vector|GetForwardVector _returnvalue_3))
  ;[0.05127 0.05127 0.05127] Vault Motion Warp
  (if (not (AI|Components|NavMovement|IsFalling (Variables|Default|GetMovementComponent)))
    (if (Math|Boolean|ANDBoolean (Variables|Default|GetCanVault) (Math|Float|InRange(Float) (- (.z (Variables|Default|GetVaultLandPos)) (.z (Transformation|GetActorLocation (Variables|Default|GetTracer)))) -99999.0 4e+01) (not (Variables|Default|GetisAction)) (Math|Float|InRange(Float) (- (.z (Variables|Default|GetVaultStartPos)) (.z (- (Transformation|GetActorLocation _tracer_3) (Math|Vector|MakeVector 0.0 0.0 (Variables|/Script/Engine.CapsuleComponent|GetCapsuleHalfHeight (Actor|GetComponentbyClass _tracer_3 "/Script/Engine.CapsuleComponent")))))) -6.0 105.0))
      (Variables|Default|SetisAction true)
      (CallFunction|CancelCover)
      (Pawn|Components|CharacterMovement|SetMovementMode (Variables|Default|GetMovementComponent) "MOVE_Flying" 0)
      (Collision|SetActorEnableCollision _tracer_2 false)
      (Class|MotionWarpingComponent|AddorUpdateWarpTargetfromLocationandRotation _motionwarping_2 "VaultStart" (Math|Vector|MakeVector (.x (Variables|Default|GetVaultStartPos)) (.y (Variables|Default|GetVaultStartPos)) (- (.z (Variables|Default|GetVaultStartPos)) 78.0)) _returnvalue_2)
      (Class|MotionWarpingComponent|AddorUpdateWarpTargetfromLocationandRotation _motionwarping_2 "VaultMiddle" (Math|Vector|MakeVector (.x _vaultmiddlepos) (.y _vaultmiddlepos) (+ (.z _vaultmiddlepos) -5e+01)) _returnvalue_2)
      (Class|MotionWarpingComponent|AddorUpdateWarpTargetfromLocationandRotation _motionwarping_2 "VaultLand" (Variables|Default|GetVaultLandPos) _returnvalue_2)
      (Animation|Montage|PlayMontage (Variables|Default|GetSkeletal%20Mesh%20Component) "/Game/NewAnim/Parkour/AM_Vault.AM_Vault" 1.2
        (:OnBlendOut
          _)
        (:OnInterrupted
          _))
      (Pawn|Components|CharacterMovement|SetMovementMode (Variables|Default|GetMovementComponent) "MOVE_Walking" 0)
      (Collision|SetActorEnableCollision (Variables|Default|GetTracer) true)
      (Variables|Default|SetisAction false)
      (Variables|Default|SetCanVault false)
      (Variables|Default|SetVaultLandPos "0, 0,20000.000000")
      (Variables|Default|SetVaultStartPos "0, 0,20000.000000")
      (else
        (Variables|Default|SetVaultLandPos "0, 0,20000.000000")
        (if (Math|Boolean|ANDBoolean (Math|Float|InRange(Float) (- (.z (Variables|Default|GetVaultStartPos)) (.z (- (Transformation|GetActorLocation _tracer_3) (Math|Vector|MakeVector 0.0 0.0 (Variables|/Script/Engine.CapsuleComponent|GetCapsuleHalfHeight (Actor|GetComponentbyClass _tracer_3 "/Script/Engine.CapsuleComponent")))))) -6.0 54.0) (not (Variables|Default|GetisAction)) (Math|Float|InRange(Float) (- (.z (Variables|Default|GetClimbLand)) (.z (Transformation|GetActorLocation (Variables|Default|GetTracer)))) -5e+02 5e+02))
          (Variables|Default|SetisAction true)
          (CallFunction|CancelCover)
          (Pawn|Components|CharacterMovement|SetMovementMode (Variables|Default|GetMovementComponent) "MOVE_Flying" 0)
          (bind _output_get (Variables|Default|SetVaultStartPos (Math|Vector|MakeVector (.x (Variables|Default|GetVaultStartPos)) (.y (Variables|Default|GetVaultStartPos)) (- (.z (Variables|Default|GetVaultStartPos)) -15.0))))
          (Class|MotionWarpingComponent|AddorUpdateWarpTargetfromLocationandRotation (Variables|Default|GetMotionWarping) "StepUp" (+ _output_get (* (Math|Vector|GetForwardVector (Transformation|GetActorRotation (Variables|Default|GetTracer))) -1.0)) (Transformation|GetActorRotation (Variables|Default|GetTracer)))
          (Animation|Montage|PlayMontage (Variables|Default|GetSkeletal%20Mesh%20Component) "/Game/NewAnim/Parkour/am_jumpup.am_jumpup"
            (:OnBlendOut
              _)
            (:OnInterrupted
              _))
          (Pawn|Components|CharacterMovement|SetMovementMode (Variables|Default|GetMovementComponent) "MOVE_Walking" 0)
          (Variables|Default|SetisAction false)
          (Variables|Default|SetClimbLand "0, 0,20000.000000")
          (Variables|Default|SetStepUpCheck false)
          (elif (Math|Boolean|ANDBoolean (Math|Float|InRange(Float) (- (.z (Variables|Default|GetClimbLand)) (.z (Transformation|GetActorLocation (Variables|Default|GetTracer)))) -5e+02 5e+02) (Math|Float|InRange(Float) (- (.z (Variables|Default|GetVaultStartPos)) (.z (- (Transformation|GetActorLocation _tracer_3) (Math|Vector|MakeVector 0.0 0.0 (Variables|/Script/Engine.CapsuleComponent|GetCapsuleHalfHeight (Actor|GetComponentbyClass _tracer_3 "/Script/Engine.CapsuleComponent")))))) 54.0 1.8e+02) (not (Variables|Default|GetisAction)))
            (Variables|Default|SetisAction true)
            (CallFunction|CancelCover)
            (Pawn|Components|CharacterMovement|SetMovementMode (Variables|Default|GetMovementComponent) "MOVE_Flying" 0)
            (bind _output_get_2 (Variables|Default|SetVaultStartPos (Math|Vector|MakeVector (.x (Variables|Default|GetVaultStartPos)) (.y (Variables|Default|GetVaultStartPos)) (- (.z (Variables|Default|GetVaultStartPos)) 0.0))))
            (Class|MotionWarpingComponent|AddorUpdateWarpTargetfromLocationandRotation (Variables|Default|GetMotionWarping) "ClimbLand" (+ _output_get_2 (* (Math|Vector|GetForwardVector _returnvalue) -3e+01)) _returnvalue)
            (Animation|Montage|PlayMontage (Variables|Default|GetSkeletal%20Mesh%20Component) "/Game/NewAnim/Parkour/AM_StepUp2.AM_StepUp2" 1.1
              (:OnBlendOut
                _)
              (:OnInterrupted
                _))
            (Pawn|Components|CharacterMovement|SetMovementMode (Variables|Default|GetMovementComponent) "MOVE_Walking" 0)
            (Variables|Default|SetisAction false)
            (Variables|Default|SetClimbLand "0.000000, 0,20000.000000")
            (Variables|Default|SetStepUpCheck false)
            (Variables|/Script/Engine.MovementComponent|SetVelocity (Variables|Default|GetMovementComponent) "0, 0, 0")
            (elif (Math|Boolean|ANDBoolean (Math|Float|InRange(Float) (- (.z (Variables|Default|GetClimbLand)) (.z (Transformation|GetActorLocation (Variables|Default|GetTracer)))) -5e+02 5e+02) (Math|Float|InRange(Float) (- (.z (Variables|Default|GetVaultStartPos)) (.z (- (Transformation|GetActorLocation _tracer_3) (Math|Vector|MakeVector 0.0 0.0 (Variables|/Script/Engine.CapsuleComponent|GetCapsuleHalfHeight (Actor|GetComponentbyClass _tracer_3 "/Script/Engine.CapsuleComponent")))))) 1.8e+02 3e+02) (not (Variables|Default|GetisAction)))
              (Variables|Default|SetisAction true)
              (CallFunction|CancelCover)
              (Pawn|Components|CharacterMovement|SetMovementMode (Variables|Default|GetMovementComponent) "MOVE_Flying" 0)
              (Collision|SetActorEnableCollision _tracer false)
              (bind _output_get_3 (Variables|Default|SetVaultStartPos (Math|Vector|MakeVector (.x (Variables|Default|GetVaultStartPos)) (.y (Variables|Default|GetVaultStartPos)) (- (.z (Variables|Default|GetVaultStartPos)) 1.8e+02))))
              (Class|MotionWarpingComponent|AddorUpdateWarpTargetfromLocationandRotation _motionwarping "ClimbStart" (+ _output_get_3 (* _returnvalue_4 -1e+02)) _returnvalue_3)
              (bind _output_get_4 (Variables|Default|SetVaultStartPos (Math|Vector|MakeVector (.x (Variables|Default|GetVaultStartPos)) (.y (Variables|Default|GetVaultStartPos)) (- (.z (Variables|Default|GetVaultStartPos)) -145.0))))
              (Class|MotionWarpingComponent|AddorUpdateWarpTargetfromLocationandRotation _motionwarping "ClimbMiddle1" (+ _output_get_4 (* _returnvalue_4 -7e+01)) _returnvalue_3)
              (bind _output_get_5 (Variables|Default|SetVaultStartPos (Math|Vector|MakeVector (.x (Variables|Default|GetVaultStartPos)) (.y (Variables|Default|GetVaultStartPos)) (- (.z (Variables|Default|GetVaultStartPos)) -3e+01))))
              (Class|MotionWarpingComponent|AddorUpdateWarpTargetfromLocationandRotation _motionwarping "ClimbLand" _output_get_5 _returnvalue_3)
              (Animation|Montage|PlayMontage (Variables|Default|GetSkeletal%20Mesh%20Component) "/Game/NewAnim/Retargeter/AM_HighClimbUp.AM_HighClimbUp" 1.3
                (:OnBlendOut
                  _)
                (:OnInterrupted
                  _))
              (Pawn|Components|CharacterMovement|SetMovementMode (Variables|Default|GetMovementComponent) "MOVE_Walking" 0)
              (Collision|SetActorEnableCollision (Variables|Default|GetTracer) true)
              (Variables|Default|SetisAction false)
              (Variables|Default|SetCanVault false)
              (Variables|Default|SetClimbLand "0, 0,20000.000000"))))))))

(event Custom|OnAnimEnd_Rolling
  (Variables|Default|SetisAction false))

(event Custom|Roll
  (bind _movementcomponent (Variables|Default|GetMovementComponent))
  (bind _tracer (Variables|Default|GetTracer))
  (bind _tracer_2 (Variables|Default|GetTracer))
  (bind _tracer_3 (Variables|Default|GetTracer))
  (bind _returnvalue (Pawn|Components|PawnMovement|GetLastInputVector _movementcomponent))
  (bind _returnvalue_2 (Transformation|GetActorLocation _tracer))
  (bind _returnvalue_3 (Transformation|GetActorForwardVector _tracer_2))
  (bind _returnvalue_4 (Utilities|Operators|EqualEqual :A _returnvalue))
  (bind _returnvalue_5 (select _returnvalue_4 _returnvalue_3 _returnvalue))
  (bind _returnvalue_6 (Math|Vector|Normalize _returnvalue_5))
  (bind _returnvalue_7 (* _returnvalue_6 5e+02))
  (bind _returnvalue_8 (+ _returnvalue_2 _returnvalue_7))
  ;[0.02732 0.02732 0.02732] Dodge
  (if (not (Variables|Default|GetisAction))
    (Variables|Default|SetisAction true)
    (CallFunction|CancelCover)
    (if (not (Animation|Montage|MontageIsPlaying (Components|SkeletalMesh|GetAnimInstance (Variables|Default|GetSkeletal%20Mesh%20Component)) "/Game/NewAnim/Parkour/AM_RollForwardRootMotion.AM_RollForwardRootMotion"))
      (bind _outhit (Collision|SphereTraceByChannel _returnvalue_8 (- _returnvalue_8 "0,0,1000.000000") 5.0 "TraceTypeQuery1" false 0 "None"))
      (Transformation|SetActorRotation _tracer_3 (Math|Rotator|MakeRotator 0.0 0.0 (.yaw (Math|Rotator|MakeRotator 0.0 0.0 (.Yaw (Math|Rotator|BreakRotator (Math|Rotator|FindLookatRotation (Transformation|GetActorLocation _tracer_3) (.Location (Collision|BreakHitResult _outhit)))))))))
      (Variables|Default|SetRollSpot (.Location (Collision|BreakHitResult _outhit)))
      (bind _as캐릭터 (Utilities|Casting|CastToCharacter _tracer_3))
      (Character|Crouch _as캐릭터)
      (Class|MotionWarpingComponent|AddorUpdateWarpTargetfromLocationandRotation (Variables|Default|GetMotionWarping) "Rolling" (Variables|Default|GetRollSpot) (Math|Rotator|MakeRotator 0.0 0.0 (.yaw (Math|Rotator|MakeRotator 0.0 0.0 (.Yaw (Math|Rotator|BreakRotator (Math|Rotator|FindLookatRotation (Transformation|GetActorLocation _tracer_3) (.Location (Collision|BreakHitResult _outhit)))))))))
      (Animation|Montage|PlayMontage (Variables|Default|GetSkeletal%20Mesh%20Component) "/Game/NewAnim/Parkour/AM_RollForwardRootMotion.AM_RollForwardRootMotion"
        (:then
          (Variables|Default|SetisAction true))
        (:OnCompleted
          (Character|UnCrouch _as캐릭터 :!label _label)
          (Variables|Default|SetisAction false))
        (:OnBlendOut
          (Character|UnCrouch _as캐릭터))
        (:OnInterrupted
          (goto _label))))))

(event EventBeginPlay
  (Variables|Default|SetCanRolling true)
  (bind _as캐릭터 (Utilities|Casting|CastToCharacter (Components|GetOwner)))
  (Variables|Default|SetTracer _as캐릭터)
  (Variables|Default|SetMotionWarping (Actor|GetComponentbyClass _as캐릭터 "/Script/MotionWarping.MotionWarpingComponent"))
  (Variables|Default|SetMovementComponent (Variables|/Script/Engine.Character|GetCharacterMovement _as캐릭터))
  (Variables|Default|SetSkeletal%20Mesh%20Component (Variables|/Script/Engine.Character|GetMesh _as캐릭터)))

(event EventSetCanRolling
  (params (pCanRolling :type Boolean))
  (Variables|Default|SetCanRolling pCanRolling))

(fn Vault
  (bind _tracer (Variables|Default|GetTracer))
  (if (Variables|Default|GetCanRolling)
    (bind _as캐릭터 (Utilities|Casting|CastToCharacter _tracer))
    (bind _index (Utilities|FlowControl|ForLoopwithBreak 2 9 :!label _label)
      (:LoopBody
        (bind (_outhit _returnvalue) (Collision|SphereTraceByChannel (- (+ (- (Transformation|GetActorLocation _tracer) (Math|Vector|MakeVector 0.0 0.0 (Components|Capsule|GetScaledCapsuleHalfHeight (Variables|/Script/Engine.Character|GetCapsuleComponent _as캐릭터)))) (Math|Vector|MakeVector 0.0 0.0 (* _index 25))) (Math|Vector|MakeVector 0.0 0.0 3e+01)) (- (+ (+ (- (Transformation|GetActorLocation _tracer) (Math|Vector|MakeVector 0.0 0.0 (Components|Capsule|GetScaledCapsuleHalfHeight (Variables|/Script/Engine.Character|GetCapsuleComponent _as캐릭터)))) (Math|Vector|MakeVector 0.0 0.0 (* _index 25))) (* (Math|Vector|GetForwardVector (Transformation|GetActorRotation (Variables|Default|GetTracer))) 45.0)) (Math|Vector|MakeVector 0.0 0.0 3e+01)) 5.0 "TraceTypeQuery8" false 0 "ForDuration"))
        (if _returnvalue
          (Utilities|FlowControl|Sequence
            (:then_0
              (goto _label Break))
            (:then_1
              (bind _index_2 (Utilities|FlowControl|ForLoopwithBreak 0 5 :!label _label_2)
                (:LoopBody
                  (bind (_outhit_2 _returnvalue_2) (Collision|SphereTraceByChannel (+ (* (Math|Vector|GetForwardVector (Transformation|GetActorRotation (Variables|Default|GetTracer))) (* (+ _index_2 1) 30)) (+ (.Location (Collision|BreakHitResult _outhit)) "0.000000,0.000000,800.000000")) (- (+ (* (Math|Vector|GetForwardVector (Transformation|GetActorRotation (Variables|Default|GetTracer))) (* (+ _index_2 1) 30)) (+ (.Location (Collision|BreakHitResult _outhit)) "0.000000,0.000000,800.000000")) "0.000000,0.000000,800.000000") 5.0 "TraceTypeQuery8" false 0 "ForDuration"))
                  (if _returnvalue_2
                    (if (.bInitialOverlap (Collision|BreakHitResult _outhit_2))
                      (Variables|Default|SetCanVault false)
                      (Variables|Default|SetVaultLandPos "0, 0,20000.000000")
                      (goto _label_2 Break)
                      (else
                        (Utilities|FlowControl|Sequence
                          (:then_0
                            (if (== _index_2 0)
                              (Variables|Default|SetVaultStartPos (.Location (Collision|BreakHitResult _outhit_2)))))
                          (:then_1
                            (Variables|Default|SetVaultMiddlePos (.Location (Collision|BreakHitResult _outhit_2)))
                            (Variables|Default|SetCanVault true)
                            (if (== _index_2 1)
                              (Variables|Default|SetClimbLand (.Location (Collision|BreakHitResult _outhit_2)))))
                          (:then_2
                            (if (== _index_2 4)
                              (Variables|Default|SetStepUpCheck true))))))
                    (else
                      (bind (_outhit_3 _returnvalue_3) (Collision|LineTraceByChannel (+ (.TraceStart (Collision|BreakHitResult _outhit_2)) (* (Math|Vector|GetForwardVector (Transformation|GetActorRotation (Variables|Default|GetTracer))) 9e+01)) (- (+ (.TraceStart (Collision|BreakHitResult _outhit_2)) (* (Math|Vector|GetForwardVector (Transformation|GetActorRotation (Variables|Default|GetTracer))) 9e+01)) "0.000000,0.000000,1000.000000") "TraceTypeQuery1" false 0 "None"))
                      (if _returnvalue_3
                        (Variables|Default|SetVaultLandPos (.Location (Collision|BreakHitResult _outhit_3)))
                        (goto _label_2 Break)))))
                (:Completed
                  (CallFunction|VaultMotionWarp))))))))))

(fn CancelCover
  (bind _tracer (Variables|Default|GetTracer))
  (bind _returnvalue (Actor|GetComponentbyClass _tracer "/Script/BaseClassModule.CoverComponent"))
  (bind _as캐릭터 (Utilities|Casting|CastToCharacter (Variables|Default|GetTracer)))
  (Utilities|IsValid _returnvalue
    (:Is%20Valid
      (Class|CoverComponent|StopCover _returnvalue)
      (Character|UnCrouch _as캐릭터)
      (return))))

(fn IsRolling
  (return (Variables|Default|GetisAction)))