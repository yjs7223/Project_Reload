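; Interactive trigger that raises a referenced elevator actor a fixed height above its starting position once Interact is called.
; BeginPlay derives the start and end locations, then Tick advances a timer and eases the elevator between them, moving this actor to the same height.
; Player camera shakes mark departure, rumble during the ride and fire once near arrival.
; The CalcNowTime function clears the Start flag after the travel time elapses.
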(event EventBeginPlay
  (bind _elevatoractor (Variables|Default|GetElevatorActor))
  (bind _returnvalue (Transformation|GetActorLocation _elevatoractor))
  (bind (_x _y _z) (Math|Vector|BreakVector _returnvalue))
  (Utilities|IsValid _elevatoractor
    (:Is%20Valid
      ;[1 1 1] 시작지점 지정(현재위치로 자동지정)
      (Variables|Default|SetStartLoc _returnvalue)
      ;[1 1 1] 도착지점 지정
      (Variables|Default|SetEndLoc (Math|Vector|MakeVector _x _y (+ _z 5e+02)))
      ;[1 1 1] 도착시간 설정
      (Variables|Default|SetArriveTime 1e+01))
    (:Is%20Not%20Valid
      (Development|PrintString "none ElevatorActor" true true "(R=0.000000,G=0.660000,B=1.000000,A=1.000000)" 2e+01))))

(event Collision|EventActorBeginOverlap
  (params (OtherActor :type Actor%20Object%20Reference)))

(event EventTick
  (params (DeltaSeconds :type Float%20%28single-precision%29))
  (bind _returnvalue (Transformation|GetActorLocation))
  (bind _nowtime (Variables|Default|GetNowTime))
  (bind _arrivetime (Variables|Default|GetArriveTime))
  (bind _startloc (Variables|Default|GetStartLoc))
  (bind _endloc (Variables|Default|GetEndLoc))
  (bind _returnvalue_2 (/ _nowtime _arrivetime))
  (bind _result (Math|Interpolation|Ease "EaseInOut" _returnvalue_2 _startloc _endloc 3.0))
  (if (Variables|Default|GetStart)
    (|CalcNowTime DeltaSeconds)
    (Transformation|SetActorLocation (Variables|Default|GetElevatorActor) _result false false)
    (Transformation|SetActorLocation (Math|Vector|MakeVector (.x _returnvalue) (.y _returnvalue) (.Z (Math|Vector|BreakVector _result))) false false)
    (if (>= (/ (Variables|Default|GetNowTime) (Variables|Default|GetArriveTime)) 0.85)
      (Utilities|FlowControl|DoOnce false
        (:Completed
          (Class|MatineeCameraShake|StartMatineeCameraShake (Game|GetPlayerCameraManager 0) "/Game/yjs/FX/BP_ElevatorShake.BP_ElevatorShake_C" 0.1 "CameraLocal" "0, 0, 0")))
      (else
        (Class|MatineeCameraShake|StartMatineeCameraShake (Game|GetPlayerCameraManager 0) "/Game/ThirdPersonKit/Blueprints/CameraShakes/BP_PistolCameraShake.BP_PistolCameraShake_C" 0.05 "CameraLocal" "0, 0, 0")))))

(event EventInteract
  (Variables|Default|SetStart true)
  (Utilities|FlowControl|Delay 0.3)
  (Class|MatineeCameraShake|StartMatineeCameraShake (Game|GetPlayerCameraManager 0) "/Game/yjs/FX/BP_ElevatorShake.BP_ElevatorShake_C" 0.1 "CameraLocal" "0, 0, 0"))

(fn ConstructionScript)