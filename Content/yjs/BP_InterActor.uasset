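; BP_InterActor is an interactive actor whose cube slides along world Y when the click flag on its rWBP_click widget is set.
; Tick polls the widget component's BClick and accumulates delta time into Move while it is true.
; Each frame adds Move to the cube's Y position, so the slide accelerates and depends on frame rate.
; Once Move exceeds 1.5 seconds, it resets and clears the flag.
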(event EventBeginPlay)

(event Collision|EventActorBeginOverlap
  (params (OtherActor :type Actor%20Object%20Reference)))

(event EventTick
  (params (DeltaSeconds :type Float%20%28single-precision%29))
  (bind _cube (Variables|Default|GetCube))
  (bind _returnvalue (Transformation|GetWorldLocation _cube))
  (bind _aswbp_click (Utilities|Casting|CastTorWBP_click (UserInterface|GetUserWidgetObject (Variables|Default|GetWidget))))
  (if (Variables|/Game/yjs/UI/Legacy/rWBP_click.rWBP_click_C|Getb_click _aswbp_click)
    (bind _output_get (Variables|Default|SetMove (+ (Variables|Default|GetMove) DeltaSeconds)))
    (if (<= _output_get 1.5)
      (Transformation|SetWorldLocation _cube (Math|Vector|MakeVector (.x _returnvalue) (+ (.y _returnvalue) (Variables|Default|GetMove)) (.z _returnvalue)) false false)
      (else
        (Variables|Default|SetMove 0.0)
        (Variables|/Game/yjs/UI/Legacy/rWBP_click.rWBP_click_C|Setb_click _aswbp_click false)))))

(fn ConstructionScript)