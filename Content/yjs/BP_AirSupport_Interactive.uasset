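; Interactive air-support actor that sends the level's A-10 (BP_West_Attack_A10) on an attack pass once its InteractiveComponent is flagged Interactive.
; BeginPlay caches the plane; Tick accumulates time and lerps it from its current position toward GoalLoc at constant altitude, using a growing alpha.
; After a short flight time, a DoOnce spawns three staggered Niagara explosions, offset along Y from the plane's current position.
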(event EventBeginPlay
  (bind _returnvalue (Actor|GetActorOfClass "/Game/VigilanteContent/Vehicles/West_Attack_A10/BP_West_Attack_A10.BP_West_Attack_A10_C"))
  (Variables|Default|SetA10_ref _returnvalue))

(event Collision|EventActorBeginOverlap
  (params (OtherActor :type Actor%20Object%20Reference)))

(event EventTick
  (params (DeltaSeconds :type Float%20%28single-precision%29))
  (bind _a10_ref (Variables|Default|GetA10_ref))
  (bind _goal_loc (Variables|Default|Getgoal_loc))
  (bind _a10_ref_2 (Variables|Default|GetA10_ref))
  (bind _a10_ref_3 (Variables|Default|GetA10_ref))
  (bind _a10_ref_4 (Variables|Default|GetA10_ref))
  (bind _returnvalue (Transformation|GetActorLocation _a10_ref_2))
  (bind _returnvalue_2 (Transformation|GetActorLocation _a10_ref_3))
  (bind _returnvalue_3 (Transformation|GetActorLocation _a10_ref_4))
  (bind _returnvalue_4 (Transformation|GetActorLocation _a10_ref))
  (if (Variables|/Script/BaseClassModule.InteractiveComponent|GetbInteractive (Actor|GetComponentbyClass "/Script/BaseClassModule.InteractiveComponent"))
    (Variables|Default|Setalpha (+ DeltaSeconds (Variables|Default|Getalpha)))
    (Transformation|SetActorLocation _a10_ref (Math|Vector|Lerp(Vector) (Math|Vector|MakeVector (.x _returnvalue_4) (.y _returnvalue_4) (.z _returnvalue_4)) (Math|Vector|MakeVector (.x _goal_loc) (.y _goal_loc) (.z _returnvalue_4)) (/ (Variables|Default|Getalpha) 4e+02)) false false)
    (if (>= (Variables|Default|Getalpha) 1.5)
      (Utilities|FlowControl|DoOnce false
        (:Completed
          (Niagara|SpawnSystematLocation "/Game/Aws/NS_Car_Expl_1.NS_Car_Expl_1" (Math|Vector|MakeVector (.x _returnvalue_2) (+ (.y _returnvalue_2) 5e+03) 0.0) "0, 0, 0" "3.000000,3.000000,3.000000")
          (Utilities|FlowControl|Delay 0.2)
          (Niagara|SpawnSystematLocation "/Game/Aws/NS_Car_Expl_1.NS_Car_Expl_1" (Math|Vector|MakeVector (.x _returnvalue_3) (+ (.y _returnvalue_3) 5e+03) 0.0) "0, 0, 0" "3.000000,3.000000,3.000000")
          (Utilities|FlowControl|Delay 0.2)
          (Niagara|SpawnSystematLocation "/Game/Aws/NS_Car_Expl_1.NS_Car_Expl_1" (Math|Vector|MakeVector (.x _returnvalue) (+ (.y _returnvalue) 5e+03) 0.0) "0, 0, 0" "3.000000,3.000000,3.000000"))))))

(fn ConstructionScript)