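; Player character Blueprint that drives crosshair, ammo, HP and navigation UI, plus interact and debug damage/infinite-ammo keys.
; BeginPlay creates the crosshair and sets starting HP; Tick consumes the weapon component's hit flag to trigger targets and hit markers, flagging headshots.
; Accumulated timers fade ammo and HP widgets after input or damage and animate the E-triggered navi progress bars.
; Ammo and HP widgets follow weapon and body mesh sockets every frame.
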(event EventBeginPlay
  ;[0.4365 0.4354 1] BeginPlay
  (Utilities|FlowControl|Sequence
    (:then_0
      (bind _returnvalue (UserInterface|CreateWidget "/Game/yjs/UI/Crosshair.Crosshair_C"))
      (bind _output_get (Variables|Default|SetCrossHair _returnvalue))
      (UserInterface|Viewport|AddtoViewport _output_get 0)
      (Class|StatComponent|SetHP (Actor|GetComponentbyClass "/Script/PlayerModule.PlayerStatComponent") 1e+03))))

(event Collision|EventActorBeginOverlap
  (params (OtherActor :type Actor%20Object%20Reference)))

(event EventTick
  (params (DeltaSeconds :type Float%20%28single-precision%29))
  ;[1 0.464 0.04688] Tick
  (Utilities|FlowControl|Sequence
    (:then_0
      (|CheckIshit
        (:true
          (Utilities|FlowControl|Sequence
            (:then_0
              (|TargetHIt))
            (:then_1
              _))
          (Default|HItUIEvent (Variables|Default|GetCrossHair) (Variables|/Script/PlayerModule.PlayerWeaponComponent|Getheadhit (Actor|GetComponentbyClass "/Script/PlayerModule.PlayerWeaponComponent"))))))
    (:then_1
      (|CalcAlpha DeltaSeconds))
    (:then_2
      (|HUDOnOff)
      (|UI_Transform))))

(event Input|KeyboardEvents|T
  (params (Key :type Key%20Structure :default "None"))
  (bind _returnvalue (Actor|GetComponentbyClass "/Script/PlayerModule.PlayerWeaponComponent"))
  ;[0.2247 1 0.9203] ammoInfinity
  (:Pressed
    (if (Variables|/Script/PlayerModule.PlayerWeaponComponent|Getammoinfinite _returnvalue)
      (Variables|/Script/PlayerModule.PlayerWeaponComponent|Setammoinfinite _returnvalue false)
      (else
        (Variables|/Script/PlayerModule.PlayerWeaponComponent|Setammoinfinite _returnvalue true)))))

(event Input|KeyboardEvents|E
  (params (Key :type Key%20Structure :default "None"))
  ;[0.2937 1 0.3786] Navi
  (:Pressed
    (Variables|Default|SetNavi_toggle true)))

(event Input|KeyboardEvents|G
  (params (Key :type Key%20Structure :default "None"))
  ;[1 0.1146 0.1146] Attacked Test
  (:Pressed
    (Class|StatComponent|Attacked (Actor|GetComponentbyClass "/Script/PlayerModule.PlayerStatComponent") 2e+01)))

(event Input|KeyboardEvents|F
  (params (Key :type Key%20Structure :default "None"))
  (bind _interactor (Variables|Default|GetInterActor))
  ;[1 0.2984 0.7753] Interaction
  (:Pressed
    (Utilities|IsValid _interactor
      (:Is%20Valid
        (bind _asbp_inter_actor_2 (Utilities|Casting|CastToBP_InterActor2 _interactor))
        (Default|InteractEvent _asbp_inter_actor_2)))))

(fn ConstructionScript)