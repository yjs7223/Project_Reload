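; BP_InterActor2 is an interactable actor that shows a proximity-based widget and can be nudged along Y.
; Each tick it fades the widget out between 450 and 500 units from the player's pawn.
; Within that range limit it registers itself as the InterActor on BP_pc, without clearing it on exit.
; MoveActor rechecks the distance, then shifts the actor a small step or prints that it is too far.
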(event Custom|MoveActor
  (bind _returnvalue (Transformation|GetActorLocation))
  (if (<= (Math|Vector|VectorLength (- (Transformation|GetActorLocation) (Transformation|GetActorLocation (Pawn|GetControlledPawn (Game|GetPlayerController 0))))) 5e+02)
    (Development|PrintString "move")
    (Transformation|SetActorLocation (Math|Vector|MakeVector (.x _returnvalue) (+ (.y _returnvalue) 1e+01) (.z _returnvalue)) false false)
    (else
      (Development|PrintString "too Far"))))

(event EventBeginPlay)

(event Collision|EventActorBeginOverlap
  (params (OtherActor :type Actor%20Object%20Reference)))

(event EventTick
  (params (DeltaSeconds :type Float%20%28single-precision%29))
  (bind _returnvalue (Game|GetPlayerController 0))
  (bind _returnvalue_2 (Transformation|GetActorLocation))
  (bind _returnvalue_3 (Pawn|GetControlledPawn _returnvalue))
  (bind _returnvalue_4 (Transformation|GetActorLocation _returnvalue_3))
  (bind _returnvalue_5 (- _returnvalue_2 _returnvalue_4))
  (bind _returnvalue_6 (Math|Vector|VectorLength _returnvalue_5))
  (if true
    (Widget|SetRenderOpacity (UserInterface|GetUserWidgetObject (Variables|Default|GetWidget)) (Math|Float|Lerp 1.0 0.0 (Math|Float|Clamp(Float) (/ (- _returnvalue_6 4.5e+02) 5e+01))))
    (if (<= _returnvalue_6 5e+02)
      (bind _asbp_pc (Utilities|Casting|CastToBP_pc _returnvalue_3))
      (Variables|/Game/yjs/BP_pc.BP_pc_C|SetInterActor _asbp_pc self))))

(fn ConstructionScript)