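; Example missile actor for the RocketAttackFX effects that flies toward a target location and detonates.
; Tick sweeps the Munitions component forward by a fixed step per frame, not scaled by delta time, and snaps its rotation toward TargetLocation.
; A blocking hit spawns explosion and aftermath Niagara systems; a timeout from BeginPlay spawns a countered effect instead.
; Both paths share cleanup that destroys Munitions, deactivates Niagara, then destroys the actor after a delay.
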(event OnComponentHit(Munitions)
  (params (HitComponent :type Primitive%20Component%20Object%20Reference) (OtherActor :type Actor%20Object%20Reference) (OtherComp :type Primitive%20Component%20Object%20Reference) (NormalImpulse :type Vector :default "0, 0, 0") (Hit :type Hit%20Result%20Structure%20%28by%20ref%29))
  (bind (_bblockinghit _binitialoverlap _time _distance _location _impactpoint _normal _impactnormal) (Collision|BreakHitResult Hit))
  (bind _munitions (Variables|Default|GetMunitions))
  (bind _returnvalue (Math|Conversions|RotationFromXVector _impactnormal))
  (if _bblockinghit
    (Niagara|SpawnSystematLocation "/Game/RocketAttackFX/FX/Vehicle/NS_RocketVehicle_Explosion.NS_RocketVehicle_Explosion" _impactpoint _returnvalue "5.000000,5.000000,5.000000")
    (Niagara|SpawnSystematLocation "/Game/RocketAttackFX/FX/Handheld/NS_RocketAttack_Aftermath.NS_RocketAttack_Aftermath" _impactpoint _returnvalue "2.000000,2.000000,2.000000")
    (Utilities|IsValid _munitions
      (:Is%20Valid
        (Components|DestroyComponent _munitions)
        (Components|Activation|Deactivate (Variables|Default|GetNiagara))
        (Utilities|FlowControl|Delay 1.0)
        (Actor|DestroyActor)))))

(event EventTick
  (params (DeltaSeconds :type Float%20%28single-precision%29))
  (bind _munitions (Variables|Default|GetMunitions))
  (Utilities|IsValid _munitions
    (:Is%20Valid
      (Transformation|AddLocalOffset _munitions "15.000000, 0, 0" true false)
      (Utilities|IsValid _munitions
        (:Is%20Valid
          (Transformation|SetWorldRotation _munitions (Math|Rotator|FindLookatRotation (Transformation|GetWorldLocation _munitions) (Variables|Default|GetTargetLocation)) true false))))))

(event EventBeginPlay
  (bind _munitions (Variables|Default|GetMunitions))
  (bind _munitions_2 (Variables|Default|GetMunitions))
  (Utilities|FlowControl|Delay 4.0)
  (Utilities|IsValid _munitions
    (:Is%20Valid
      (Niagara|SpawnSystematLocation "/Game/RocketAttackFX/FX/Handheld/NS_RocketAttack_Countered.NS_RocketAttack_Countered" (Transformation|GetWorldLocation _munitions))
      (Utilities|IsValid _munitions_2
        (:Is%20Valid
          (Components|DestroyComponent _munitions_2)
          (Components|Activation|Deactivate (Variables|Default|GetNiagara))
          (Utilities|FlowControl|Delay 1.0)
          (Actor|DestroyActor))))))

(fn ConstructionScript)