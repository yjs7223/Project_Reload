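; BP_RocketAttack_Example is a demo rocket projectile that showcases the RocketAttack Niagara effects.
; Tick sweeps the Munitions component forward by a fixed local offset each frame, so its speed depends on frame rate.
; A blocking hit spawns Explosion and Aftermath systems aligned to the impact normal, then destroys the actor.
; If still alive two seconds after BeginPlay, it spawns the Countered effect at its position and destroys itself.
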(event OnComponentHit(Munitions)
  (params (HitComponent :type Primitive%20Component%20Object%20Reference) (OtherActor :type Actor%20Object%20Reference) (OtherComp :type Primitive%20Component%20Object%20Reference) (NormalImpulse :type Vector :default "0, 0, 0") (Hit :type Hit%20Result%20Structure%20%28by%20ref%29))
  (bind (_bblockinghit _binitialoverlap _time _distance _location _impactpoint _normal _impactnormal) (Collision|BreakHitResult Hit))
  (bind _returnvalue (Math|Conversions|RotationFromXVector _impactnormal))
  (if _bblockinghit
    (Niagara|SpawnSystematLocation "/Game/RocketAttackFX/FX/Handheld/NS_RocketAttack_Explosion.NS_RocketAttack_Explosion" _impactpoint _returnvalue)
    (Niagara|SpawnSystematLocation "/Game/RocketAttackFX/FX/Handheld/NS_RocketAttack_Aftermath.NS_RocketAttack_Aftermath" _impactpoint _returnvalue))
  (Actor|DestroyActor))

(event EventTick
  (params (DeltaSeconds :type Float%20%28single-precision%29))
  (Transformation|AddLocalOffset (Variables|Default|GetMunitions) "50.000000, 0, 0" true false))

(event EventBeginPlay
  (Utilities|FlowControl|Delay 2.0)
  (Niagara|SpawnSystematLocation "/Game/RocketAttackFX/FX/Handheld/NS_RocketAttack_Countered.NS_RocketAttack_Countered" (Transformation|GetWorldLocation (Variables|Default|GetMunitions)))
  (Actor|DestroyActor))

(fn ConstructionScript)