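; First-person demo character for showing off rocket and missile attack effects, with timeline-driven WASD movement, mouse look and jump.
; Mouse buttons and E/R spawn handheld or vehicle rockets and missiles at GunPoint, restarting the matching launch effects.
; Each Tick, a camera line trace positions TargetBase, whose location steers the latest missile of each type.
; The target bounce and scale timelines are never triggered.
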(event EventTick
  (params (DeltaSeconds :type Float%20%28single-precision%29))
  (bind _returnvalue (Game|GetPlayerCameraManager 0))
  (bind _targetbase (Variables|Default|GetTargetBase))
  (bind _refmissile (Variables|Default|GetRefMissile))
  (bind _targetbase_2 (Variables|Default|GetTargetBase))
  (bind _refbigmissile (Variables|Default|GetRefBigMissile))
  (bind _returnvalue_2 (Transformation|GetWorldLocation _targetbase_2))
  (bind _transformcomponent (Variables|/Script/Engine.PlayerCameraManager|GetTransformComponent _returnvalue))
  (bind _returnvalue_3 (Transformation|GetWorldLocation _transformcomponent))
  ;[1 1 1] Target point location and trace
  (Utilities|FlowControl|Sequence
    (:then_0
      (Utilities|IsValid _refmissile
        (:Is%20Valid
          (Variables|/Game/RocketAttackFX/Blueprints/BP_MissileAttack_Example.BP_MissileAttack_Example_C|SetTargetLocation _refmissile _returnvalue_2))))
    (:then_1
      (bind _outhit (Collision|LineTraceByChannel _returnvalue_3 (+ _returnvalue_3 (* (Math|Vector|GetForwardVector (Transformation|GetWorldRotation _transformcomponent)) (Math|Conversions|ToVector(Float) 1e+04))) "TraceTypeQuery1" false (Utilities|Array|MakeArray (Variables|Default|GetRefMissile) (Variables|Default|GetRefBigMissile)) "None"))
      (if (.bBlockingHit (Collision|BreakHitResult _outhit))
        (Transformation|SetWorldTransform _targetbase (Math|Transform|MakeTransform (.Location (Collision|BreakHitResult _outhit)) "0, 0, 0" "1.000000,1.000000,1.000000") false false)
        (else
          (Transformation|SetWorldTransform _targetbase (Math|Transform|MakeTransform (.TraceEnd (Collision|BreakHitResult _outhit)) "0, 0, 0" "1.000000,1.000000,1.000000") false false))))
    (:then_2
      (Utilities|IsValid _refbigmissile
        (:Is%20Valid
          (Variables|/Game/RocketAttackFX/Blueprints/BP_MissileVehicle_Example.BP_MissileVehicle_Example_C|SetTargetLocation _refbigmissile _returnvalue_2))))))

(event Input|MouseEvents|MouseX
  (params (AxisValue :type Float%20%28single-precision%29))
  ;[1 1 1] Movement controls
  (Pawn|Input|AddControllerYawInput AxisValue))

(event Input|MouseEvents|MouseY
  (params (AxisValue :type Float%20%28single-precision%29))
  ;[1 1 1] Movement controls
  (Pawn|Input|AddControllerPitchInput (* AxisValue -1.0)))

(event Input|KeyboardEvents|W
  (params (Key :type Key%20Structure))
  ;[1 1 1] Movement controls
  (:Pressed
    (Timeline|Timeline_0 PlayFromStart
      (:Update
        (Pawn|Input|AddMovementInput (* (Math|Vector|GetForwardVector (Variables|Default|GetCamera)) 1e+01) 1.0 false))))
  (:Released
    (Timeline|Timeline_0 Stop)))

(event Input|MouseEvents|RightMouseButton
  (params (Key :type Key%20Structure))
  (bind _gunpoint (Variables|Default|GetGunPoint))
  ;[1 1 1] Shoot rockets and missiles
  (:Pressed
    (Game|SpawnActorfromClass "/Game/RocketAttackFX/Blueprints/BP_RocketVehicle_Example.BP_RocketVehicle_Example_C" (Math|Transform|MakeTransform (Transformation|GetWorldLocation _gunpoint) (Transformation|GetWorldRotation _gunpoint) "1.000000,1.000000,1.000000") "AlwaysSpawn" 0 0)
    (Components|Activation|SetActive (Variables|Default|GetVehicle__Fumes) true true)))

(event Input|KeyboardEvents|R
  (params (Key :type Key%20Structure))
  (bind _gunpoint (Variables|Default|GetGunPoint))
  ;[1 1 1] Shoot rockets and missiles
  (:Pressed
    (bind _returnvalue (Game|SpawnActorfromClass "/Game/RocketAttackFX/Blueprints/BP_MissileVehicle_Example.BP_MissileVehicle_Example_C" (Math|Transform|MakeTransform (Transformation|GetWorldLocation _gunpoint) (Transformation|GetWorldRotation _gunpoint) "1.000000,1.000000,1.000000") "AlwaysSpawn" 0 0))
    (Variables|Default|SetRefBigMissile _returnvalue)
    (Components|Activation|SetActive (Variables|Default|GetVehicle__Fumes) true true)))

(event Input|KeyboardEvents|A
  (params (Key :type Key%20Structure))
  ;[1 1 1] Movement controls
  (:Pressed
    (Timeline|Timeline_1 PlayFromStart
      (:Update
        (Pawn|Input|AddMovementInput (* (Math|Vector|GetRightVector (Variables|Default|GetCamera)) -1e+01) 1.0 false))))
  (:Released
    (Timeline|Timeline_1 Stop)))

(event Input|KeyboardEvents|S
  (params (Key :type Key%20Structure))
  ;[1 1 1] Movement controls
  (:Pressed
    (Timeline|Timeline_2 PlayFromStart
      (:Update
        (Pawn|Input|AddMovementInput (* (Math|Vector|GetForwardVector (Variables|Default|GetCamera)) -1e+01) 1.0 false))))
  (:Released
    (Timeline|Timeline_2 Stop)))

(event Input|KeyboardEvents|SpaceBar
  (params (Key :type Key%20Structure))
  ;[1 1 1] Movement controls
  (:Pressed
    (Character|Jump)))

(event Input|KeyboardEvents|D
  (params (Key :type Key%20Structure))
  ;[1 1 1] Movement controls
  (:Pressed
    (Timeline|Timeline_3 PlayFromStart
      (:Update
        (Pawn|Input|AddMovementInput (* (Math|Vector|GetRightVector (Variables|Default|GetCamera)) 1e+01) 1.0 false))))
  (:Released
    (Timeline|Timeline_3 Stop)))

(event Input|MouseEvents|LeftMouseButton
  (params (Key :type Key%20Structure))
  (bind _gunpoint (Variables|Default|GetGunPoint))
  ;[1 1 1] Shoot rockets and missiles
  (:Pressed
    (Game|SpawnActorfromClass "/Game/RocketAttackFX/Blueprints/BP_RocketAttack_Example.BP_RocketAttack_Example_C" (Math|Transform|MakeTransform (Transformation|GetWorldLocation _gunpoint) (Transformation|GetWorldRotation _gunpoint) "1.000000,1.000000,1.000000") "AlwaysSpawn" 0 0)
    (Components|Activation|SetActive (Variables|Default|GetHandheld_BackExhaust) true true)))

(event Input|KeyboardEvents|E
  (params (Key :type Key%20Structure))
  (bind _gunpoint (Variables|Default|GetGunPoint))
  ;[1 1 1] Shoot rockets and missiles
  (:Pressed
    (bind _returnvalue (Game|SpawnActorfromClass "/Game/RocketAttackFX/Blueprints/BP_MissileAttack_Example.BP_MissileAttack_Example_C" (Math|Transform|MakeTransform (Transformation|GetWorldLocation _gunpoint) (Transformation|GetWorldRotation _gunpoint) "1.000000,1.000000,1.000000") "AlwaysSpawn" 0 0))
    (Variables|Default|SetRefMissile _returnvalue)
    (Components|Activation|SetActive (Variables|Default|GetHandheld_BackExhaust) true true)))

(fn ConstructionScript)