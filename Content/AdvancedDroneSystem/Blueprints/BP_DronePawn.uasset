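; Player-controlled drone pawn with speed boost, scroll zoom, first/third-person toggle, projectile firing, high-res screenshots and exit back to the character.
; Tick spins four propellers, matches actor yaw to the camera and blends in-air sound pitch from boost and velocity.
; Night vision, thermal and glitch effects each overwrite camera post-process settings with a new dynamic material instance.
; DroneSettings supplies tuning, and a WBP_Drone widget provides HUD and animations.
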(event Custom|End%20Drone%20Mode
  (bind _inairsound (Variables|Default|GetInAirSound))
  ;[0 0 0] Enable Drone Mode
  (CallFunction|GlitchEffect)
  (Utilities|FlowControl|DoOnce false
    (:Completed
      (Utilities|FlowControl|Delay 0.2)
      (Pawn|Possess (Game|GetPlayerController 0) (Variables|Default|GetCharacterReference))
      (Widget|RemovefromParent (Variables|Default|GetWBP_Drone))
      (Audio|Components|Audio|Stop _inairsound)
      (Components|DestroyComponent _inairsound)
      (Actor|DestroyActor))))

(event Custom|GlitchEffect
  ;[0.005591 0 0.01562] Glitch Effect
  (Variables|Default|SetGlitchEnable 1.0)
  (Utilities|FlowControl|DoOnce false :!label _label
    (:Completed
      (bind _returnvalue (Rendering|Material|CreateDynamicMaterialInstance "/Game/AdvancedDroneSystem/Materials/MaterialInstances/MI_Glitch.MI_Glitch" "None" "None" :!class /Script/Engine.KismetMaterialLibrary))
      (Variables|/Script/Engine.CameraComponent|SetPostProcessSettings (Variables|Default|GetCamera) (Utilities|Struct|MakePostProcessSettings (Utilities|Struct|MakeWeightedBlendables (Utilities|Array|MakeArray (Utilities|Struct|MakeWeightedBlendable (Variables|Default|GetGlitchEnable) _returnvalue)))))
      (Utilities|FlowControl|Delay 0.2)
      (Variables|Default|SetGlitchEnable 0.0)
      (bind _returnvalue_2 (Rendering|Material|CreateDynamicMaterialInstance "/Game/AdvancedDroneSystem/Materials/MaterialInstances/MI_Glitch.MI_Glitch" "None" "None" :!class /Script/Engine.KismetMaterialLibrary))
      (Variables|/Script/Engine.CameraComponent|SetPostProcessSettings (Variables|Default|GetCamera) (Utilities|Struct|MakePostProcessSettings (Utilities|Struct|MakeWeightedBlendables (Utilities|Array|MakeArray (Utilities|Struct|MakeWeightedBlendable (Variables|Default|GetGlitchEnable) _returnvalue_2)))))
      (goto _label Reset))))

(event Custom|DroneSound
  ;[0 0 0] DroneSound
  (bind _returnvalue (Audio|CreateSound2D "/Game/AdvancedDroneSystem/Sound/A_InAir_Cue.A_InAir_Cue" 1.0 1.0 0.0 0))
  (bind _output_get (Variables|Default|SetInAirSound _returnvalue))
  (Audio|Components|Audio|Play _output_get 0.0)
  (bind _newtrack_0 (Timeline|Volume PlayFromStart)
    (:Update
      (Audio|Components|Audio|SetVolumeMultiplier _output_get _newtrack_0 :!class /Script/Engine.AudioComponent))))

(event Custom|UpdateDroneSound
  (bind _inairsound (Variables|Default|GetInAirSound))
  ;[0.005591 0 0.01562] Drone Sound
  (Utilities|IsValid _inairsound
    (:Is%20Valid
      (Audio|Components|Audio|SetPitchMultiplier _inairsound (Math|Interpolation|FInterpTo (Variables|/Script/Engine.AudioComponent|GetPitchMultiplier _inairsound) (select (Game|Player|IsInputKeyDown (Game|GetPlayerController 0) "LeftShift") 1.5 (select (> (Math|Vector|VectorLength (Transformation|GetVelocity)) 0.0) 1.0 0.9)) (Utilities|Time|GetWorldDeltaSeconds) 2.0))
      (Variables|Default|SetPropellerSpeed (select (Game|Player|IsInputKeyDown (Game|GetPlayerController 0) "LeftShift") 1e+02 (select (> (Math|Vector|VectorLength (Transformation|GetVelocity)) 0.0) 5e+01 4e+01))))))

(event EventBeginPlay
  (bind _returnvalue (Game|GetPlayerCameraManager 0))
  (bind _dronesettings (Variables|Default|GetDroneSettings))
  (bind (_pitchmin _pitchmax) (Utilities|Struct|BreakF_DroneSettings _dronesettings))
  ;[0.005591 0 0.01562] Begin Play
  (Utilities|FlowControl|Sequence
    (:then_0
      (bind _aswbp_drone (Utilities|Casting|CastToWBP_Drone (UserInterface|GetUserWidgetObject (Variables|Default|GetWidget))))
      (Variables|/Game/AdvancedDroneSystem/Blueprints/Widgerts/WBP_Drone.WBP_Drone_C|SetDroneRef _aswbp_drone self)
      (Variables|Default|SetWBP_Drone _aswbp_drone)
      (CallFunction|GlitchEffect))
    (:then_1
      ;;[0.005591 0 0.01562] Clamp Pitch View
      (Variables|/Script/Engine.PlayerCameraManager|SetViewPitchMin _returnvalue _pitchmin)
      (Variables|/Script/Engine.PlayerCameraManager|SetViewPitchMax _returnvalue _pitchmax)
      (CallFunction|DroneSound))))

(event EventTick
  (params (DeltaSeconds :type Float%20%28single-precision%29))
  ;[0.005591 0 0.01562] Event Tick
  (Utilities|FlowControl|Sequence
    (:then_0
      (CallFunction|UpdatePropeller))
    (:then_1
      (CallFunction|SetFollowCameraRotation))
    (:then_2
      (CallFunction|UpdateDroneSound))))

(event Input|MouseEvents|MouseWheelAxis
  (params (AxisValue :type Float%20%28single-precision%29))
  (bind _dronesettings (Variables|Default|GetDroneSettings))
  (bind _camera (Variables|Default|GetCamera))
  (bind (_zoommin _zoommax _zoomspeed) (Utilities|Struct|BreakF_DroneSettings _dronesettings))
  ;[0.005591 0 0.01562] Zoom
  (Variables|Default|SetZoomRange (Math|Float|Clamp(Float) (+ (Variables|Default|GetZoomRange) (* (* AxisValue -1.0) _zoomspeed)) _zoommin _zoommax))
  (Camera|SetFieldOfView _camera (Math|Interpolation|FInterpTo (Variables|/Script/Engine.CameraComponent|GetFieldOfView _camera) (Variables|Default|GetZoomRange) (Utilities|Time|GetWorldDeltaSeconds) 5.0)))

(event Input|KeyboardEvents|Z
  (params (Key :type Key%20Structure :default "None"))
  (bind _shootpoint (Variables|Default|GetShootPoint))
  (bind _returnvalue (Transformation|GetWorldLocation _shootpoint))
  (:Pressed
    (Game|SpawnActorfromClass "/Game/Boss/Projectile/BP_DroneProjectile.BP_DroneProjectile_C" (Math|Transform|MakeTransform _returnvalue (Camera|GetCameraRotation (Game|GetPlayerCameraManager 0)) "1.000000,1.000000,1.000000") "Undefined" 0 0 false 2e+03 3e+03 0)
    (Audio|PlaySoundatLocation "/Game/ExplosionSoundPack/ExplosionSoundsMONO/Wavs/explosion_large_10.explosion_large_10" _returnvalue "0, 0, 0" 1.0 1.0 0.0 0 0 0 0)))

(event Input|KeyboardEvents|R
  (params (Key :type Key%20Structure :default "None"))
  ;[0.005591 0 0.01562] NightVision
  (:Pressed
    (Utilities|FlowControl|FlipFlop
      (:A
        (Variables|Default|SetNightVisionEnable 1.0)
        (Variables|Default|SetNightVisionEnabled? true))
      (:B
        (Variables|Default|SetNightVisionEnable 0.0)
        (Variables|Default|SetNightVisionEnabled? false)))
    (bind _returnvalue (Rendering|Material|CreateDynamicMaterialInstance "/Game/AdvancedDroneSystem/Materials/MaterialInstances/MI_NightVision_01.MI_NightVision_01" "None" "None" :!class /Script/Engine.KismetMaterialLibrary))
    (Variables|/Script/Engine.CameraComponent|SetPostProcessSettings (Variables|Default|GetCamera) (Utilities|Struct|MakePostProcessSettings (Utilities|Struct|MakeWeightedBlendables (Utilities|Array|MakeArray (Utilities|Struct|MakeWeightedBlendable (Variables|Default|GetNightVisionEnable) _returnvalue)))))))

(event Input|KeyboardEvents|T
  (params (Key :type Key%20Structure :default "None"))
  ;[0.005591 0 0.01562] ThermalVision
  (:Pressed
    (Utilities|FlowControl|FlipFlop
      (:A
        (Variables|Default|SetThermalEnable 1.0)
        (Variables|Default|SetThermalEnabled? true))
      (:B
        (Variables|Default|SetThermalEnable 0.0)
        (Variables|Default|SetThermalEnabled? false)))
    (bind _returnvalue (Rendering|Material|CreateDynamicMaterialInstance "/Game/AdvancedDroneSystem/Materials/MaterialInstances/M_ThermalVisionMaster_Inst.M_ThermalVisionMaster_Inst" "None" "None" :!class /Script/Engine.KismetMaterialLibrary))
    (Variables|/Script/Engine.CameraComponent|SetPostProcessSettings (Variables|Default|GetCamera) (Utilities|Struct|MakePostProcessSettings (Utilities|Struct|MakeWeightedBlendables (Utilities|Array|MakeArray (Utilities|Struct|MakeWeightedBlendable (Variables|Default|GetThermalEnable) _returnvalue)))))))

(event Input|KeyboardEvents|LeftShift
  (params (Key :type Key%20Structure :default "None"))
  (bind _movementcomponent (Variables|Default|GetMovementComponent))
  (bind _dronesettings (Variables|Default|GetDroneSettings))
  (bind (_currentspeed _maxspeed) (Utilities|Struct|BreakF_DroneSettings _dronesettings))
  (bind _as플로팅_폰_이동 (Utilities|Casting|CastToFloatingPawnMovement _movementcomponent))
  ;[0.005591 0 0.01562] SpeedUp
  (:Pressed
    (Variables|/Script/Engine.FloatingPawnMovement|SetMaxSpeed _as플로팅_폰_이동 _maxspeed))
  (:Released
    (Variables|/Script/Engine.FloatingPawnMovement|SetMaxSpeed _as플로팅_폰_이동 _currentspeed)))

(event Input|KeyboardEvents|V
  (params (Key :type Key%20Structure :default "None"))
  (bind _inairsound (Variables|Default|GetInAirSound))
  ;[0 0 0] Enable Drone Mode
  (:Pressed
    (CallFunction|GlitchEffect)
    (Utilities|FlowControl|DoOnce false
      (:Completed
        (Utilities|FlowControl|Delay 0.2)
        (Pawn|Possess (Game|GetPlayerController 0) (Variables|Default|GetCharacterReference))
        (Widget|RemovefromParent (Variables|Default|GetWBP_Drone))
        (Audio|Components|Audio|Stop _inairsound)
        (Components|DestroyComponent _inairsound)
        (Actor|DestroyActor)))))

(event Input|KeyboardEvents|A
  (params (Key :type Key%20Structure :default "None"))
  ;[0.005591 0 0.01562] RightVector
  (:Pressed
    (Variables|Default|SetMoveRight%20 -1.0))
  (:Released
    (Variables|Default|SetMoveRight%20 0.0)))

(event Input|KeyboardEvents|D
  (params (Key :type Key%20Structure :default "None"))
  ;[0.005591 0 0.01562] RightVector
  (:Pressed
    (Variables|Default|SetMoveRight%20 1.0))
  (:Released
    (Variables|Default|SetMoveRight%20 0.0)))

(event Input|KeyboardEvents|M
  (params (Key :type Key%20Structure :default "None"))
  (bind _wbp_drone (Variables|Default|GetWBP_Drone))
  (bind _springarm (Variables|Default|GetSpringArm))
  (bind _collisioncomponent (Variables|Default|GetCollisionComponent))
  ;[0.005591 0 0.01562] Set Fpp / 3rd
  (:Pressed
    (Utilities|FlowControl|FlipFlop
      (:A
        (Variables|/Script/Engine.SpringArmComponent|SetSocketOffset _springarm "-300.000000, 0,20.000000")
        (Components|Sphere|SetSphereRadius _collisioncomponent 2e+01 true)
        (Default|PlayBeginAnimation _wbp_drone "Forward")
        (Widget|SetVisibility (Variables|/Game/AdvancedDroneSystem/Blueprints/Widgerts/WBP_Drone.WBP_Drone_C|GetHUD_01 _wbp_drone) "Hidden"))
      (:B
        (Variables|/Script/Engine.SpringArmComponent|SetSocketOffset _springarm "0, 0, 0")
        (Components|Sphere|SetSphereRadius _collisioncomponent 5e+01 true)
        (Default|PlayBeginAnimation (Variables|Default|GetWBP_Drone) "Forward")
        (Widget|SetVisibility (Variables|/Game/AdvancedDroneSystem/Blueprints/Widgerts/WBP_Drone.WBP_Drone_C|GetHUD_01 _wbp_drone) "Visible")))))

(event Input|KeyboardEvents|G
  (params (Key :type Key%20Structure :default "None"))
  ;[0 0 0] Take Screenshot
  (:Pressed
    (Utilities|TakeScreenshot)))

(fn ConstructionScript)

(fn UpdatePropeller
  ;[0.005591 0 0.01562] Update Propeller
  (for _array_element (Utilities|Array|MakeArray (Variables|Default|GetPropeller_01) (Variables|Default|GetPropeller_02) (Variables|Default|GetPropeller_03) (Variables|Default|GetPropeller_04))
    (Transformation|AddRelativeRotation _array_element (Math|Rotator|MakeRotator 0.0 0.0 (Variables|Default|GetPropellerSpeed)) false false)))

(fn SetFollowCameraRotation
  (bind _returnvalue (Transformation|GetActorRotation))
  ;[0.005591 0 0.01562] SetFollowCameraRotation
  (Transformation|SetActorRotation (Math|Rotator|MakeRotator (.roll _returnvalue) (.pitch _returnvalue) (.yaw (Camera|GetCameraRotation (Game|GetPlayerCameraManager 0))))))