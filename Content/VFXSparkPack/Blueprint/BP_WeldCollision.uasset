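; Welding spark effect actor that switches on when it touches a surface, judging by the VFX it drives.
; Each tick a short downward sphere trace looks for world, pawn, physics, vehicle or destructible objects.
; A hit orients VFXWeldNoLight to the surface normal, activates the effect, applies the LightOn visibility and starts playback once per contact.
; Losing contact resets that gate, deactivates the effect, applies LightOff and stops playback.
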(event Custom|OnLoop)

(event EventTick
  (params (DeltaSeconds :type Float%20%28single-precision%29))
  (bind _returnvalue (Transformation|GetWorldLocation))
  (bind (_outhit _returnvalue_2) (Collision|SphereTraceForObjects _returnvalue (+ _returnvalue "0.000000,0.000000,-20.000000") 5e+01 (Utilities|Array|MakeArray "ObjectTypeQuery1" "ObjectTypeQuery2" "ObjectTypeQuery3" "ObjectTypeQuery4" "ObjectTypeQuery5" "ObjectTypeQuery6") false 0 "None"))
  (if _returnvalue_2
    (Transformation|SetWorldRotation (Variables|Default|GetVFX_WeldNoLight) (Math|Rotator|MakeRotationfromAxes (.Normal (Collision|BreakHitResult _outhit)) "0, 0, 0" "0, 0, 0") false false)
    (Components|Activation|Activate false)
    (Rendering|SetVisibility (Variables|Default|GetLightOn) false)
    (|DoOnceMultiInput :!label _label
      (:A%20Out
        (Audio|Components|Audio|Play 0.0)
        (Audio|Components|Audio|Play 0.0)))
    (else
      (Utilities|FlowControl|Sequence
        (:then_0
          (goto _label Reset%20In))
        (:then_1
          (Components|Activation|Deactivate)
          (Rendering|SetVisibility (Variables|Default|GetLightOff) false)
          (Audio|Components|Audio|Stop))))))

(fn ConstructionScript)