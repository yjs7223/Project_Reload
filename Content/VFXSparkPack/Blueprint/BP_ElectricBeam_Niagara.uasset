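; Electric arc VFX actor that throws random lightning zaps from a central sphere onto nearby surfaces.
; On BeginPlay a looping timer calls ShootArc, firing three near-identical zap events.
; Each line-traces toward a randomly offset dummy target, spawning Niagara beam and impact systems on a hit and briefly flashing a light.
; The construction script applies exposed core light, impact light and beam settings.
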(event Custom|CE_ShootArc
  (bind _beam_time_min (Variables|Effects|GetBeam%20Time%20Min))
  (bind _beam_time_max (Variables|Effects|GetBeam%20Time%20Max))
  (bind _returnvalue (Math|Random|RandomFloatinRange _beam_time_min _beam_time_max))
  ;[1 1 1] Beam1
  (Utilities|FlowControl|Sequence
    (:then_0
      (bind _output_get (Variables|Default|SetNewVar0 (* (Math|Random|RandomUnitVector) (Math|Random|RandomFloatinRange (Variables|Effects|GetBeam%20Radius%201%20Min) (Variables|Effects|GetBeam%20Radius%201%20Max)))))
      (Transformation|SetRelativeLocation (Variables|Default|GetDummyTarget) _output_get false false)
      (bind (_outhit _returnvalue_2) (Collision|LineTraceByChannel (Transformation|GetWorldLocation (Variables|Default|GetSphere)) (Transformation|GetWorldLocation (Variables|Default|GetDummyTarget)) "TraceTypeQuery2" false 0 "None"))
      (if _returnvalue_2
        (bind _returnvalue_3 (Niagara|SpawnSystemAttached "/Game/VFXSparkPack/Niagara/NS_ElectricBeam.NS_ElectricBeam" (Variables|Default|GetSphere) "None" "0, 0, 0" "0, 0, 0" "KeepRelativeOffset" true))
        (Effects|Components|ParticleSystem|SetVectorParameter _returnvalue_3 "BeamEnd" (.ImpactPoint (Collision|BreakHitResult _outhit)))
        (Niagara|SetNiagaraVariable(Float) _returnvalue_3 "Lifetime" _returnvalue)
        (bind _returnvalue_4 (Niagara|SpawnSystematLocation "/Game/VFXSparkPack/Niagara/NS_ElectricBeamHit_move.NS_ElectricBeamHit_move" (.ImpactPoint (Collision|BreakHitResult _outhit)) (Math|Rotator|MakeRotationfromAxes (.Normal (Collision|BreakHitResult _outhit)) "0, 0, 0" "0, 0, 0")))
        (Utilities|FlowControl|Sequence
          (:then_0
            (Effects|Components|ParticleSystem|SetColorParameter _returnvalue_4 "SparkColor" (Variables|EffectColorSettings|GetEffect%20Color))
            (Effects|Components|ParticleSystem|SetFloatParameter _returnvalue_4 "SparkColorScale" (Variables|EffectColorSettings|GetBeam%20Color%20Intensity))
            (Effects|Components|ParticleSystem|SetFloatParameter _returnvalue_4 "SparkAlphaScale" (Variables|EffectColorSettings|GetBeam%20Alpha%20Intensity))
            (Effects|Components|ParticleSystem|SetColorParameter _returnvalue_3 "SparkColor" (Variables|EffectColorSettings|GetEffect%20Color))
            (Effects|Components|ParticleSystem|SetFloatParameter _returnvalue_3 "SparkColorScale" (Variables|EffectColorSettings|GetBeam%20Color%20Intensity))
            (Effects|Components|ParticleSystem|SetFloatParameter _returnvalue_3 "SparkAlphaScale" (Variables|EffectColorSettings|GetBeam%20Alpha%20Intensity)))
          (:then_1
            (Rendering|SetVisibility (Variables|Default|GetLightOn) false)
            (Transformation|SetWorldLocation (.ImpactPoint (Collision|BreakHitResult _outhit)) false false)
            (Utilities|FlowControl|RetriggerableDelay 0.2)
            (Rendering|SetVisibility (Variables|Default|GetLightOff) false)
            (Components|Activation|Deactivate (Variables|Default|GetNiagara_Beam))))
        (else
          (bind _returnvalue_5 (Niagara|SpawnSystemAttached "/Game/VFXSparkPack/Niagara/NS_ElectricBeam.NS_ElectricBeam" (Variables|Default|GetSphere) "None" "0, 0, 0" "0, 0, 0" "KeepRelativeOffset" true))
          (Effects|Components|ParticleSystem|SetVectorParameter _returnvalue_5 "BeamEnd" (Transformation|GetWorldLocation (Variables|Default|GetSphere)))
          (Niagara|SetNiagaraVariable(Float) _returnvalue_5 "Lifetime" _returnvalue)
          (Rendering|SetVisibility (Variables|Default|GetLightOff) false)
          (Components|Activation|Deactivate (Variables|Default|GetNiagara_Beam)))))))

(event Custom|CE_ShootArc2
  (bind _niagara_beam (Variables|Default|GetNiagara_Beam))
  ;[1 1 1] second zap
  (Utilities|FlowControl|Sequence
    (:then_0
      (bind _output_get (Variables|Default|SetNewVar0 (* (Math|Random|RandomUnitVector) (Math|Random|RandomFloatinRange (Variables|Effects|GetBeam%20Radius%201%20Min) (Variables|Effects|GetBeam%20Radius%201%20Max)))))
      (Transformation|SetRelativeLocation (Variables|Default|GetDummyTarget) _output_get false false)
      (bind (_outhit _returnvalue) (Collision|LineTraceByChannel (Transformation|GetWorldLocation (Variables|Default|GetSphere)) (Transformation|GetWorldLocation (Variables|Default|GetDummyTarget)) "TraceTypeQuery2" false 0 "None"))
      (if _returnvalue
        (bind _returnvalue_2 (Niagara|SpawnSystemAttached "/Game/VFXSparkPack/Niagara/NS_ElectricBeam.NS_ElectricBeam" (Variables|Default|GetNiagara_Beam) "None" "0, 0, 0" "0, 0, 0" "KeepRelativeOffset" false))
        (Effects|Components|ParticleSystem|SetVectorParameter _returnvalue_2 "BeamEnd" (.ImpactPoint (Collision|BreakHitResult _outhit)))
        (Niagara|SetNiagaraVariable(Float) _returnvalue_2 "Lifetime" (Math|Random|RandomFloatinRange (Variables|Effects|GetBeam%20Time%20Min) (Variables|Effects|GetBeam%20Time%20Max)))
        (bind _returnvalue_3 (Niagara|SpawnSystematLocation "/Game/VFXSparkPack/Niagara/NS_ElectricBeamHit_move.NS_ElectricBeamHit_move" (.ImpactPoint (Collision|BreakHitResult _outhit)) (Math|Rotator|MakeRotationfromAxes (.Normal (Collision|BreakHitResult _outhit)) "0, 0, 0" "0, 0, 0")))
        (Utilities|FlowControl|Sequence
          (:then_0
            (Effects|Components|ParticleSystem|SetColorParameter _returnvalue_3 "SparkColor" (Variables|EffectColorSettings|GetEffect%20Color))
            (Effects|Components|ParticleSystem|SetFloatParameter _returnvalue_3 "SparkColorScale" (Variables|EffectColorSettings|GetBeam%20Color%20Intensity))
            (Effects|Components|ParticleSystem|SetFloatParameter _returnvalue_3 "SparkAlphaScale" (Variables|EffectColorSettings|GetBeam%20Alpha%20Intensity))
            (Effects|Components|ParticleSystem|SetColorParameter _returnvalue_2 "SparkColor" (Variables|EffectColorSettings|GetEffect%20Color))
            (Effects|Components|ParticleSystem|SetFloatParameter _returnvalue_2 "SparkColorScale" (Variables|EffectColorSettings|GetBeam%20Color%20Intensity))
            (Effects|Components|ParticleSystem|SetFloatParameter _returnvalue_2 "SparkAlphaScale" (Variables|EffectColorSettings|GetBeam%20Alpha%20Intensity)))
          (:then_1
            (Rendering|SetVisibility (Variables|Default|GetLightOn) false)
            (Transformation|SetWorldLocation (.ImpactPoint (Collision|BreakHitResult _outhit)) false false)
            (Utilities|FlowControl|RetriggerableDelay 0.2)
            (Rendering|SetVisibility (Variables|Default|GetLightOff) false)
            (Components|Activation|Deactivate (Variables|Default|GetNiagara_Beam))))
        (else
          (Effects|Components|ParticleSystem|SetVectorParameter _niagara_beam "User.BeamEnd" (Transformation|GetWorldLocation (Variables|Default|GetSphere)))
          (Components|Activation|Deactivate _niagara_beam)
          (Rendering|SetVisibility (Variables|Default|GetLightOff) false)
          (Components|Activation|Deactivate (Variables|Default|GetNiagara_Beam)))))))

(event Custom|CE_shootArc3
  (bind _niagara_beam (Variables|Default|GetNiagara_Beam))
  ;[1 1 1] third zap
  (Utilities|FlowControl|Sequence
    (:then_0
      (bind _output_get (Variables|Default|SetNewVar0 (* (Math|Random|RandomUnitVector) (Math|Random|RandomFloatinRange (Variables|Effects|GetBeam%20Radius%201%20Min) (Variables|Effects|GetBeam%20Radius%201%20Max)))))
      (Transformation|SetRelativeLocation (Variables|Default|GetDummyTarget) _output_get false false)
      (bind (_outhit _returnvalue) (Collision|LineTraceByChannel (Transformation|GetWorldLocation (Variables|Default|GetSphere)) (Transformation|GetWorldLocation (Variables|Default|GetDummyTarget)) "TraceTypeQuery2" false 0 "None"))
      (if _returnvalue
        (bind _returnvalue_2 (Niagara|SpawnSystemAttached "/Game/VFXSparkPack/Niagara/NS_ElectricBeam.NS_ElectricBeam" (Variables|Default|GetNiagara_Beam) "None" "0, 0, 0" "0, 0, 0" "KeepRelativeOffset" false))
        (Effects|Components|ParticleSystem|SetVectorParameter _returnvalue_2 "BeamEnd" (.ImpactPoint (Collision|BreakHitResult _outhit)))
        (Niagara|SetNiagaraVariable(Float) _returnvalue_2 "Lifetime" (Math|Random|RandomFloatinRange (Variables|Effects|GetBeam%20Time%20Min) (Variables|Effects|GetBeam%20Time%20Max)))
        (bind _returnvalue_3 (Niagara|SpawnSystematLocation "/Game/VFXSparkPack/Niagara/NS_ElectricBeamHit_move.NS_ElectricBeamHit_move" (.ImpactPoint (Collision|BreakHitResult _outhit)) (Math|Rotator|MakeRotationfromAxes (.Normal (Collision|BreakHitResult _outhit)) "0, 0, 0" "0, 0, 0")))
        (Utilities|FlowControl|Sequence
          (:then_0
            (Effects|Components|ParticleSystem|SetColorParameter _returnvalue_3 "SparkColor" (Variables|EffectColorSettings|GetEffect%20Color))
            (Effects|Components|ParticleSystem|SetFloatParameter _returnvalue_3 "SparkColorScale" (Variables|EffectColorSettings|GetBeam%20Color%20Intensity))
            (Effects|Components|ParticleSystem|SetFloatParameter _returnvalue_3 "SparkAlphaScale" (Variables|EffectColorSettings|GetBeam%20Alpha%20Intensity))
            (Effects|Components|ParticleSystem|SetColorParameter _returnvalue_2 "SparkColor" (Variables|EffectColorSettings|GetEffect%20Color))
            (Effects|Components|ParticleSystem|SetFloatParameter _returnvalue_2 "SparkColorScale" (Variables|EffectColorSettings|GetBeam%20Color%20Intensity))
            (Effects|Components|ParticleSystem|SetFloatParameter _returnvalue_2 "SparkAlphaScale" (Variables|EffectColorSettings|GetBeam%20Alpha%20Intensity)))
          (:then_1
            (Rendering|SetVisibility (Variables|Default|GetLightOn) false)
            (Transformation|SetWorldLocation (.ImpactPoint (Collision|BreakHitResult _outhit)) false false)
            (Utilities|FlowControl|RetriggerableDelay 0.2)
            (Rendering|SetVisibility (Variables|Default|GetLightOff) false)
            (Components|Activation|Deactivate (Variables|Default|GetNiagara_Beam))))
        (else
          (Effects|Components|ParticleSystem|SetVectorParameter _niagara_beam "User.BeamEnd" (Transformation|GetWorldLocation (Variables|Default|GetSphere)))
          (Components|Activation|Deactivate _niagara_beam)
          (Rendering|SetVisibility (Variables|Default|GetLightOff) false)
          (Components|Activation|Deactivate (Variables|Default|GetNiagara_Beam)))))))

(event EventBeginPlay
  ;[1 1 1] link to function
  (Utilities|Time|SetTimerbyFunctionName 0 "ShootArc" (Math|Random|RandomFloatinRange (Variables|Effects|GetBeam%20Time%20Min) (Variables|Effects|GetBeam%20Time%20Max)) true))

(fn ConstructionScript
  (bind _niagara_beam (Variables|Default|GetNiagara_Beam))
  (bind _corelight (Variables|Default|GetCoreLight))
  (bind _impactlight (Variables|Default|GetImpactLight))
  ;[1 1 1] Core Light Settings
  (Rendering|Components|Light|SetLightColor _corelight (Variables|CoreLightSettings|GetCore%20Light%20Color) true)
  (Rendering|Components|Light|SetIntensity _corelight (Variables|CoreLightSettings|GetCore%20Light%20Intensity))
  (Rendering|Lighting|SetAttenuationRadius _corelight (Variables|CoreLightSettings|GetCore%20Light%20Attenuation%20Radius))
  (Rendering|Components|Light|SetCastShadows _corelight (Variables|CoreLightSettings|GetCore%20Light%20Cast%20Shadows))
  (Transformation|AddRelativeLocation _corelight (Variables|CoreLightSettings|GetCore%20Light%20Location) false false)
  (Rendering|Components|Light|SetLightFunctionMaterial _corelight (Variables|CoreLightSettings|GetCore%20Light%20Function))
  ;[1 1 1] Impact Light settings
  (Rendering|Components|Light|SetLightColor _impactlight (Variables|ImpactLightSettings|GetImpact%20Light%20Color) true)
  (Rendering|Components|Light|SetIntensity _impactlight (Variables|ImpactLightSettings|GetImpact%20Light%20Intensity))
  (Rendering|Lighting|SetAttenuationRadius _impactlight (Variables|ImpactLightSettings|GetImpact%20Light%20Attenuation%20Radius))
  (Rendering|Components|Light|SetCastShadows _impactlight (Variables|ImpactLightSettings|GetImpact%20Light%20Cast%20Shadows))
  (Rendering|Components|Light|SetLightFunctionMaterial _impactlight (Variables|ImpactLightSettings|GetImpact%20Light%20Function))
  ;[1 1 1] Beam Settings
  (Effects|Components|ParticleSystem|SetColorParameter _niagara_beam "SparkColor" (Variables|EffectColorSettings|GetEffect%20Color))
  (Effects|Components|ParticleSystem|SetFloatParameter _niagara_beam "SparkColorScale" (Variables|EffectColorSettings|GetBeam%20Color%20Intensity))
  (Effects|Components|ParticleSystem|SetFloatParameter _niagara_beam "SparkAlphaScale" (Variables|EffectColorSettings|GetBeam%20Alpha%20Intensity)))

(fn ShootArc
  (CallFunction|CEShootArc)
  (CallFunction|CEShootArc2)
  (CallFunction|CEShootArc3))