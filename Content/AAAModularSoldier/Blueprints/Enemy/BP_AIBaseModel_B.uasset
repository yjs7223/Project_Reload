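; BP_AIBaseModel_B is an enemy AI soldier model assembled from modular clothing and gear meshes.
; Its construction script links parts through master pose components so each follows the animation of a parent piece.
; Gloves and shirt patches follow the body Mesh, while helmet, pants, vest, shoulder, war belt and balaclava pieces each drive their own accessories and patches.
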(fn ConstructionScript
  (Class|SkinnedMeshComponent|SetMasterPoseComponent (Variables|Default|GetGloves) (Variables|Character|GetMesh) false)
  (Class|SkinnedMeshComponent|SetMasterPoseComponent (Variables|Default|GetHelmetPreset) (Variables|Default|GetHelmet) false)
  (Class|SkinnedMeshComponent|SetMasterPoseComponent (Variables|Default|GetBoots) (Variables|Default|GetPants) false)
  (Class|SkinnedMeshComponent|SetMasterPoseComponent (Variables|Default|GetVestPatches) (Variables|Default|GetVest) false)
  (Class|SkinnedMeshComponent|SetMasterPoseComponent (Variables|Default|GetTacticalShouldersPatch) (Variables|Default|GetTacticalShoulders) false)
  (Class|SkinnedMeshComponent|SetMasterPoseComponent (Variables|Default|GetWarBeltPreset) (Variables|Default|GetWarBelt) false)
  (Class|SkinnedMeshComponent|SetMasterPoseComponent (Variables|Default|GetHat) (Variables|Default|GetBalaclava) false))