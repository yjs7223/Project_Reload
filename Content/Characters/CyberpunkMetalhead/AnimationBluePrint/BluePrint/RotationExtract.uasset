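; Animation modifier that bakes a RotationYaw float curve from a sequence's root bone rotation.
; On apply, it steps through the sequence's frames and reads the root yaw with root motion extraction.
; Each key stores that yaw clamp-remapped against the final frame's yaw, giving a normalized turn-progress curve that ends at one when the clip has a net yaw.
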(event EventOnApply
  (params (AnimationSequence :type Anim%20Sequence%20Object%20Reference))
  (bind _output_get (Variables|Default|SetAnimationSequence AnimationSequence))
  (Class|AnimationBlueprintLibrary|AddCurve _output_get "RotationYaw" "RCT_Float" false)
  (for _index (range 0 (Class|AnimationBlueprintLibrary|GetNumFrames (Variables|Default|GetAnimationSequence)))
    (Class|AnimationBlueprintLibrary|AddFloatCurveKey (Variables|Default|GetAnimationSequence) "RotationYaw" (Class|AnimationBlueprintLibrary|GetTimeatFrame (Variables|Default|GetAnimationSequence) _index) (Math|Float|MapRangeClamped (.yaw (.rotation (Class|AnimationBlueprintLibrary|GetBonePoseforFrame (Variables|Default|GetAnimationSequence) "root" _index true))) 0.0 (.yaw (.rotation (Class|AnimationBlueprintLibrary|GetBonePoseforFrame (Variables|Default|GetAnimationSequence) "root" (Class|AnimationBlueprintLibrary|GetNumFrames (Variables|Default|GetAnimationSequence)) true))) 0.0 1.0))))