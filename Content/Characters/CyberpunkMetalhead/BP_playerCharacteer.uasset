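; Player character Blueprint that handles parkour, landing reactions and commands to a companion drone.
; LeftAlt and Space trigger Vault and Roll on BPCParkour, while Tab starts a montage call that disables input until completion.
; Landing selects a normal or strong montage by vertical fall speed.
; Q box-traces from the player's viewpoint and passes the hit location to the MascotDrone's SlecetMove.
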(event EventBeginPlay)

(event EventOnLanded
  (params (Hit :type Hit%20Result%20Structure%20%28by%20ref%29))
  (bind _returnvalue (Transformation|GetVelocity))
  (if (and (< (.z _returnvalue) -3e+02) (>= (.z _returnvalue) -8e+02))
    (Animation|Montage|PlayMontage (Variables|Character|GetMesh) "/Game/NewAnim/Land/AM_JumpLandInPlace_01.AM_JumpLandInPlace_01")
    (elif (< (.z _returnvalue) -8e+02)
      (Animation|Montage|PlayMontage (Variables|Character|GetMesh) "/Game/NewAnim/Land/AM_LandStrong_01.AM_LandStrong_01"))))

(event Collision|EventActorBeginOverlap
  (params (OtherActor :type Actor%20Object%20Reference)))

(event Input|AxisEvents|InputAxisTurnRight/LeftMouse
  (params (AxisValue :type Float%20%28single-precision%29))
  (Variables|Default|SetTurnRate AxisValue))

(event Input|KeyboardEvents|Q
  (params (Key :type Key%20Structure :default "None"))
  (bind _returnvalue (Game|GetPlayerCharacter 0))
  (bind _returnvalue_2 (Pawn|GetController _returnvalue))
  (bind (_location _rotation) (Pawn|GetPlayerViewPoint _returnvalue_2))
  (:Pressed
    (bind _outhit (Collision|BoxTraceByChannel _location (+ _location (* (Math|Rotator|GetRotationXVector _rotation) 9999.0)) "10.000000,10.000000,10.000000" "0, 0, 0" "TraceTypeQuery1" false 0 "ForDuration"))
    (bind _returnvalue_3 (Actor|GetActorOfClass "/Game/_sjs/Drone/MascotDrone.MascotDrone_C"))
    (bind _asmascot_drone (Utilities|Casting|CastToMascotDrone _returnvalue_3))
    (Default|SlecetMove _asmascot_drone (.Location (Collision|BreakHitResult _outhit)))))

(event Input|KeyboardEvents|SpaceBar
  (params (Key :type Key%20Structure :default "None"))
  (:Pressed
    (Default|Roll (Variables|Default|GetBPC_Parkour))))

(event Input|KeyboardEvents|Tab
  (params (Key :type Key%20Structure :default "None"))
  (:Pressed
    (Animation|Montage|PlayMontage (Variables|Character|GetMesh) 0
      (:then
        (Input|DisableInput 0))
      (:OnCompleted
        (Input|EnableInput 0)))))

(event Input|KeyboardEvents|LeftAlt
  (params (Key :type Key%20Structure :default "None"))
  (:Pressed
    (Default|Vault (Variables|Default|GetBPC_Parkour))))

(fn ConstructionScript)