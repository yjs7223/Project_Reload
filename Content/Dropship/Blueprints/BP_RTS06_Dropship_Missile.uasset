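; Dropship missile actor that animates its own launch and flight as a visual projectile, with no hit or damage logic.
; On BeginPlay it brightens the glow on its dynamic material and shows the point light and rocket flare.
; A timeline then accelerates it along local Y while easing out an initial drop and leveling pitch, without sweeping for collision.
; The actor destroys itself when the timeline finishes.
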(event EventBeginPlay
  (bind _returnvalue (Transformation|GetActorRotation))
  (bind (_roll _pitch _yaw) (Math|Rotator|BreakRotator _returnvalue))
  (Rendering|Material|SetScalarParameterValue (Variables|Default|GetMaterial) "Glow_Multiply" 2e+01 :!class /Script/Engine.MaterialInstanceDynamic)
  (Rendering|SetVisibility (Variables|Default|GetPointLight) true false)
  (Development|SetHiddeninGame (Variables|Default|GetSM_RocketFlare) false false)
  (bind (_direction _movement_lerp _drop _rotation) (Timeline|Timeline_0 PlayFromStart)
    (:Update
      (Transformation|AddActorLocalOffset (Math|Vector|MakeVector 0.0 (Math|Float|Lerp 1e+01 1e+03 _movement_lerp) (Math|Float|Lerp -5.0 0.0 _drop)) false false)
      (Transformation|SetActorRotation (Math|Rotator|MakeRotator _roll (Math|Float|Lerp _pitch 0.0 _rotation) _yaw)))
    (:Finished
      (Actor|DestroyActor))))

(fn ConstructionScript
  (bind _sm_rts06_dropship_missile (Variables|Default|GetSM_RTS06_Dropship_Missile))
  (bind _returnvalue (Rendering|Material|CreateDynamicMaterialInstance _sm_rts06_dropship_missile 0 "/Game/Dropship/Materials/MI_RTS06_Dropship_Weapons.MI_RTS06_Dropship_Weapons" :!class /Script/Engine.PrimitiveComponent))
  (bind _output_get (Variables|Default|SetMaterial _returnvalue))
  (Rendering|Material|SetMaterial _sm_rts06_dropship_missile 0 _output_get))