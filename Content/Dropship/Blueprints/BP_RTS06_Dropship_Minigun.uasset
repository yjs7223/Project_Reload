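; BP_RTS06_Dropship_Minigun is a dropship minigun actor that animates its barrel spin when firing.
; Fire and Stop events toggle a Firing flag.
; Each Tick interpolates the spin speed toward a firing rate or zero and adds it as local pitch rotation to the barrel mesh, giving gradual spin-up and spin-down.
; It handles only the visual spin, with no projectile or damage logic.
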(event Custom|Fire
  (Variables|Default|SetFiring true))

(event Custom|Stop
  (Variables|Default|SetFiring false))

(event EventBeginPlay)

(event Collision|EventActorBeginOverlap
  (params (OtherActor :type Actor%20Object%20Reference)))

(event EventTick
  (params (DeltaSeconds :type Float%20%28single-precision%29))
  (bind _output_get (Variables|Default|SetCurrent%20Rotation (Math|Interpolation|FInterpTo (Variables|Default|GetCurrent%20Rotation) (Math|Float|SelectFloat 2e+01 0.0 (Variables|Default|GetFiring)) (Utilities|Time|GetWorldDeltaSeconds) 1.0)))
  (Transformation|AddLocalRotation (Variables|Default|GetSM_RTS06_Dropship_MinigunBarrel) (Math|Rotator|MakeRotator 0.0 _output_get 0.0) false false))

(fn ConstructionScript)