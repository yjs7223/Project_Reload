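; Small dropship missile actor that launches itself on BeginPlay and destroys itself when its flight ends.
; The construction script creates a dynamic weapons material, whose glow is raised at launch alongside the point light and rocket flare.
; A timeline drives per-update local offsets, ramping forward speed along Y and easing out an initial downward drop.
; Movement does not sweep, and the graph contains no hit or damage logic.
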(event EventBeginPlay
  (Rendering|Material|SetScalarParameterValue (Variables|Default|GetMaterial) "Glow_Multiply" 2e+01 :!class /Script/Engine.MaterialInstanceDynamic)
  (Rendering|SetVisibility (Variables|Default|GetPointLight) true false)
  (Development|SetHiddeninGame (Variables|Default|GetSM_RocketFlare) false false)
  (bind (_direction _movement_lerp _drop) (Timeline|Timeline_0 PlayFromStart)
    (:Update
      (Transformation|AddActorLocalOffset (Math|Vector|MakeVector 0.0 (Math|Float|Lerp 1e+01 1e+03 _movement_lerp) (Math|Float|Lerp -5.0 0.0 _drop)) false false))
    (:Finished
      (Actor|DestroyActor))))

(fn ConstructionScript
  (bind _sm_rts06_dropship_missile_small (Variables|Default|GetSM_RTS06_Dropship_Missile_Small))
  (bind _returnvalue (Rendering|Material|CreateDynamicMaterialInstance _sm_rts06_dropship_missile_small 0 "/Game/Dropship/Materials/MI_RTS06_Dropship_Weapons.MI_RTS06_Dropship_Weapons" :!class /Script/Engine.PrimitiveComponent))
  (bind _output_get (Variables|Default|SetMaterial _returnvalue))
  (Rendering|Material|SetMaterial _sm_rts06_dropship_missile_small 0 _output_get))