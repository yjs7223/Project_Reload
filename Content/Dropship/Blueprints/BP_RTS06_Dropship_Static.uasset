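; Static RTS06 dropship actor configured entirely in the Construction Script, with no runtime logic.
; Dynamic material instances apply tunable glass and a camo or plain finish to hull, wings, gear and door.
; Door and landing gear options repose those meshes, and a closed door also removes the point lights.
; Wing gun and missile selectors swap meshes and destroy unused components, including the Blueprint miniguns.
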(event EventBeginPlay)

(event Collision|EventActorBeginOverlap
  (params (OtherActor :type Actor%20Object%20Reference)))

(event EventTick
  (params (DeltaSeconds :type Float%20%28single-precision%29)))

(fn ConstructionScript
  (|ModifyMaterial)
  (if (Variables|Default|GetBackDoor_Open)
    _
    (else
      (Transformation|SetRelativeRotation (Variables|Default|GetSM_RT06_Dropship_Door) "0.000000, 0, 0" false false)
      (Components|DestroyComponent (Variables|Default|GetPointLight1))))
  (Utilities|FlowControl|Sequence
    (:then_0
      (CallFunction|ConstructLandingGear))
    (:then_1
      (CallFunction|ConstructWingsGunType))
    (:then_2
      (CallFunction|ConstructMissileType))))

(fn ConstructWingsGunType
  (switch int (Variables|Default|GetWings_Gun_Type)
    (:Default
      (Components|StaticMesh|SetStaticMesh (Variables|Default|GetSM_MachineGun_L) "/Game/Dropship/Meshes/Weapons/SM_RTS06_Dropship_Machinegun_X2.SM_RTS06_Dropship_Machinegun_X2" :!label _label)
      (Components|StaticMesh|SetStaticMesh (Variables|Default|GetSM_MachineGun_R) "/Game/Dropship/Meshes/Weapons/SM_RTS06_Dropship_Machinegun_X2.SM_RTS06_Dropship_Machinegun_X2")
      (Components|DestroyComponent (Variables|Default|GetBP_Minigun_L) :!label _label_2))
    (:0
      (Components|DestroyComponent (Variables|Default|GetSM_MachineGun_L))
      (goto _label_2))
    (:1
      (Components|StaticMesh|SetStaticMesh (Variables|Default|GetSM_MachineGun_L) "/Game/Dropship/Meshes/Weapons/SM_RTS06_Dropship_Machinegun_X1.SM_RTS06_Dropship_Machinegun_X1")
      (Components|StaticMesh|SetStaticMesh (Variables|Default|GetSM_MachineGun_R) "/Game/Dropship/Meshes/Weapons/SM_RTS06_Dropship_Machinegun_X1.SM_RTS06_Dropship_Machinegun_X1")
      (goto _label_2))
    (:2
      (goto _label))
    (:3
      (Components|DestroyComponent (Variables|Default|GetSM_MachineGun_L)))))

(fn ConstructLandingGear
  (if (not (Variables|Default|GetLandingGear_Down))
    (Transformation|SetRelativeLocation (Variables|Default|GetSM_RTS06_Dropship_LandingGear_F) "0,203.899994,98.500000" false false)
    (Transformation|SetRelativeRotation (Variables|Default|GetSM_RTS06_Dropship_LandingGear_L) "-90.000000, 0, 0" false false)
    (Transformation|SetRelativeRotation (Variables|Default|GetSM_RTS06_Dropship_LandingGear_R) "90.000000, 0, 0" false false)))

(fn ConstructMissileType
  (bind _sm_missile_r (Variables|Default|GetSM_Missile_R))
  (switch int (Variables|Default|GetWings_Missile_Type)
    (:Default
      (Components|StaticMesh|SetStaticMesh _sm_missile_r "/Game/Dropship/Meshes/Weapons/SM_RTS06_Dropship_MissileSmall.SM_RTS06_Dropship_MissileSmall" :!label _label)
      (Components|StaticMesh|SetStaticMesh (Variables|Default|GetSM_Missile_L) "/Game/Dropship/Meshes/Weapons/SM_RTS06_Dropship_MissileSmall.SM_RTS06_Dropship_MissileSmall")
      (Transformation|SetRelativeLocation _sm_missile_r "0,29.500000,-40.000000" false false))
    (:0
      (Components|DestroyComponent (Variables|Default|GetSM_MissileRack_L)))
    (:1
      (goto _label))
    (:2
      (Components|StaticMesh|SetStaticMesh (Variables|Default|GetSM_Missile_R) "/Game/Dropship/Meshes/Weapons/SM_RTS06_Dropship_Missile.SM_RTS06_Dropship_Missile")
      (Components|StaticMesh|SetStaticMesh (Variables|Default|GetSM_Missile_L) "/Game/Dropship/Meshes/Weapons/SM_RTS06_Dropship_Missile.SM_RTS06_Dropship_Missile"))))