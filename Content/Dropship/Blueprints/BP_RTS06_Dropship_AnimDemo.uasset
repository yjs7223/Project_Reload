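; Demo dropship actor with configurable wing guns, missiles, camo or plain paint and glass, applied by the construction script through mesh swaps and dynamic materials.
; Left mouse fires child-actor miniguns when fitted; right mouse alternately spawns left and right missiles, briefly hiding each wing mesh.
; A ping-pong timeline is set up to animate door, gear, wings, height, rotation and thrusters, but nothing in the graph starts it.
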(event EventBeginPlay
  (|CasttoMiniguns))

(event Input|MouseEvents|LeftMouseButton
  (params (Key :type Key%20Structure :default "AnyKey"))
  (bind _wings_gun_type (Variables|Default|GetWings_Gun_Type))
  (bind _returnvalue (== _wings_gun_type 3))
  (:Pressed
    (if _returnvalue
      (Default|Fire (Variables|Default|GetMinigun_L))
      (Default|Fire (Variables|Default|GetMinigun_R))))
  (:Released
    (if _returnvalue
      (Default|Stop (Variables|Default|GetMinigun_L))
      (Default|Stop (Variables|Default|GetMinigun_R)))))

(event Input|MouseEvents|RightMouseButton
  (params (Key :type Key%20Structure :default "AnyKey"))
  (bind _self self)
  (bind _wings_missile_type (Variables|Default|GetWings_Missile_Type))
  (bind _sm_missile_r (Variables|Default|GetSM_Missile_R))
  (bind _sm_missile_l (Variables|Default|GetSM_Missile_L))
  (bind _returnvalue (== _wings_missile_type 2))
  (bind _returnvalue_2 (select _returnvalue "/Game/Dropship/Blueprints/BP_RTS06_Dropship_Missile.BP_RTS06_Dropship_Missile_C" "/Game/Dropship/Blueprints/BP_RTS06_Dropship_Missile_Small.BP_RTS06_Dropship_Missile_Small_C"))
  (:Pressed
    (if (!= (Variables|Default|GetWings_Missile_Type) 0)
      (Utilities|FlowControl|FlipFlop
        (:A
          (Development|SetHiddeninGame _sm_missile_r true false)
          (Game|SpawnActorfromClass _returnvalue_2 (Transformation|GetWorldTransform _sm_missile_r) "Undefined" _self 0)
          (Utilities|FlowControl|Delay 2.0)
          (Development|SetHiddeninGame (Variables|Default|GetSM_Missile_R) false false))
        (:B
          (Development|SetHiddeninGame _sm_missile_l true false)
          (Game|SpawnActorfromClass _returnvalue_2 (Transformation|GetWorldTransform _sm_missile_l) "Undefined" _self 0)
          (Utilities|FlowControl|Delay 2.0)
          (Development|SetHiddeninGame (Variables|Default|GetSM_Missile_L) false false))))))

(fn ConstructionScript
  (|ModifyMaterial)
  (Variables|Default|SetSpawnLocation (Transformation|GetActorLocation))
  (Utilities|FlowControl|Sequence
    (:then_0
      (CallFunction|ConstructWingsGunType))
    (:then_1
      (CallFunction|ConstructMissileType))))

(fn ConstructWingsGunType
  (switch int (Variables|Default|GetWings_Gun_Type)
    (:Default
      (Components|StaticMesh|SetStaticMesh (Variables|Default|GetSM_MachineGun_L) "/Game/Dropship/Meshes/Weapons/SM_RTS06_Dropship_Machinegun_X2.SM_RTS06_Dropship_Machinegun_X2" :!label _label)
      (Components|StaticMesh|SetStaticMesh (Variables|Default|GetSM_MachineGun_R) "/Game/Dropship/Meshes/Weapons/SM_RTS06_Dropship_Machinegun_X2.SM_RTS06_Dropship_Machinegun_X2")
      (Components|DestroyComponent (Variables|Default|GetBP_Minigun_L) :!label _label_2))
    (:0
      (Components|DestroyComponent (Variables|Default|GetSM_MachineGun_L))
      (goto _label_2))
    (:1
      (Components|StaticMesh|SetStaticMesh (Variables|Default|GetSM_MachineGun_L) "/Game/Dropship/Meshes/Weapons/SM_RTS06_Dropship_Machinegun_X1.SM_RTS06_Dropship_Machinegun_X1")
      (Components|StaticMesh|SetStaticMesh (Variables|Default|GetSM_MachineGun_R) "/Game/Dropship/Meshes/Weapons/SM_RTS06_Dropship_Machinegun_X1.SM_RTS06_Dropship_Machinegun_X1")
      (goto _label_2))
    (:2
      (goto _label))
    (:3
      (Components|DestroyComponent (Variables|Default|GetSM_MachineGun_L)))))

(fn ConstructLandingGear
  (if (not (Variables|Default|GetLandingGear_Down))
    (Transformation|SetRelativeLocation (Variables|Default|GetSM_RTS06_Dropship_LandingGear_F) "0,203.899994,98.500000" false false)
    (Transformation|SetRelativeRotation (Variables|Default|GetSM_RTS06_Dropship_LandingGear_L) "-90.000000, 0, 0" false false)
    (Transformation|SetRelativeRotation (Variables|Default|GetSM_RTS06_Dropship_LandingGear_R) "90.000000, 0, 0" false false)))

(fn ConstructMissileType
  (bind _sm_missile_r (Variables|Default|GetSM_Missile_R))
  (switch int (Variables|Default|GetWings_Missile_Type)
    (:Default
      (Components|StaticMesh|SetStaticMesh _sm_missile_r "/Game/Dropship/Meshes/Weapons/SM_RTS06_Dropship_MissileSmall.SM_RTS06_Dropship_MissileSmall" :!label _label)
      (Components|StaticMesh|SetStaticMesh (Variables|Default|GetSM_Missile_L) "/Game/Dropship/Meshes/Weapons/SM_RTS06_Dropship_MissileSmall.SM_RTS06_Dropship_MissileSmall")
      (Transformation|SetRelativeLocation _sm_missile_r "0,29.500000,-40.000000" false false))
    (:0
      (Components|DestroyComponent (Variables|Default|GetSM_MissileRack_L)))
    (:1
      (goto _label))
    (:2
      (Components|StaticMesh|SetStaticMesh (Variables|Default|GetSM_Missile_R) "/Game/Dropship/Meshes/Weapons/SM_RTS06_Dropship_Missile.SM_RTS06_Dropship_Missile")
      (Components|StaticMesh|SetStaticMesh (Variables|Default|GetSM_Missile_L) "/Game/Dropship/Meshes/Weapons/SM_RTS06_Dropship_Missile.SM_RTS06_Dropship_Missile"))))