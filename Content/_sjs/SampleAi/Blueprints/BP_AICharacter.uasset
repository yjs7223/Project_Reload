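; BP_AICharacter is a sample AI character Blueprint that can shoot projectiles at a target actor.
; Its Shoot function validates the target, then spawns a BP_Projectile at the ShootPoint component with itself as instigator.
; The projectile's rotation is built from the normalized direction toward the target's location, raised slightly on Z to aim above its origin.
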(fn ConstructionScript)

(fn Shoot
  (params (TargetActor :type Actor%20Object%20Reference))
  (bind _output_get (LocalVariables|SetTarget TargetActor))
  (Utilities|IsValid _output_get
    (:Is%20Valid
      (Game|SpawnActorfromClass "/Game/_sjs/SampleAi/Blueprints/BP_Projectile.BP_Projectile_C" (Math|Transform|MakeTransform (Transformation|GetWorldLocation (Variables|Default|GetShootPoint)) (Math|Rotator|MakeRotfromX (Math|Vector|Normalize (- (+ (Transformation|GetActorLocation (LocalVariables|GetTarget)) "0,0,50.000000") (Transformation|GetWorldLocation (Variables|Default|GetShootPoint)))))) "Undefined" 0 self))))