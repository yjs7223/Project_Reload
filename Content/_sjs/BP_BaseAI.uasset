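; BP_BaseAI is a base AI Blueprint with an unfinished Shoot function for attacking a target actor.
; Shoot stores the passed actor as Target and checks its validity, but nothing follows the check.
; A disconnected SpawnActor node, with no class shown, would spawn at ShootPoint aimed slightly above the target's location, with itself as Instigator.
; The event graph and construction script are empty.
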(event EventBeginPlay)

(event Collision|EventActorBeginOverlap
  (params (OtherActor :type Actor%20Object%20Reference)))

(event EventTick
  (params (DeltaSeconds :type Float%20%28single-precision%29)))

(fn ConstructionScript)

(fn Shoot
  (params (TargetActor :type Actor%20Object%20Reference))
  (bind _output_get (LocalVariables|SetTarget TargetActor))
  (Utilities|IsValid _output_get))