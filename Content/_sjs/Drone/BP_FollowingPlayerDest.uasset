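; Invisible-target style actor that marks where the companion drone should sit relative to the player character.
; Each Tick it places itself above and to the left of the player using the character's forward and right vectors.
; The forward lead grows from nearly none when idle, to short when moving, to far ahead in the custom Runing movement mode.
; Movement is a swept SetActorLocation with no interpolation.
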(event EventTick
  (params (DeltaSeconds :type Float%20%28single-precision%29))
  (bind _returnvalue (Game|GetPlayerCharacter 0))
  (bind _returnvalue_2 (Transformation|GetActorLocation _returnvalue))
  (bind _returnvalue_3 (Transformation|GetActorLocation _returnvalue))
  (bind _returnvalue_4 (Transformation|GetActorForwardVector _returnvalue))
  (bind _returnvalue_5 (Transformation|GetActorRightVector _returnvalue))
  (bind _returnvalue_6 (Transformation|GetActorForwardVector _returnvalue))
  (bind _returnvalue_7 (Transformation|GetActorLocation _returnvalue))
  (bind _returnvalue_8 (Transformation|GetActorForwardVector _returnvalue))
  (bind _returnvalue_9 (Transformation|GetActorRightVector _returnvalue))
  (bind _returnvalue_10 (Transformation|GetActorRightVector _returnvalue))
  (bind _returnvalue_11 (Actor|GetComponentbyClass _returnvalue "/Script/Engine.CharacterMovementComponent"))
  (bind _returnvalue_12 (* _returnvalue_8 1.0))
  (bind _returnvalue_13 (* _returnvalue_9 -6e+01))
  (bind _returnvalue_14 (* _returnvalue_6 5e+01))
  (bind _returnvalue_15 (* _returnvalue_10 -6e+01))
  (bind _returnvalue_16 (* _returnvalue_5 -6e+01))
  (bind _returnvalue_17 (* _returnvalue_4 3.5e+02))
  (if (Utilities|Enum|Equal(Enum) (Utilities|Enum|ByteToEnumECustomMovementMode (Variables|/Script/Engine.CharacterMovementComponent|GetCustomMovementMode _returnvalue_11)) "CMOVE_Runing")
    (bind _output_get (Variables|Default|SetDronePos (+ (Math|Vector|MakeVector (.x _returnvalue_3) (.y _returnvalue_3) (+ (.z _returnvalue_3) 9e+01)) (Math|Vector|MakeVector (.x _returnvalue_17) (.y _returnvalue_17) 0.0) (Math|Vector|MakeVector (.x _returnvalue_16) (.y _returnvalue_16) 0.0))))
    (Transformation|SetActorLocation _output_get true false)
    (elif (> (Math|Vector|VectorLength (Variables|/Script/Engine.MovementComponent|GetVelocity _returnvalue_11)) 0.0)
      (bind _output_get_2 (Variables|Default|SetDronePos (+ (Math|Vector|MakeVector (.x _returnvalue_2) (.y _returnvalue_2) (+ (.z _returnvalue_2) 9e+01)) (Math|Vector|MakeVector (.x _returnvalue_14) (.y _returnvalue_14) 0.0) (Math|Vector|MakeVector (.x _returnvalue_15) (.y _returnvalue_15) 0.0))))
      (Transformation|SetActorLocation _output_get_2 true false)
      (else
        (bind _output_get_3 (Variables|Default|SetDronePos (+ (Math|Vector|MakeVector (.x _returnvalue_7) (.y _returnvalue_7) (+ (.z _returnvalue_7) 9e+01)) (Math|Vector|MakeVector (.x _returnvalue_12) (.y _returnvalue_12) 0.0) (Math|Vector|MakeVector (.x _returnvalue_13) (.y _returnvalue_13) 0.0))))
        (Transformation|SetActorLocation _output_get_3 true false)))))

(fn ConstructionScript)