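; BP_PWQ_LASER is an interactable pickup that attaches an accessory to the player's current weapon.
; On interaction, it proceeds only if that weapon is valid and its SMFlashlight component is hidden, then triggers the player's pickup and, after a short delay, a sound.
; It then reveals SMFlashlight, calls FlashlightAttached on the weapon and destroys itself.
; Despite the LASER name, all attachment logic targets the weapon's flashlight.
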(event EventBeginPlay
  (|CallParentFunction) ; This node is disabled and will not be called.\nDrag off pins to build functionality.
)

(event Collision|EventActorBeginOverlap
  (params (OtherActor :type Actor%20Object%20Reference))
  (|CallParentFunction OtherActor) ; This node is disabled and will not be called.\nDrag off pins to build functionality.
)

(event EventTick
  (params (DeltaSeconds :type Float%20%28single-precision%29))
  (|CallParentFunction DeltaSeconds) ; This node is disabled and will not be called.\nDrag off pins to build functionality.
)

(event EventOnInteracted
  (params (Player%200 :type BP%20FPS%20Arms%20Object%20Reference))
  (bind _currentweapon (Variables|/Game/FaLMG/FPS_Arms/Bluprints/BP_FPS_Arms.BP_FPS_Arms_C|GetCurrentWeapon Player%200))
  (bind _sm_flashlight (Variables|/Game/FaLMG/Weapons/Blueprints/PickUp_Master/Gun/BP_Weapon_Base.BP_Weapon_Base_C|GetSM_Flashlight _currentweapon))
  (Utilities|IsValid _currentweapon
    (:Is%20Valid
      (if (not (Rendering|IsVisible _sm_flashlight))
        (Default|ItemPickUp Player%200)
        (Utilities|FlowControl|Delay 0.2)
        (CallFunction|PickUpSound Player%200)
        (Rendering|SetVisibility _sm_flashlight true true)
        (Default|FlashlightAttached _currentweapon)
        (Actor|DestroyActor)))))

(fn ConstructionScript
  (|CallParentFunction))