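; Separated-mesh Blueprint of the AngryCat LMG weapon, extending a parent class with attachment, effect and ammo-belt visuals.
; Construction snaps flashlight, light and laser parts to sockets, while events play bipod montages and toggle iron sights and flashlight extras by attachment visibility.
; Smoke events drive muzzle and chamber particles, with a timeline animating silencer emissive through a dynamic material.
; Belt events show cartridge counts through SelectCartridge, and Tick updates the laser point.
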(event EventScopeAttached
  ;[1 1 1] Scope Attached
  (CallFunction|IronSightStates))

(event EventFlashlightAttached
  (bind _sm_flswitcher (Variables|Default|GetSM_FLSwitcher))
  ;[1 1 1] FlashlightAttached
  (if (Rendering|IsVisible (Variables|Default|GetSM_Flashlight))
    (Rendering|SetVisibility _sm_flswitcher true false)
    (else
      (Rendering|SetVisibility _sm_flswitcher false false))))

(event EventChamberSmoke
  ;[1 1 1] ChamberSmoke_Activated
  (Components|Activation|Activate (Variables|Default|GetChamber_smoke_PS) true))

(event EventInVisAllCartridges
  ;[1 0.08899 0] Invisible all cartridges (for separated mesh)
  (for _index (range 1 9)
    (bind _falmg_cartridge (CallFunction|SelectCartridge _index))
    (Rendering|SetVisibility _falmg_cartridge false false)))

(event EventInVisChainLink
  ;[1 0.08899 0] Invisible all cartridges (for separated mesh)
  (bind _falmg_cartridge (CallFunction|SelectCartridge))
  (Rendering|SetVisibility _falmg_cartridge false false))

(event EventVisible1b
  ;[1 1 1] Visible cartridges (for Separated mesh)
  (bind _falmg_cartridge (CallFunction|SelectCartridge))
  (Rendering|SetVisibility _falmg_cartridge true false)
  (bind _falmg_cartridge_2 (CallFunction|SelectCartridge 9))
  (Rendering|SetVisibility _falmg_cartridge_2 true false)
  ;;[1 0.06632 0] Invisible
  (for _index (range 1 8)
    (bind _falmg_cartridge_3 (CallFunction|SelectCartridge _index))
    (Rendering|SetVisibility _falmg_cartridge_3 false false)))

(event EventVisible2b
  ;[1 1 1] Visible cartridges (for Separated mesh)
  (bind _falmg_cartridge (CallFunction|SelectCartridge))
  (Rendering|SetVisibility _falmg_cartridge true false)
  (for _index (range 8 9)
    (bind _falmg_cartridge_2 (CallFunction|SelectCartridge _index))
    (Rendering|SetVisibility _falmg_cartridge_2 true false)
    ;;[1 0.06632 0] Invisible
    (for _index_2 (range 1 7)
      (bind _falmg_cartridge_3 (CallFunction|SelectCartridge _index_2))
      (Rendering|SetVisibility _falmg_cartridge_3 false false))))

(event EventVisible3b
  ;[1 1 1] Visible cartridges (for Separated mesh)
  (bind _falmg_cartridge (CallFunction|SelectCartridge))
  (Rendering|SetVisibility _falmg_cartridge true false)
  (for _index (range 7 9)
    (bind _falmg_cartridge_2 (CallFunction|SelectCartridge _index))
    (Rendering|SetVisibility _falmg_cartridge_2 true false)
    ;;[1 0.06632 0] Invisible
    (for _index_2 (range 1 6)
      (bind _falmg_cartridge_3 (CallFunction|SelectCartridge _index_2))
      (Rendering|SetVisibility _falmg_cartridge_3 false false))))

(event EventVisible4b
  ;[1 1 1] Visible cartridges (for Separated mesh)
  (bind _falmg_cartridge (CallFunction|SelectCartridge))
  (Rendering|SetVisibility _falmg_cartridge true false)
  (for _index (range 6 9)
    (bind _falmg_cartridge_2 (CallFunction|SelectCartridge _index))
    (Rendering|SetVisibility _falmg_cartridge_2 true false)
    ;;[1 0.06632 0] Invisible
    (for _index_2 (range 1 5)
      (bind _falmg_cartridge_3 (CallFunction|SelectCartridge _index_2))
      (Rendering|SetVisibility _falmg_cartridge_3 false false))))

(event EventVisible5b
  ;[1 1 1] Visible cartridges (for Separated mesh)
  (bind _falmg_cartridge (CallFunction|SelectCartridge))
  (Rendering|SetVisibility _falmg_cartridge true false)
  (for _index (range 5 9)
    (bind _falmg_cartridge_2 (CallFunction|SelectCartridge _index))
    (Rendering|SetVisibility _falmg_cartridge_2 true false)
    ;;[1 0.06632 0] Invisible
    (for _index_2 (range 1 4)
      (bind _falmg_cartridge_3 (CallFunction|SelectCartridge _index_2))
      (Rendering|SetVisibility _falmg_cartridge_3 false false))))

(event EventVisible6b
  ;[1 1 1] Visible cartridges (for Separated mesh)
  (bind _falmg_cartridge (CallFunction|SelectCartridge))
  (Rendering|SetVisibility _falmg_cartridge true false)
  (for _index (range 4 9)
    (bind _falmg_cartridge_2 (CallFunction|SelectCartridge _index))
    (Rendering|SetVisibility _falmg_cartridge_2 true false)
    ;;[1 0.06632 0] Invisible
    (for _index_2 (range 1 3)
      (bind _falmg_cartridge_3 (CallFunction|SelectCartridge _index_2))
      (Rendering|SetVisibility _falmg_cartridge_3 false false))))

(event EventVisible7b
  ;[1 1 1] Visible cartridges (for Separated mesh)
  (bind _falmg_cartridge (CallFunction|SelectCartridge))
  (Rendering|SetVisibility _falmg_cartridge true false)
  (for _index (range 3 9)
    (bind _falmg_cartridge_2 (CallFunction|SelectCartridge _index))
    (Rendering|SetVisibility _falmg_cartridge_2 true false)
    ;;[1 0.06632 0] Invisible
    (for _index_2 (range 1 2)
      (bind _falmg_cartridge_3 (CallFunction|SelectCartridge _index_2))
      (Rendering|SetVisibility _falmg_cartridge_3 false false))))

(event EventVisible8b
  ;[1 1 1] Visible cartridges (for Separated mesh)
  (bind _falmg_cartridge (CallFunction|SelectCartridge))
  (Rendering|SetVisibility _falmg_cartridge true false)
  (for _index (range 2 9)
    (bind _falmg_cartridge_2 (CallFunction|SelectCartridge _index))
    (Rendering|SetVisibility _falmg_cartridge_2 true false)
    ;;[1 0.06632 0] Invisible
    (bind _falmg_cartridge_3 (CallFunction|SelectCartridge 1))
    (Rendering|SetVisibility _falmg_cartridge_3 false false)))

(event EventVisibleAllCartridges
  ;[1 1 1] Visible cartridges (for Separated mesh)
  (bind _falmg_cartridge (CallFunction|SelectCartridge))
  (Rendering|SetVisibility _falmg_cartridge true false)
  (for _index (range 0 9)
    (bind _falmg_cartridge_2 (CallFunction|SelectCartridge _index))
    (Rendering|SetVisibility _falmg_cartridge_2 true false)))

(event EventBeginPlay
  (|CallParentFunction)
  ;[1 1 1] Silencer_Dynamic Material Instance
  (bind _returnvalue (Rendering|Material|CreateDynamicMaterialInstance (Variables|Default|GetSM_Silencer) 0 "/Game/FaLMG/Weapons/Materials/MaterialInstances/MI_FaLMG_Silencer_Inst.MI_FaLMG_Silencer_Inst" "None" :!class /Script/Engine.PrimitiveComponent))
  (Variables|Default|SetSilencer_DM _returnvalue))

(event EventBipodEvent
  (bind _skm_bipod (Variables|Default|GetSKM_Bipod))
  (bind _weapondata (Variables|Default|GetWeaponData))
  (bind _bipods_anim (Utilities|Struct|BreakBP_WeaponData_Struct _weapondata))
  (bind _returnvalue (Components|SkeletalMesh|GetAnimInstance _skm_bipod))
  ;[1 1 0] Bipods
  (if (Variables|/Game/FaLMG/FPS_Arms/Bluprints/BP_FPS_Arms.BP_FPS_Arms_C|GetBipodOpen (Variables|Default|GetCharacter%20Ref))
    (Animation|Montage|MontagePlay _returnvalue (Utilities|Array|Get(acopy) _bipods_anim) 1.0 "MontageLength" 0.0 true)
    (else
      (Animation|Montage|MontagePlay _returnvalue (Utilities|Array|Get(acopy) _bipods_anim 1) 1.0 "MontageLength" 0.0 true))))

(event EventBSmokeStop
  ;[1 1 1] MuzzleSmoke
  (Components|Activation|Deactivate (Variables|Default|GetMuzzleSmoke_PS))
  (Transformation|SetRelativeLocation (Variables|Default|GetMuzzleSmoke_PS) "0, 0, 0" false false)
  (if (Rendering|IsVisible (Variables|Default|GetSM_Silencer))
    ;[1 1 0] Silencer Emissive
    (bind _emissive_alpha (Timeline|Emissive_TL Play)
      (:Update
        (Rendering|Material|SetScalarParameterValue (Variables|Default|GetSilencer_DM) "Emissive Intensity" _emissive_alpha :!class /Script/Engine.MaterialInstanceDynamic)))))

(event EventBSmokeStart
  ;[1 1 1] MuzzleSmoke
  (if (> (.AmmoCurrent (Utilities|Struct|BreakBP_WeaponData_Struct (Variables|Default|GetWeaponData))) 0)
    (Utilities|FlowControl|Sequence
      (:then_0
        _)
      (:then_1
        (goto _label Reset)))
    (else
      (Utilities|FlowControl|DoOnce false :!label _label
        (:Completed
          _))))
  (Components|Activation|Activate (Variables|Default|GetMuzzleSmoke_PS) false)
  (if (Rendering|IsVisible (Variables|Default|GetSM_Silencer))
    (Transformation|SetRelativeLocation (Variables|Default|GetMuzzleSmoke_PS) (+ (Variables|/Script/Engine.SceneComponent|GetRelativeLocation (Variables|Default|GetMuzzleSmoke_PS)) "20.000000, 0, 0") false false)
    ;[1 1 0] Silencer Emissive
    (bind _emissive_alpha (Timeline|Emissive_TL Reverse)
      (:Update
        (Rendering|Material|SetScalarParameterValue (Variables|Default|GetSilencer_DM) "Emissive Intensity" _emissive_alpha :!class /Script/Engine.MaterialInstanceDynamic)))
    (else
      (Transformation|SetRelativeLocation (Variables|Default|GetMuzzleSmoke_PS) "0, 0, 0" false false)
      (if (Rendering|IsVisible (Variables|Default|GetSM_Silencer))
        (Timeline|Emissive_TL Play)))))

(event EventTick
  (params (DeltaSeconds :type Float%20%28single-precision%29))
  ;[1 1 1] Laser
  (if (not (and (== self (Variables|/Game/FaLMG/FPS_Arms/Bluprints/BP_FPS_Arms.BP_FPS_Arms_C|GetCurrentWeapon (Variables|Default|GetCharacter%20Ref))) (Rendering|IsVisible (Variables|Default|GetSM_Flashlight))))
    (Rendering|SetVisibility (Variables|Default|GetSM_Laser) false false)
    (Rendering|SetVisibility (Variables|Default|GetLaser_Point) false false)
    (else
      (CallFunction|LaserPointPosition))))

(fn ConstructionScript
  (|CallParentFunction)
  (CallFunction|AttachtoComponentFunc))

(fn AttachtoComponentFunc
  (Transformation|AttachComponentToComponent (Variables|Default|GetSM_Flashlight) (Variables|Default|GetHandguard) "PWQ_Laser_Sckt" "SnapToTarget" "SnapToTarget" "SnapToTarget" true)
  (Transformation|AttachComponentToComponent (Variables|Default|GetSpotLight) (Variables|Default|GetSM_Flashlight) "Light_Sckt" "SnapToTarget" "SnapToTarget" "SnapToTarget" true)
  (Transformation|AttachComponentToComponent (Variables|Default|GetLaser_Point) (Variables|Default|GetSM_Flashlight) "Light_Sckt" "SnapToTarget" "SnapToTarget" "SnapToTarget" true)
  (Transformation|AttachComponentToComponent (Variables|Default|GetSM_Laser) (Variables|Default|GetSM_Flashlight) "Laser_Sckt" "SnapToTarget" "SnapToTarget" "SnapToTarget" true)
  (Transformation|SetRelativeScale3D (Variables|Default|GetSM_Laser) "10.000000,0.200000,0.200000"))

(fn IronSightStates
  (bind _irs_pro_front_raised (Variables|Default|GetIRS_pro_Front_Raised))
  (bind _irs_pro_front (Variables|Default|GetIRS_pro_Front))
  (if (Rendering|IsVisible (Variables|Default|GetSM_Scope))
    (Rendering|SetVisibility _irs_pro_front_raised false false)
    (Rendering|SetVisibility _irs_pro_front true false)
    (else
      (Rendering|SetVisibility _irs_pro_front_raised true false)
      (Rendering|SetVisibility _irs_pro_front false false))))

(fn SelectCartridge
  (params (index :type Integer))
  (if (== index 0)
    (return (Variables|Default|GetSM_bChainLink))
    (elif (== index 1)
      (return (Variables|Default|GetCartridge_01))
      (elif (== index 2)
        (return (Variables|Default|GetCartridge_02))
        (elif (== index 3)
          (return (Variables|Default|GetCartridge_03))
          (elif (== index 4)
            (return (Variables|Default|GetCartridge_04))
            (elif (== index 5)
              (return (Variables|Default|GetCartridge_05))
              (elif (== index 6)
                (return (Variables|Default|GetCartridge_06))
                (elif (== index 7)
                  (return (Variables|Default|GetCartridge_07))
                  (elif (== index 8)
                    (return (Variables|Default|GetCartridge_08))
                    (elif (== index 9)
                      (return (Variables|Default|GetCartridge_09)))))))))))))