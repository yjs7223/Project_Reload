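; BP_FaLMG_Chainsaw is a child weapon Blueprint for the Chainsaw LMG, handling its attachments and cosmetic effects.
; Construction socket-attaches the flashlight, spotlight and laser; Tick updates or hides the laser, and iron sights switch with scope visibility.
; Events drive bipod montages, muzzle and chamber smoke, chain-link ejection and a timeline-animated silencer glow.
; The visible ammo belt changes by swapping cartridge material slots between red and invisible materials.
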(event EventFlashlightAttached
  (bind _sm_flswitcher_flmg_chs (Variables|Default|GetSM_FLSwitcher_FLMG_ChS))
  ;[1 1 1] FlashlightAttached
  (if (Rendering|IsVisible (Variables|Default|GetSM_Flashlight))
    (Rendering|SetVisibility _sm_flswitcher_flmg_chs true false)
    (else
      (Rendering|SetVisibility _sm_flswitcher_flmg_chs false false))))

(event EventChamberSmoke
  ;[1 1 1] ChamberSmoke_Activated
  (Components|Activation|Activate (Variables|Default|GetChamber_smoke_PS) true))

(event EventInVisAllCartridges
  ;[1 0.08899 0] Invisible all cartridges
  (for _index (range 2 10)
    (Rendering|Material|SetMaterial (Variables|Default|GetWeapon_SKMesh) _index "/Game/FaLMG/Weapons/Materials/MasterMaterials/MM_Invisible.MM_Invisible")))

(event EventInVisChainLink
  ;[1 0.08899 0] Invisible all cartridges
  (Rendering|Material|SetMaterial (Variables|Default|GetWeapon_SKMesh) 1 "/Game/FaLMG/Weapons/Materials/MasterMaterials/MM_Invisible.MM_Invisible"))

(event EventVisible1b
  (bind _weapon_skmesh (Variables|Default|GetWeapon_SKMesh))
  ;[1 1 1] Visible cartridges
  (Rendering|Material|SetMaterial _weapon_skmesh 1 "/Game/FaLMG/Weapons/Materials/MaterialInstances/Variations/MI_Cartridge_Red_RGBM.MI_Cartridge_Red_RGBM")
  (Rendering|Material|SetMaterial _weapon_skmesh 10 "/Game/FaLMG/Weapons/Materials/MaterialInstances/Variations/MI_Cartridge_Red_RGBM.MI_Cartridge_Red_RGBM")
  ;;[1 0.06632 0] Invisible
  (for _index (range 2 9)
    (Rendering|Material|SetMaterial _weapon_skmesh _index "/Game/FaLMG/Weapons/Materials/MasterMaterials/MM_Invisible.MM_Invisible")))

(event EventVisible2b
  (bind _weapon_skmesh (Variables|Default|GetWeapon_SKMesh))
  ;[1 1 1] Visible cartridges
  (Rendering|Material|SetMaterial _weapon_skmesh 1 "/Game/FaLMG/Weapons/Materials/MaterialInstances/Variations/MI_Cartridge_Red_RGBM.MI_Cartridge_Red_RGBM")
  (for _index (range 9 10)
    (Rendering|Material|SetMaterial _weapon_skmesh _index "/Game/FaLMG/Weapons/Materials/MaterialInstances/Variations/MI_Cartridge_Red_RGBM.MI_Cartridge_Red_RGBM")
    ;;[1 0.06632 0] Invisible
    (for _index_2 (range 2 8)
      (Rendering|Material|SetMaterial _weapon_skmesh _index_2 "/Game/FaLMG/Weapons/Materials/MasterMaterials/MM_Invisible.MM_Invisible"))))

(event EventVisible3b
  (bind _weapon_skmesh (Variables|Default|GetWeapon_SKMesh))
  ;[1 1 1] Visible cartridges
  (Rendering|Material|SetMaterial _weapon_skmesh 1 "/Game/FaLMG/Weapons/Materials/MaterialInstances/Variations/MI_Cartridge_Red_RGBM.MI_Cartridge_Red_RGBM")
  (for _index (range 8 10)
    (Rendering|Material|SetMaterial _weapon_skmesh _index "/Game/FaLMG/Weapons/Materials/MaterialInstances/Variations/MI_Cartridge_Red_RGBM.MI_Cartridge_Red_RGBM")
    ;;[1 0.06632 0] Invisible
    (for _index_2 (range 2 7)
      (Rendering|Material|SetMaterial _weapon_skmesh _index_2 "/Game/FaLMG/Weapons/Materials/MasterMaterials/MM_Invisible.MM_Invisible"))))

(event EventVisible4b
  (bind _weapon_skmesh (Variables|Default|GetWeapon_SKMesh))
  ;[1 1 1] Visible cartridges
  (Rendering|Material|SetMaterial _weapon_skmesh 1 "/Game/FaLMG/Weapons/Materials/MaterialInstances/Variations/MI_Cartridge_Red_RGBM.MI_Cartridge_Red_RGBM")
  (for _index (range 7 10)
    (Rendering|Material|SetMaterial _weapon_skmesh _index "/Game/FaLMG/Weapons/Materials/MaterialInstances/Variations/MI_Cartridge_Red_RGBM.MI_Cartridge_Red_RGBM")
    ;;[1 0.06632 0] Invisible
    (for _index_2 (range 2 6)
      (Rendering|Material|SetMaterial _weapon_skmesh _index_2 "/Game/FaLMG/Weapons/Materials/MasterMaterials/MM_Invisible.MM_Invisible"))))

(event EventVisible5b
  (bind _weapon_skmesh (Variables|Default|GetWeapon_SKMesh))
  ;[1 1 1] Visible cartridges
  (Rendering|Material|SetMaterial _weapon_skmesh 1 "/Game/FaLMG/Weapons/Materials/MaterialInstances/Variations/MI_Cartridge_Red_RGBM.MI_Cartridge_Red_RGBM")
  (for _index (range 6 10)
    (Rendering|Material|SetMaterial _weapon_skmesh _index "/Game/FaLMG/Weapons/Materials/MaterialInstances/Variations/MI_Cartridge_Red_RGBM.MI_Cartridge_Red_RGBM")
    ;;[1 0.06632 0] Invisible
    (for _index_2 (range 2 5)
      (Rendering|Material|SetMaterial _weapon_skmesh _index_2 "/Game/FaLMG/Weapons/Materials/MasterMaterials/MM_Invisible.MM_Invisible"))))

(event EventVisible6b
  (bind _weapon_skmesh (Variables|Default|GetWeapon_SKMesh))
  ;[1 1 1] Visible cartridges
  (Rendering|Material|SetMaterial _weapon_skmesh 1 "/Game/FaLMG/Weapons/Materials/MaterialInstances/Variations/MI_Cartridge_Red_RGBM.MI_Cartridge_Red_RGBM")
  (for _index (range 5 10)
    (Rendering|Material|SetMaterial _weapon_skmesh _index "/Game/FaLMG/Weapons/Materials/MaterialInstances/Variations/MI_Cartridge_Red_RGBM.MI_Cartridge_Red_RGBM")
    ;;[1 0.06632 0] Invisible
    (for _index_2 (range 2 4)
      (Rendering|Material|SetMaterial _weapon_skmesh _index_2 "/Game/FaLMG/Weapons/Materials/MasterMaterials/MM_Invisible.MM_Invisible"))))

(event EventVisible7b
  (bind _weapon_skmesh (Variables|Default|GetWeapon_SKMesh))
  ;[1 1 1] Visible cartridges
  (Rendering|Material|SetMaterial _weapon_skmesh 1 "/Game/FaLMG/Weapons/Materials/MaterialInstances/Variations/MI_Cartridge_Red_RGBM.MI_Cartridge_Red_RGBM")
  (for _index (range 4 10)
    (Rendering|Material|SetMaterial _weapon_skmesh _index "/Game/FaLMG/Weapons/Materials/MaterialInstances/Variations/MI_Cartridge_Red_RGBM.MI_Cartridge_Red_RGBM")
    ;;[1 0.06632 0] Invisible
    (for _index_2 (range 2 3)
      (Rendering|Material|SetMaterial _weapon_skmesh _index_2 "/Game/FaLMG/Weapons/Materials/MasterMaterials/MM_Invisible.MM_Invisible"))))

(event EventVisible8b
  (bind _weapon_skmesh (Variables|Default|GetWeapon_SKMesh))
  ;[1 1 1] Visible cartridges
  (Rendering|Material|SetMaterial _weapon_skmesh 1 "/Game/FaLMG/Weapons/Materials/MaterialInstances/Variations/MI_Cartridge_Red_RGBM.MI_Cartridge_Red_RGBM")
  (for _index (range 3 10)
    (Rendering|Material|SetMaterial _weapon_skmesh _index "/Game/FaLMG/Weapons/Materials/MaterialInstances/Variations/MI_Cartridge_Red_RGBM.MI_Cartridge_Red_RGBM")
    ;;[1 0.06632 0] Invisible
    (Rendering|Material|SetMaterial _weapon_skmesh 2 "/Game/FaLMG/Weapons/Materials/MasterMaterials/MM_Invisible.MM_Invisible")))

(event EventVisibleAllCartridges
  ;[1 1 1] Visible cartridges
  (for _index (range 1 10)
    (Rendering|Material|SetMaterial (Variables|Default|GetWeapon_SKMesh) _index "/Game/FaLMG/Weapons/Materials/MaterialInstances/Variations/MI_Cartridge_Red_RGBM.MI_Cartridge_Red_RGBM")))

(event EventBeginPlay
  (|CallParentFunction)
  ;[1 1 1] Silencer_Dynamic Material Instance
  (bind _returnvalue (Rendering|Material|CreateDynamicMaterialInstance (Variables|Default|GetSM_Silencer) 0 "/Game/FaLMG/Weapons/Materials/MaterialInstances/MI_FaLMG_Silencer_Inst.MI_FaLMG_Silencer_Inst" "None" :!class /Script/Engine.PrimitiveComponent))
  (Variables|Default|SetSilencer_DM _returnvalue))

(event EventBipodEvent
  (bind _skm_bipod (Variables|Default|GetSKM_Bipod))
  (bind _weapondata (Variables|Default|GetWeaponData))
  (bind _bipods_anim (Utilities|Struct|BreakBP_WeaponData_Struct _weapondata))
  (bind _returnvalue (Components|SkeletalMesh|GetAnimInstance _skm_bipod))
  ;[1 1 0] Bipods
  (if (Variables|/Game/FaLMG/FPS_Arms/Bluprints/BP_FPS_Arms.BP_FPS_Arms_C|GetBipodOpen (Variables|Default|GetCharacter%20Ref))
    (Animation|Montage|MontagePlay _returnvalue (Utilities|Array|Get(acopy) _bipods_anim) 1.0 "MontageLength" 0.0 true)
    (else
      (Animation|Montage|MontagePlay _returnvalue (Utilities|Array|Get(acopy) _bipods_anim 1) 1.0 "MontageLength" 0.0 true))))

(event EventBSmokeStop
  ;[1 1 1] MuzzleSmoke
  (Components|Activation|Deactivate (Variables|Default|GetMuzzleSmoke_PS))
  (Transformation|SetRelativeLocation (Variables|Default|GetMuzzleSmoke_PS) "0, 0, 0" false false)
  (if (Rendering|IsVisible (Variables|Default|GetSM_Silencer))
    ;[1 1 0] Silencer Emissive
    (bind _emissive_alpha (Timeline|Emissive_TL Play)
      (:Update
        (Rendering|Material|SetScalarParameterValue (Variables|Default|GetSilencer_DM) "Emissive Intensity" _emissive_alpha :!class /Script/Engine.MaterialInstanceDynamic)))))

(event EventBSmokeStart
  ;[1 1 1] MuzzleSmoke
  (if (> (.AmmoCurrent (Utilities|Struct|BreakBP_WeaponData_Struct (Variables|Default|GetWeaponData))) 0)
    (Utilities|FlowControl|Sequence
      (:then_0
        _)
      (:then_1
        (goto _label Reset)))
    (else
      (Utilities|FlowControl|DoOnce false :!label _label
        (:Completed
          _))))
  (Components|Activation|Activate (Variables|Default|GetMuzzleSmoke_PS) false)
  (if (Rendering|IsVisible (Variables|Default|GetSM_Silencer))
    (Transformation|SetRelativeLocation (Variables|Default|GetMuzzleSmoke_PS) (+ (Variables|/Script/Engine.SceneComponent|GetRelativeLocation (Variables|Default|GetMuzzleSmoke_PS)) "20.000000, 0, 0") false false)
    ;[1 1 0] Silencer Emissive
    (bind _emissive_alpha (Timeline|Emissive_TL Reverse)
      (:Update
        (Rendering|Material|SetScalarParameterValue (Variables|Default|GetSilencer_DM) "Emissive Intensity" _emissive_alpha :!class /Script/Engine.MaterialInstanceDynamic)))
    (else
      (Transformation|SetRelativeLocation (Variables|Default|GetMuzzleSmoke_PS) "0, 0, 0" false false)
      (if (Rendering|IsVisible (Variables|Default|GetSM_Silencer))
        (Timeline|Emissive_TL Play)))))

(event EventTick
  (params (DeltaSeconds :type Float%20%28single-precision%29))
  ;[1 1 1] Laser
  (if (not (and (== self (Variables|/Game/FaLMG/FPS_Arms/Bluprints/BP_FPS_Arms.BP_FPS_Arms_C|GetCurrentWeapon (Variables|Default|GetCharacter%20Ref))) (Rendering|IsVisible (Variables|Default|GetSM_Flashlight))))
    (Rendering|SetVisibility (Variables|Default|GetSM_Laser) false false)
    (Rendering|SetVisibility (Variables|Default|GetLaser_Point) false false)
    (else
      (CallFunction|LaserPointPosition))))

(fn ConstructionScript
  (|CallParentFunction)
  (CallFunction|AttachtoComponentFunc))

(fn AttachtoComponentFunc
  (Transformation|AttachComponentToComponent (Variables|Default|GetSM_Flashlight) (Variables|Default|GetHandguard) "PWQ_Laser_Sckt" "SnapToTarget" "SnapToTarget" "SnapToTarget" true)
  (Transformation|AttachComponentToComponent (Variables|Default|GetSpotLight) (Variables|Default|GetSM_Flashlight) "Light_Sckt" "SnapToTarget" "SnapToTarget" "SnapToTarget" true)
  (Transformation|AttachComponentToComponent (Variables|Default|GetLaser_Point) (Variables|Default|GetSM_Flashlight) "Light_Sckt" "SnapToTarget" "SnapToTarget" "SnapToTarget" true)
  (Transformation|AttachComponentToComponent (Variables|Default|GetSM_Laser) (Variables|Default|GetSM_Flashlight) "Laser_Sckt" "SnapToTarget" "SnapToTarget" "SnapToTarget" true)
  (Transformation|SetRelativeScale3D (Variables|Default|GetSM_Laser) "10.000000,0.200000,0.200000"))

(fn IronSightStates
  (bind _irs_pro_front_raised (Variables|Default|GetIRS_pro_Front_Raised))
  (bind _irs_pro_front (Variables|Default|GetIRS_pro_Front))
  (if (Rendering|IsVisible (Variables|Default|GetSM_Scope))
    (Rendering|SetVisibility _irs_pro_front_raised false false)
    (Rendering|SetVisibility _irs_pro_front true false)
    (else
      (Rendering|SetVisibility _irs_pro_front_raised true false)
      (Rendering|SetVisibility _irs_pro_front false false))))