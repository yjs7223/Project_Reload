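; Showcase variant of the East MRAP Ural Typhoon vehicle, exposing its adjustable features to slider, checkbox and button controls.
; Generic control events forward their values to setters for wheel speed and angle, damaged state, skin type, hatch and door angles, and light emissivity.
; Construction defers to the parent, and the Blueprint runs no active BeginPlay, overlap or Tick logic of its own.
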(event EventSetButtonsVariable0
  (params (NewIndex :type Integer))
  ;[1 1 1] Maps button controls to vehicle properties
  (CallFunction|SetSkinType (Math|Conversions|ToFloat(Integer) NewIndex)))

(event Collision|EventActorBeginOverlap
  (params (OtherActor :type Actor%20Object%20Reference))
  (|CallParentFunction OtherActor) ; This node is disabled and will not be called.\nDrag off pins to build functionality.
)

(event EventSetCheckboxVariable0
  (params (NewState :type Boolean))
  ;[1 1 1] Maps checkbox controls to vehicle properties
  (CallFunction|SetShowDamaged NewState))

(event EventTick
  (params (DeltaSeconds :type Float%20%28single-precision%29))
  (|CallParentFunction DeltaSeconds) ; This node is disabled and will not be called.\nDrag off pins to build functionality.
)

(event EventSetSliderVariable0
  (params (NewValue :type Float%20%28single-precision%29))
  ;[1 1 1] Maps slider controls to vehicle properties
  (CallFunction|SetWheelSpeed NewValue))

(event EventBeginPlay
  (|CallParentFunction) ; This node is disabled and will not be called.\nDrag off pins to build functionality.
)

(event EventSetSliderVariable1
  (params (NewValue :type Float%20%28single-precision%29))
  ;[1 1 1] Maps slider controls to vehicle properties
  (CallFunction|SetWheelAngle NewValue))

(event EventSetSliderVariable2
  (params (NewValue :type Float%20%28single-precision%29))
  ;[1 1 1] Maps slider controls to vehicle properties
  (CallFunction|SetHatchesAngle NewValue))

(event EventSetSliderVariable3
  (params (NewValue :type Float%20%28single-precision%29))
  ;[1 1 1] Maps slider controls to vehicle properties
  (CallFunction|SetDoorsAngle NewValue))

(event EventSetSliderVariable4
  (params (NewValue :type Float%20%28single-precision%29))
  ;[1 1 1] Maps slider controls to vehicle properties
  (CallFunction|SetLightsEmissivity NewValue))

(fn ConstructionScript
  (|CallParentFunction))